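; BP_GrabSocket is a socket that snaps grabbable objects of a configured class onto itself.
; Collision overlap stores a matching Grabbable actor as the candidate and attaches it immediately if it is not held.
; Tick attaches the candidate unless it is both held and already the slotted object, then records it as the slot occupant.
; Ending overlap with any Grabbable clears the candidate.
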(event OnComponentBeginOverlap(Collision)
  (params (OverlappedComponent :type Primitive%20Component%20Object%20Reference) (OtherActor :type Actor%20Object%20Reference) (OtherComp :type Primitive%20Component%20Object%20Reference) (OtherBodyIndex :type Integer) (bFromSweep :type Boolean) (SweepResult :type Hit%20Result%20Structure%20%28by%20ref%29))
  (if (Utilities|DoesObjectImplementInterface OtherActor "/Script/CouchGame.Grabbable")
    (if (== (Utilities|GetClass OtherActor) (Variables|Default|GetObjectType))
      (Variables|Default|SetGrabObject OtherActor)
      (bind _returnvalue (Class|Grabbable|GetIsGrabbed(Message) OtherActor))
      (if (not _returnvalue)
        (Transformation|AttachComponentToComponent OtherActor (Variables|Default|GetParent) "None" "SnapToTarget" "SnapToTarget" "KeepWorld" true)))))

(event OnComponentEndOverlap(Collision)
  (params (OverlappedComponent :type Primitive%20Component%20Object%20Reference) (OtherActor :type Actor%20Object%20Reference) (OtherComp :type Primitive%20Component%20Object%20Reference) (OtherBodyIndex :type Integer))
  (if (Utilities|DoesObjectImplementInterface OtherActor "/Script/CouchGame.Grabbable")
    (Variables|Default|SetGrabObject 0)))

(event EventTick
  (params (DeltaSeconds :type Float%20%28single-precision%29))
  (Utilities|IsValid (Variables|Default|GetGrabObject)
    (:Is%20Valid
      (bind _returnvalue (Class|Grabbable|GetIsGrabbed(Message) (Variables|Default|GetGrabObject)))
      (if (not (and _returnvalue (== (Variables|Default|GetGrabObject) (Variables|Default|GetObjectInSlot))))
        (Transformation|AttachComponentToComponent (Variables|Default|GetGrabObject) (Variables|Default|GetParent) "None" "SnapToTarget" "SnapToTarget" "KeepWorld" true)
        (Variables|Default|SetObjectInSlot (Variables|Default|GetGrabObject))
        (Variables|Default|SetGrabObject 0)))))

(fn ConstructionScript)
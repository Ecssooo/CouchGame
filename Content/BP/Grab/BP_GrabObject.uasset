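; BP_GrabObject is a grabbable object that tracks whether a player holds it.
; OnGrab stores the player and sets IsGrabbed, and OnDrop clears the flag, both printing debug strings.
; FixPosition snaps the root component to the stored player's location and rotation, though nothing in this Blueprint calls it.
; GetIsGrabbed exposes the held state.
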(event EventOnDrop
  (params (Player :type Character%20Player%20Object%20Reference))
  (Variables|Default|SetIsGrabbed false)
  (Development|PrintString "OnDrop"))

(event EventOnGrab
  (params (Player :type Character%20Player%20Object%20Reference))
  (Development|PrintString "Grab")
  (Variables|Default|SetIsGrabbed true)
  (Variables|Default|SetPlayer Player))

(fn ConstructionScript)

(fn FixPosition
  (bind _player (Variables|Default|GetPlayer))
  (bind _returnvalue (Transformation|GetActorTransform _player))
  (Transformation|SetWorldLocationAndRotation (Variables|Default|GetDefaultSceneRoot) (.location _returnvalue) (.rotation _returnvalue) false false))

(fn GetIsGrabbed
  (return (Variables|Default|GetIsGrabbed)))
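; BP_GrabMultiSocket is a multi-socket grab Blueprint that reveals a sub-level when its quest is validated.
; On QuestValid it reports its face and sub-level IDs to LevelComunicationSubsystem as discovered.
; If the level ID held by M matches that face, it also has M load that sub-level's partition.
; The construction script is empty, and no grab or socket logic appears in these graphs.
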(event EventQuestValid
  (bind _idface (Variables|Default|GetIDFace))
  (Class|LevelComunicationSubsystem|DiscoveredSubLevel (Subsystems|GetLevelComunicationSubsystem) _idface (Variables|Default|GetIDSubLevel))
  (if (== (Variables|/Script/CouchGame.LevelComunicationManager|GetLevelID (Variables|Default|Getm)) _idface)
    (Class|LevelComunicationManager|LoadSpecificPartition (Variables|Default|Getm) (Variables|Default|GetIDSubLevel))))

(fn ConstructionScript)
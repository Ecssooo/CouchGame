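; Camera transition actor that moves the main camera toward an "in" or "out" camera position and binds to a cube's rotation-end event.
; Two timelines take their float curves from TimelineSettings class defaults at BeginPlay.
; Each update lerps location only, from the camera's current position, so the easing compounds.
; Blend-out disables camera following at its start, while blend-in re-enables it on finish.
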(event Custom|CE_BlendOut
  (Variables|/Game/BP/Camera/BP_CameraActor.BP_CameraActor_C|SetCanFollow (Variables|Default|GetMainCamera) false)
  (bind _blendout (Timeline|BlendOut PlayFromStart)
    (:Update
      (Transformation|SetActorLocation (Variables|Default|GetMainCamera) (Math|Vector|Lerp(Vector) (Transformation|GetActorLocation (Variables|Default|GetMainCamera)) (Transformation|GetActorLocation (Variables|Default|GetOutCamera)) _blendout) false false))))

(event Custom|CE_BlendIn
  (bind _blendin (Timeline|BlendIn PlayFromStart)
    (:Update
      (Transformation|SetActorLocation (Variables|Default|GetMainCamera) (Math|Vector|Lerp(Vector) (Transformation|GetActorLocation (Variables|Default|GetMainCamera)) (Transformation|GetActorLocation (Variables|Default|GetInCamera)) _blendin) false false))
    (:Finished
      (Variables|/Game/BP/Camera/BP_CameraActor.BP_CameraActor_C|SetCanFollow (Variables|Default|GetMainCamera) true))))

(event EventBeginPlay
  (bind (_blendcamerain _blendcameraout) (Utilities|GetClassDefaults "/Script/CouchGame.TimelineSettings"))
  (EventDispatchers|BindEventtoOnRotationEnd (Variables|Default|GetCube) (EventDispatchers|CreateEvent :!event Custom|CE_BlendIn))
  (Class|TimelineComponent|SetFloatCurve (Variables|Default|GetBlendIn) (Utilities|ResolveSoftReference _blendcamerain) "BlendIn")
  (Class|TimelineComponent|SetFloatCurve (Variables|Default|GetBlendOut) (Utilities|ResolveSoftReference _blendcameraout) "BlendOut"))

(fn ConstructionScript)
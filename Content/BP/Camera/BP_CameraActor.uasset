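; Two-player camera actor that slides between its starting position and a target point marked by its CameraTargetPos component.
; BeginPlay waits briefly, then caches both player characters and the two world positions.
; Each Tick, it moves toward the target when both players' X reaches the target X plus a margin, otherwise back to the start.
; Forward/back flags select which VInterpTo drives the actor's location at a configurable speed.
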(event EventBeginPlay
  ;[0.15 0.15 0.15 0.5] Begin Play
  (Utilities|FlowControl|Delay 1.0)
  (Variables|Default|SetPlayer_1 (Game|GetPlayerCharacter 0))
  (Variables|Default|SetPlayer_2 (Game|GetPlayerCharacter 1))
  (Variables|Default|SetCamStartPos (Transformation|GetActorLocation))
  (Variables|Default|SetTargetPos (Transformation|GetWorldLocation (Variables|Default|GetCameraTargetPos)))
  (Components|Activation|SetAutoActivate (Variables|Default|GetCameraTargetPos) false))

(event EventTick
  (params (DeltaSeconds :type Float%20%28single-precision%29))
  (bind _targetpos (Variables|Default|GetTargetPos))
  (Variables|Default|SetDelta%20Seconds DeltaSeconds)
  (Utilities|IsValid (Variables|Default|GetPlayer_1)
    (:Is%20Valid
      (Utilities|IsValid (Variables|Default|GetPlayer_2)
        (:Is%20Valid
          (Utilities|FlowControl|Sequence
            (:then_0
              ;[0.15 0.15 0.15 0.5] Avance Camera
              (if (Variables|Default|GetIsForward)
                (bind _returnvalue (Math|Interpolation|VInterpTo (Transformation|GetActorLocation) (Variables|Default|GetTargetPos) (Variables|Default|GetDelta%20Seconds) (Variables|Default|GetSpeedMovementCamera)))
                (Transformation|SetActorLocation _returnvalue false false)))
            (:then_1
              ;[0.15 0.15 0.15 0.5] Recule Camera
              (if (Variables|Default|GetIsBack)
                (bind _returnvalue_2 (Math|Interpolation|VInterpTo (Transformation|GetActorLocation) (Variables|Default|GetCamStartPos) (Variables|Default|GetDelta%20Seconds) (Variables|Default|GetSpeedMovementCamera)))
                (Transformation|SetActorLocation _returnvalue_2 false false)))
            (:then_2
              (if (and (>= (.x (Transformation|GetActorLocation (Variables|Default|GetPlayer_2))) (+ (.x _targetpos) (Variables|Default|GetMargeCamera))) (>= (.x (Transformation|GetActorLocation (Variables|Default|GetPlayer_1))) (+ (.x _targetpos) (Variables|Default|GetMargeCamera))))
                (if (not (Variables|Default|GetIsForward))
                  (Variables|Default|SetIsForward true)
                  (Variables|Default|SetIsBack false))
                (elif (not (Variables|Default|GetIsBack))
                  (Variables|Default|SetIsForward false)
                  (Variables|Default|SetIsBack true))))))))))

(fn ConstructionScript)
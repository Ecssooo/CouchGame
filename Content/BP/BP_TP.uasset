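; BP_TP is a teleport trigger that moves players out and rotates the cube once two player overlaps are counted.
; It caches the TP manager, cube and game mode on BeginPlay, then counts overlaps from BPI_Player actors, with no decrement.
; At exactly two, it calls the game mode's teleport, unloads the level through the manager, and calls the cube rotation matching its Direction.
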(event OnComponentBeginOverlap(Trigger)
  (params (OverlappedComponent :type Primitive%20Component%20Object%20Reference) (OtherActor :type Actor%20Object%20Reference) (OtherComp :type Primitive%20Component%20Object%20Reference) (OtherBodyIndex :type Integer) (bFromSweep :type Boolean) (SweepResult :type Hit%20Result%20Structure%20%28by%20ref%29))
  (if (Utilities|DoesObjectImplementInterface OtherActor "/Game/BP/BPI_Player.BPI_Player_C")
    (Variables|Default|SetNbPlayerHir (+ (Variables|Default|GetNbPlayerHir) 1))
    (CallFunction|FTryTP)))

(event EventBeginPlay
  (Utilities|FlowControl|Sequence
    (:then_0
      (bind _returnvalue (Actor|GetActorOfClass "/Game/BP/BP_TPManager.BP_TPManager_C"))
      (Variables|Default|SetBP_TPManager _returnvalue))
    (:then_1
      (bind _returnvalue_2 (Actor|GetActorOfClass "/Game/BP/BP_Cube.BP_Cube_C"))
      (Variables|Default|SetBP_Cube _returnvalue_2))
    (:then_2
      (bind _ascube_game_mode (Utilities|Casting|CastToCubeGameMode (Game|GetGameMode)))
      (Variables|Default|SetAs%20Cube%20Game%20Mode _ascube_game_mode))))

(fn ConstructionScript)

(fn FTryTP
  (if (== (Variables|Default|GetNbPlayerHir) 2)
    (Class|CubeGameMode|TeleportCharacterOut (Variables|Default|GetAs%20Cube%20Game%20Mode))
    (switch Utilities|FlowControl|Switch|SwitchonELevelDir (Variables|Default|GetDirection)
      (:Up
        (Default|FUnloadLevel (Variables|Default|GetBP_TPManager))
        (Default|CERotateUp (Variables|Default|GetBP_Cube) "Up"))
      (:Down
        (Default|FUnloadLevel (Variables|Default|GetBP_TPManager))
        (Default|CERotateDown (Variables|Default|GetBP_Cube) "Up"))
      (:Left
        (Default|FUnloadLevel (Variables|Default|GetBP_TPManager))
        (Default|CERotateLeft (Variables|Default|GetBP_Cube) "Up"))
      (:Right
        (Default|FUnloadLevel (Variables|Default|GetBP_TPManager))
        (Default|CERotateRight (Variables|Default|GetBP_Cube) "Up")))))
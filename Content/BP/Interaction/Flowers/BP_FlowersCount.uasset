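; BP_FlowersCount is an actor that shows a flower count on a widget component in the world.
; On BeginPlay it caches the camera actor, BP_Step_FlowerFace6 and its WBP_FlowersCount widget, then after a short delay rotates the widget once to face the camera, keeping its roll.
; Every Tick it pushes the step actor's FlowerCount into the widget.
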(event Custom|CE_RotationWidget
  (bind _worldcamera (Variables|Default|GetWorldCamera))
  (bind _widget (Variables|Default|GetWidget))
  (bind _returnvalue (Transformation|GetWorldLocation _widget))
  (bind _rootcomponent (Variables|/Script/Engine.Actor|GetRootComponent _worldcamera))
  (bind _returnvalue_2 (Transformation|GetWorldLocation _rootcomponent))
  (bind _returnvalue_3 (Math|Rotator|FindLookatRotation _returnvalue _returnvalue_2))
  ;[0.15 0.15 0.15 0.5] Rotation Widget
  (Transformation|SetWorldRotation (Variables|Default|GetWidget) (Math|Rotator|MakeRotator (.roll (Transformation|GetWorldRotation (Variables|Default|GetWidget))) (.pitch _returnvalue_3) (.yaw _returnvalue_3)) false false))

(event EventBeginPlay
  ;[0.15 0.15 0.15 0.5] Begin Play
  (bind _returnvalue (Actor|GetActorOfClass "/Game/BP/Camera/BP_CameraActor.BP_CameraActor_C"))
  (Variables|Default|SetWorldCamera _returnvalue)
  (bind _returnvalue_2 (Actor|GetActorOfClass "/Game/BP/Steps/Face6/BP_Step_FlowerFace6.BP_Step_FlowerFace6_C"))
  (Variables|Default|SetStepFlower _returnvalue_2)
  (bind _aswbp_flowers_count (Utilities|Casting|CastToWBP_FlowersCount (UserInterface|GetUserWidgetObject (Variables|Default|GetWidget))))
  (Variables|Default|SetAs%20WBP%20Flowers%20Count _aswbp_flowers_count)
  (Utilities|FlowControl|Delay 1.0)
  (CallFunction|CERotationWidget))

(event EventTick
  (params (DeltaSeconds :type Float%20%28single-precision%29))
  (Default|CESetFlowerCount (Variables|Default|GetAs%20WBP%20Flowers%20Count) (Variables|/Game/BP/Steps/Face6/BP_Step_FlowerFace6.BP_Step_FlowerFace6_C|GetFlowerCount (Variables|Default|GetStepFlower))))

(fn ConstructionScript)
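; Interactable physics ball that players grab, throw and pass to each other to unlock sublevels.
; QTE1 toggles grab and drop at the player's grab parent; QTE2 throws the held ball in an arc or pushes a loose one.
; A different player overlapping the launched ball catches it and scores; enough catches reveal and load sublevels.
; A Tick line trace clears the launched state when it hits the BP_Cube.
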(event OnComponentBeginOverlap(Box)
  (params (OverlappedComponent :type Primitive%20Component%20Object%20Reference) (OtherActor :type Actor%20Object%20Reference) (OtherComp :type Primitive%20Component%20Object%20Reference) (OtherBodyIndex :type Integer) (bFromSweep :type Boolean) (SweepResult :type Hit%20Result%20Structure%20%28by%20ref%29))
  (bind _levelcommanager (Variables|Default|GetLevelComManager))
  (bind _levelcommanager_2 (Variables|Default|GetLevelComManager))
  (if (Variables|Default|GetIsBallLaunch)
    (if (Utilities|DoesObjectImplementInterface OtherActor "/Game/BP/BPI/BPI_Player.BPI_Player_C")
      (if (!= OtherActor (Variables|Default|GetPlayer))
        (Variables|Default|SetIsBallLaunch false)
        (bind _ascharacter_player (Utilities|Casting|CastToCharacterPlayer OtherActor))
        (bind _returnvalue (Class|CharacterPlayer|GetGrabParent _ascharacter_player))
        (Transformation|AttachComponentToComponent _returnvalue "None" "SnapToTarget" "KeepRelative" "KeepWorld" true)
        (Variables|/Script/CouchGame.CharacterPlayer|SetInteractableActor _ascharacter_player self)
        (bind _result (Math|Integer|IncrementInt (Variables|Default|GetScore))
          (:%20%20
            (if (>= _result 3)
              (Class|LevelComunicationSubsystem|DiscoveredSubLevel (Subsystems|GetLevelComunicationSubsystem) 2 3)
              (if (== (Variables|/Script/CouchGame.LevelComunicationManager|GetLevelID _levelcommanager_2) 2)
                (Class|LevelComunicationManager|LoadSpecificPartition _levelcommanager_2 3)
                (Class|LevelComunicationSubsystem|DiscoveredSubLevel (Subsystems|GetLevelComunicationSubsystem) 2 5)
                (if (== (Variables|/Script/CouchGame.LevelComunicationManager|GetLevelID _levelcommanager) 2)
                  (Class|LevelComunicationManager|LoadSpecificPartition _levelcommanager 5)
                  (Class|LevelComunicationSubsystem|DiscoveredSubLevel (Subsystems|GetLevelComunicationSubsystem) 4 8))))))))))

(event EventTick
  (params (DeltaSeconds :type Float%20%28single-precision%29))
  (bind _sphere (Variables|Default|GetSphere))
  (bind _returnvalue (Transformation|GetWorldLocation _sphere))
  (if (Variables|Default|GetIsBallLaunch)
    (bind _outhit (Collision|LineTraceByChannel _returnvalue (+ _returnvalue (* (Math|Vector|GetUpVector (Variables|Default|GetSphere)) -75)) "TraceTypeQuery1" false 0 "None"))
    (if (== (.HitActor (Collision|BreakHitResult _outhit)) (Variables|Default|GetBPCube))
      (Utilities|FlowControl|Delay 0.2)
      (Variables|Default|SetIsBallLaunch false))))

(event EventSetCharacterinInteract
  (params (Player :type Character%20Player%20Object%20Reference))
  (Variables|Default|SetPlayerIn Player))

(event EventOnInteract
  (params (Player :type Character%20Player%20Object%20Reference) (InputID :type EInputID%20Enum :default "QTE1")))

(event EventOnStartInteract
  (params (Player :type Character%20Player%20Object%20Reference) (InputID :type EInputID%20Enum :default "QTE1"))
  (bind _returnvalue (Transformation|GetActorForwardVector Player))
  (bind _returnvalue_2 (* _returnvalue 1000))
  (Variables|Default|SetPlayer Player)
  (switch Utilities|FlowControl|Switch|SwitchonEInputID InputID
    (:QTE1
      (if (not (Variables|Default|GetIsBallLaunch))
        (if (Variables|Default|GetIsBallGrab)
          (Transformation|DetachFromActor "KeepWorld" "KeepRelative" "KeepRelative")
          (Physics|SetSimulatePhysics (Variables|Default|GetSphere) true)
          (Variables|Default|SetIsBallGrab false)
          (else
            (bind _returnvalue_3 (Class|CharacterPlayer|GetGrabParent Player))
            (Transformation|AttachComponentToComponent _returnvalue_3 "None" "SnapToTarget" "KeepRelative" "KeepWorld" true)
            (Variables|/Script/CouchGame.CharacterPlayer|SetInteractableActor Player self)
            (Variables|Default|SetIsBallGrab true)))))
    (:QTE2
      (if (not (Variables|Default|GetIsBallLaunch))
        (if (Variables|Default|GetIsBallGrab)
          (Transformation|DetachFromActor "KeepWorld" "KeepWorld" "KeepRelative")
          (Physics|SetSimulatePhysics (Variables|Default|GetSphere) true)
          (Physics|SetPhysicsLinearVelocity (Variables|Default|GetSphere) (Math|Vector|MakeVector (.x _returnvalue_2) (.y _returnvalue_2) 1e+03) false "None")
          (Utilities|FlowControl|Delay 0.2)
          (Variables|Default|SetIsBallLaunch true)
          (Variables|Default|SetIsBallGrab false)
          (else
            (Physics|SetPhysicsLinearVelocity (Variables|Default|GetSphere) (* (Transformation|GetActorForwardVector Player) 1000) false "None")))))))

(event EventBeginPlay
  (bind _returnvalue (Actor|GetActorOfClass "/Script/CouchGame.CubeController"))
  (bind _asbp_cube (Utilities|Casting|CastToBP_Cube _returnvalue))
  (Variables|Default|SetBPCube _asbp_cube))

(event EventOnEndInteract
  (params (Player :type Character%20Player%20Object%20Reference) (InputID :type EInputID%20Enum :default "QTE1")))

(fn ConstructionScript)

(fn GetCharacterinInteract
  (return 0))

(fn GetInteractWidget
  (return 0))

(fn GetPlayerLockParent
  (return 0))

(fn GetUnlockTP
  (return 0))

(fn IsPlayerLocked
  (return false))

(fn LockedPlayer
  (return false))
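; Interactable swing that runs a timing minigame: one player is locked on it while another presses QTE1 to keep it going.
; A timeline rotates the pivot and opens an input window; each hit restarts it, five hits win, and a run that finishes resets the count.
; While occupied, Tick reattaches the seated player, snaps them to the lock point and copies their rotation onto the swing actor.
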(event Custom|StopSwing
  ;[0.15 0.15 0.15 0.5] OnStartInteract
  (bind _rotation_1 (Timeline|TimelineSwing Stop)
    (:Update
      (Transformation|SetRelativeRotation (Variables|Default|GetPivot) (Math|Rotator|MakeRotator (* _rotation_1 (Variables|Default|GetValueRotation)) 0.0 0.0) false false))
    (:Finished
      (Development|PrintString "END")
      (Variables|Default|SetIsGameSwing false)
      (Variables|Default|SetCanInput false)
      (Variables|Default|SetValueGame 0))
    (:QTE_Start
      (Development|PrintString "Start")
      (Variables|Default|SetHasInput false)
      (Variables|Default|SetCanInput true))
    (:QTE_END
      (Development|PrintString "QTE END")
      (if (Variables|Default|GetHasInput)
        (CallFunction|StopSwing)
        (bind _result (Math|Integer|IncrementInt (Variables|Default|GetValueGame))
          (:%20%20
            (if (>= _result 5)
              (Development|PrintString "FIN DE LA GAME")
              (Variables|Default|SetIsGameSwing false)
              (Variables|Default|SetValueGame 0)
              (CallFunction|CESucces)
              (else
                (CallFunction|RetryPlayer)
                (Development|PrintString (Utilities|String|ToString(Integer) (Variables|Default|GetValueGame)))))))))))

(event Custom|RetryPlayer
  ;[0.15 0.15 0.15 0.5] OnStartInteract
  (bind _rotation_1 (Timeline|TimelineSwing PlayFromStart)
    (:Update
      (Transformation|SetRelativeRotation (Variables|Default|GetPivot) (Math|Rotator|MakeRotator (* _rotation_1 (Variables|Default|GetValueRotation)) 0.0 0.0) false false))
    (:Finished
      (Development|PrintString "END")
      (Variables|Default|SetIsGameSwing false)
      (Variables|Default|SetCanInput false)
      (Variables|Default|SetValueGame 0))
    (:QTE_Start
      (Development|PrintString "Start")
      (Variables|Default|SetHasInput false)
      (Variables|Default|SetCanInput true))
    (:QTE_END
      (Development|PrintString "QTE END")
      (if (Variables|Default|GetHasInput)
        (CallFunction|StopSwing)
        (bind _result (Math|Integer|IncrementInt (Variables|Default|GetValueGame))
          (:%20%20
            (if (>= _result 5)
              (Development|PrintString "FIN DE LA GAME")
              (Variables|Default|SetIsGameSwing false)
              (Variables|Default|SetValueGame 0)
              (CallFunction|CESucces)
              (else
                (CallFunction|RetryPlayer)
                (Development|PrintString (Utilities|String|ToString(Integer) (Variables|Default|GetValueGame)))))))))))

(event Custom|CE_Succes
  ;[0.15 0.15 0.15 0.5] SUCESS GAME
  (Development|PrintString "GAME REUSSIE" true true "(R=0.019072,G=1.000000,B=0.000000,A=1.000000)")
  (Class|PlayerStateMachine|ChangeState (Variables|/Script/CouchGame.CharacterPlayer|GetStateMachine (Variables|Default|GetPlayerIn)) "Idle"))

(event EventOnStartInteract
  (params (Player :type Character%20Player%20Object%20Reference) (InputID :type EInputID%20Enum :default "QTE1"))
  ;[0.15 0.15 0.15 0.5] OnStartInteract
  (switch Utilities|FlowControl|Switch|SwitchonEInputID InputID
    (:QTE1
      (bind _returnvalue (CallFunction|IsPlayerLocked))
      (if _returnvalue
        (if (not (== Player (Variables|Default|GetPlayerIn)))
          (Development|PrintString (Utilities|String|ToString(Boolean) (Variables|Default|GetCanInput)) true true "(R=1.000000,G=0.000000,B=0.971819,A=1.000000)")
          (if (Variables|Default|GetCanInput)
            (Development|PrintString "INPUT" true true "(R=1.000000,G=0.630659,B=0.000000,A=1.000000)")
            (Variables|Default|SetHasInput true)
            (Variables|Default|SetCanInput false)
            (elif (not (Variables|Default|GetIsGameSwing))
              (Variables|Default|SetIsGameSwing true)
              (bind _rotation_1 (Timeline|TimelineSwing PlayFromStart)
                (:Update
                  (Transformation|SetRelativeRotation (Variables|Default|GetPivot) (Math|Rotator|MakeRotator (* _rotation_1 (Variables|Default|GetValueRotation)) 0.0 0.0) false false))
                (:Finished
                  (Development|PrintString "END")
                  (Variables|Default|SetIsGameSwing false)
                  (Variables|Default|SetCanInput false)
                  (Variables|Default|SetValueGame 0))
                (:QTE_Start
                  (Development|PrintString "Start")
                  (Variables|Default|SetHasInput false)
                  (Variables|Default|SetCanInput true))
                (:QTE_END
                  (Development|PrintString "QTE END")
                  (if (Variables|Default|GetHasInput)
                    (CallFunction|StopSwing)
                    (bind _result (Math|Integer|IncrementInt (Variables|Default|GetValueGame))
                      (:%20%20
                        (if (>= _result 5)
                          (Development|PrintString "FIN DE LA GAME")
                          (Variables|Default|SetIsGameSwing false)
                          (Variables|Default|SetValueGame 0)
                          (CallFunction|CESucces)
                          (else
                            (CallFunction|RetryPlayer)
                            (Development|PrintString (Utilities|String|ToString(Integer) (Variables|Default|GetValueGame)))))))))))))))))

(event EventTick
  (params (DeltaSeconds :type Float%20%28single-precision%29))
  ;[0.15 0.15 0.15 0.5] FIX POS PLAYER IN TICK
  (bind _returnvalue (CallFunction|IsPlayerLocked))
  (if _returnvalue
    (CallFunction|FixPlayer)))

(event EventOnEndInteract
  (params (Player :type Character%20Player%20Object%20Reference) (InputID :type EInputID%20Enum :default "QTE1"))
  ;[0.15 0.15 0.15 0.5] OnEndInteract
)

(event EventStartInteract
  (params (Player :type Character%20Player%20Object%20Reference))
  ;[0.15 0.15 0.15 0.5 20] StartInteract
  (Development|PrintString "Interact_Swing"))

(event EventSetCharacterinInteract
  (params (Player :type Character%20Player%20Object%20Reference))
  ;[0.15 0.15 0.15 0.5] SET CHARACTER INTERACT
  (Variables|Default|SetPlayerIn Player))

(fn ConstructionScript)

(fn FixPlayer
  (bind _playerin (Variables|Default|GetPlayerIn))
  (bind _tplock (Variables|Default|GetTpLock))
  (bind _returnvalue (Transformation|GetWorldLocation _tplock))
  (bind _rootcomponent (Variables|/Script/Engine.Actor|GetRootComponent _playerin))
  (bind _returnvalue_2 (Transformation|GetWorldRotation _rootcomponent))
  (bind (_roll _pitch _yaw) (Math|Rotator|BreakRotator _returnvalue_2))
  (Transformation|AttachActorToActor (Variables|Default|GetPlayerIn) self "" "KeepWorld" "KeepWorld" "KeepWorld" true)
  (Transformation|SetActorLocation (Variables|Default|GetPlayerIn) (Math|Vector|MakeVector (.x _returnvalue) (.y _returnvalue) (.z _returnvalue)) false false)
  (Transformation|SetActorRotation (Math|Rotator|MakeRotator _roll _pitch _yaw)))

(fn UnFixPlayer
  (params (LockTP :type Scene%20Component%20Object%20Reference))
  (bind _returnvalue (Transformation|GetWorldLocation LockTP))
  (Transformation|DetachFromActor (Variables|Default|GetPlayerIn) "KeepWorld" "KeepWorld" "KeepWorld")
  (Transformation|SetActorLocation (Variables|Default|GetPlayerIn) (Math|Vector|MakeVector (.x _returnvalue) (.y _returnvalue) (.z _returnvalue)) false false)
  (Variables|Default|SetPlayerIn 0))

(fn GetCharacterinInteract
  (return (Variables|Default|GetPlayerIn)))

(fn GetInteractWidget
  (return (Variables|Default|GetInteractWidget)))

(fn GetPlayerLockParent
  (return (Variables|Default|GetTpLock)))

(fn GetUnlockTP
  (return (Variables|Default|GetTpUnLock)))

(fn IsPlayerLocked
  (return (Utilities|IsValid (Variables|Default|GetPlayerIn))))

(fn LockedPlayer
  (return true))
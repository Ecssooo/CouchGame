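; Swing interactable where one player rides while another pushes through timed QTE presses.
; The rider attaches to PivotSwing and is held at TpLock as a timeline rotates the pivot, using a curve and duration from a settings class.
; Timeline events open the WBP_QTE input window; successful hits replay the swing until the required count saves completion through SaveCubeSubsystem.
; Once completed, successful hits simply keep the swing going.
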(event Custom|StopSwing
  ;[0.15 0.15 0.15 0.5] OnStartInteract
  (bind _swingcurve (Timeline|TimelineSwing Stop)
    (:Update
      (Transformation|SetRelativeRotation (Variables|Default|GetPivotSwing) (Math|Rotator|MakeRotator (* _swingcurve (Variables|Default|GetValueRotation)) 0.0 0.0) false false)
      (CallFunction|FixPlayer))
    (:Finished
      (Development|PrintString "END")
      (Variables|Default|SetIsGameSwing false)
      (Variables|Default|SetCanInput false)
      (Variables|Default|SetValueGame 0))
    (:QTE_Start
      (Development|PrintString "Start")
      (Variables|Default|SetHasInput false)
      (Variables|Default|SetCanInput true)
      (CallFunction|CEPlayQTE 1.95))
    (:QTE_END
      (Development|PrintString "QTE END")
      (if (Variables|Default|GetHasInput)
        (bind _returnvalue (Class|SaveCubeSubsystem|GetInteractionsDatasfromID (Subsystems|GetSaveCubeSubsystem) 101))
        (if (.iscompleted _returnvalue)
          (CallFunction|RetryPlayer :!label _label)
          (else
            (CallFunction|StopSwing)
            (bind _result (Math|Integer|IncrementInt (Variables|Default|GetValueGame))
              (:%20%20
                (if (>= _result (Variables|Default|GetNbMouvementSwing))
                  (Development|PrintString "FIN DE LA GAME")
                  (Variables|Default|SetIsGameSwing false)
                  (Variables|Default|SetValueGame 0)
                  (CallFunction|CESucces)
                  (else
                    (goto _label)))))))))))

(event Custom|CE_SetOutline
  (params (Isenable :type Boolean))
  ;[0.15 0.15 0.15 0.5] Highlight
  (Rendering|SetRenderCustomDepth (Variables|Default|GetStructure) Isenable))

(event Custom|CE_RotationWidget
  (bind _worldcamera (Variables|Default|GetWorldCamera))
  (bind _widget (Variables|Default|GetWidget))
  (bind _returnvalue (Transformation|GetWorldLocation _widget))
  (bind _rootcomponent (Variables|/Script/Engine.Actor|GetRootComponent _worldcamera))
  (bind _returnvalue_2 (Transformation|GetWorldLocation _rootcomponent))
  (bind _returnvalue_3 (Math|Rotator|FindLookatRotation _returnvalue _returnvalue_2))
  (Transformation|SetWorldRotation (Variables|Default|GetWidget) (Math|Rotator|MakeRotator (.roll (Transformation|GetWorldRotation _widget)) (.pitch _returnvalue_3) (.yaw _returnvalue_3)) false false))

(event Custom|CE_Succes
  ;[0.15 0.15 0.15 0.5] SUCESS GAME
  (Development|PrintString "GAME REUSSIE" true true "(R=0.019072,G=1.000000,B=0.000000,A=1.000000)")
  (Class|PlayerStateMachine|ChangeState (Variables|/Script/CouchGame.CharacterPlayer|GetStateMachine (Variables|Default|GetPlayerIn)) "Idle")
  (Class|SaveCubeSubsystem|SaveInteractionData (Subsystems|GetSaveCubeSubsystem) 101 true))

(event Custom|RetryPlayer
  ;[0.15 0.15 0.15 0.5] OnStartInteract
  (bind _swingcurve (Timeline|TimelineSwing PlayFromStart)
    (:Update
      (Transformation|SetRelativeRotation (Variables|Default|GetPivotSwing) (Math|Rotator|MakeRotator (* _swingcurve (Variables|Default|GetValueRotation)) 0.0 0.0) false false)
      (CallFunction|FixPlayer))
    (:Finished
      (Development|PrintString "END")
      (Variables|Default|SetIsGameSwing false)
      (Variables|Default|SetCanInput false)
      (Variables|Default|SetValueGame 0))
    (:QTE_Start
      (Development|PrintString "Start")
      (Variables|Default|SetHasInput false)
      (Variables|Default|SetCanInput true)
      (CallFunction|CEPlayQTE 1.95))
    (:QTE_END
      (Development|PrintString "QTE END")
      (if (Variables|Default|GetHasInput)
        (bind _returnvalue (Class|SaveCubeSubsystem|GetInteractionsDatasfromID (Subsystems|GetSaveCubeSubsystem) 101))
        (if (.iscompleted _returnvalue)
          (CallFunction|RetryPlayer :!label _label)
          (else
            (CallFunction|StopSwing)
            (bind _result (Math|Integer|IncrementInt (Variables|Default|GetValueGame))
              (:%20%20
                (if (>= _result (Variables|Default|GetNbMouvementSwing))
                  (Development|PrintString "FIN DE LA GAME")
                  (Variables|Default|SetIsGameSwing false)
                  (Variables|Default|SetValueGame 0)
                  (CallFunction|CESucces)
                  (else
                    (goto _label)))))))))))

(event Custom|CE_PlayQTE
  (params (TimerQTE :type Float%20%28double-precision%29))
  ;[0.15 0.15 0.15 0.5] Play QTE
  (Variables|Default|SetIsPlayable true)
  (CallFunction|ShowQTE)
  (Default|PlayQTE (Variables|Default|GetAs%20WBP%20QTE) TimerQTE))

(event Custom|CE_StopQTE
  ;[0.15 0.15 0.15 0.5] STOP QTE
  (Variables|Default|SetIsPlayable false)
  (CallFunction|HideQTE)
  (Default|FClickQTE (Variables|Default|GetAs%20WBP%20QTE)))

(event EventOnStartInteract
  (params (Player :type Character%20Player%20Object%20Reference) (InputID :type EInputID%20Enum :default "QTE1"))
  ;[0.15 0.15 0.15 0.5] OnStartInteract
  (switch Utilities|FlowControl|Switch|SwitchonEInputID InputID
    (:QTE1
      (bind _returnvalue (CallFunction|IsPlayerLocked))
      (if _returnvalue
        (if (not (== Player (Variables|Default|GetPlayerIn)))
          (if (Variables|Default|GetCanInput)
            (Variables|Default|SetCanInput false)
            (bind _win (Default|FClickQTE (Variables|Default|GetAs%20WBP%20QTE)))
            (Variables|Default|SetHasInput _win)
            (elif (not (Variables|Default|GetIsGameSwing))
              (Variables|Default|SetIsGameSwing true)
              (bind _swingcurve (Timeline|TimelineSwing PlayFromStart)
                (:Update
                  (Transformation|SetRelativeRotation (Variables|Default|GetPivotSwing) (Math|Rotator|MakeRotator (* _swingcurve (Variables|Default|GetValueRotation)) 0.0 0.0) false false)
                  (CallFunction|FixPlayer))
                (:Finished
                  (Development|PrintString "END")
                  (Variables|Default|SetIsGameSwing false)
                  (Variables|Default|SetCanInput false)
                  (Variables|Default|SetValueGame 0))
                (:QTE_Start
                  (Development|PrintString "Start")
                  (Variables|Default|SetHasInput false)
                  (Variables|Default|SetCanInput true)
                  (CallFunction|CEPlayQTE 1.95))
                (:QTE_END
                  (Development|PrintString "QTE END")
                  (if (Variables|Default|GetHasInput)
                    (bind _returnvalue_2 (Class|SaveCubeSubsystem|GetInteractionsDatasfromID (Subsystems|GetSaveCubeSubsystem) 101))
                    (if (.iscompleted _returnvalue_2)
                      (CallFunction|RetryPlayer :!label _label)
                      (else
                        (CallFunction|StopSwing)
                        (bind _result (Math|Integer|IncrementInt (Variables|Default|GetValueGame))
                          (:%20%20
                            (if (>= _result (Variables|Default|GetNbMouvementSwing))
                              (Development|PrintString "FIN DE LA GAME")
                              (Variables|Default|SetIsGameSwing false)
                              (Variables|Default|SetValueGame 0)
                              (CallFunction|CESucces)
                              (else
                                (goto _label)))))))))))))))))

(event EventTick
  (params (DeltaSeconds :type Float%20%28single-precision%29))
  ;[0.15 0.15 0.15 0.5] FIX POS PLAYER IN TICK
  (bind _returnvalue (CallFunction|IsPlayerLocked))
  (if _returnvalue
    (CallFunction|FixPlayer)
    (if (Variables|Default|GetIsVisible)
      (bind _isrunning (Default|FGetIsRunning (Variables|Default|GetAs%20WBP%20QTE)))
      (if (not _isrunning)
        (CallFunction|HideQTE)))))

(event EventOnEndInteract
  (params (Player :type Character%20Player%20Object%20Reference) (InputID :type EInputID%20Enum :default "QTE1"))
  ;[0.15 0.15 0.15 0.5] OnEndInteract
)

(event EventStartInteract
  (params (Player :type Character%20Player%20Object%20Reference))
  ;[0.15 0.15 0.15 0.5 20] StartInteract
  (CallFunction|CERotationWidget)
  (Development|PrintString "Interact_Swing")
  (Utilities|FlowControl|Delay 0.1)
  (Transformation|AttachComponentToComponent (Variables|Default|GetPlayerIn) (Variables|Default|GetPivotSwing) "None" "KeepWorld" "KeepWorld" "KeepWorld" true)
  (CallFunction|ShowQTE)
  (bind _returnvalue (Class|CharacterPlayer|GetBlueprintAnim (Variables|Default|GetPlayerIn)))
  (Class|BPIAnim|PlayInteract(Message) _returnvalue "NewEnumerator0"))

(event EventBeginPlay
  (bind (_swingcurve _swingduration) (Utilities|GetClassDefaults "/Script/CouchGame.TimelineSettings"))
  (bind _aswbp_qte (Utilities|Casting|CastToWBP_QTE (UserInterface|GetUserWidgetObject (Variables|Default|GetWidget))))
  (Variables|Default|SetAs%20WBP%20QTE _aswbp_qte)
  (bind _returnvalue (Actor|GetActorOfClass "/Game/BP/Camera/BP_CameraActor.BP_CameraActor_C"))
  (Variables|Default|SetWorldCamera _returnvalue)
  (bind _returnvalue_2 (Actor|GetActorOfClass "/Game/BP/Steps/Face1/BP_StepManager.BP_StepManager_C"))
  (Variables|Default|SetStepManager _returnvalue_2)
  (Class|TimelineComponent|SetFloatCurve (Variables|Default|GetTimelineSwing) (Utilities|ResolveSoftReference _swingcurve) "SwingCurve")
  (Components|Timeline|SetPlayRate (Variables|Default|GetTimelineSwing) (Math|Float|SafeDivide 1.0 _swingduration)))

(event EventSetCharacterinInteract
  (params (Player :type Character%20Player%20Object%20Reference))
  ;[0.15 0.15 0.15 0.5] SET CHARACTER INTERACT
  (Variables|Default|SetPlayerIn Player))

(event EventEndInteract
  (params (Player :type Character%20Player%20Object%20Reference))
  (bind _playerin (Variables|Default|GetPlayerIn))
  ;[0.15 0.15 0.15 0.5] END Interact
  (CallFunction|HideQTE)
  (bind _returnvalue (Class|CharacterPlayer|GetBlueprintAnim _playerin))
  (Class|Interactable|EndInteract(Message) _returnvalue _playerin))

(event EventHighlightInteraction
  (params (IsHighlight :type Boolean))
  ;[0.15 0.15 0.15 0.5] Highlight
  (CallFunction|CESetOutline IsHighlight))

(fn ConstructionScript)

(fn FixPlayer
  (bind _tplock (Variables|Default|GetTpLock))
  (bind _pivotswing (Variables|Default|GetPivotSwing))
  (bind _returnvalue (Transformation|GetWorldLocation _tplock))
  (bind _returnvalue_2 (Transformation|GetWorldRotation _pivotswing))
  (bind (_roll _pitch _yaw) (Math|Rotator|BreakRotator _returnvalue_2))
  (bind _playerin (Variables|Default|GetPlayerIn)
    (:then
      (Transformation|SetActorLocation _playerin (Math|Vector|MakeVector (.x _returnvalue) (.y _returnvalue) (.z _returnvalue)) false false)
      (Transformation|SetActorRotation (Variables|Default|GetPlayerIn) (Math|Rotator|MakeRotator 0.0 (* _roll -1.0) (+ _yaw 9e+01))))
    (:else)))

(fn UnFixPlayer
  (params (LockTP :type Scene%20Component%20Object%20Reference))
  (bind _returnvalue (Transformation|GetWorldLocation LockTP))
  (Transformation|DetachFromActor (Variables|Default|GetPlayerIn) "KeepWorld" "KeepWorld" "KeepWorld")
  (Transformation|SetActorLocation (Variables|Default|GetPlayerIn) (Math|Vector|MakeVector (.x _returnvalue) (.y _returnvalue) (.z _returnvalue)) false false)
  (Variables|Default|SetPlayerIn 0))

(fn ShowQTE
  (Variables|Default|SetIsVisible true)
  (Rendering|SetVisibility (Variables|Default|GetWidget) true false))

(fn HideQTE
  (Variables|Default|SetIsVisible false)
  (Rendering|SetVisibility (Variables|Default|GetWidget) false false))

(fn GetCharacterinInteract
  (return (Variables|Default|GetPlayerIn)))

(fn GetInteractWidget
  (bind _returnvalue (CallFunction|IsPlayerLocked))
  (if _returnvalue
    (return "/Game/BP/Widget/WBP_InteractY.WBP_InteractY_C")
    (else
      (return (Variables|Default|GetInteractWidget)))))

(fn GetPlayerLockParent
  (return (Variables|Default|GetTpLock)))

(fn GetUnlockTP
  (return (Variables|Default|GetTpUnLock)))

(fn IsPlayerLocked
  (return (Utilities|IsValid (Variables|Default|GetPlayerIn))))

(fn LockedPlayer
  (return true))
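; Interaction point on the swing (balançoire) that serves as the lock spot for a second player.
; It starts disabled, and an activation event toggles its box collision and cube visibility together.
; Start, ongoing and end interact calls are forwarded to the referenced Swing.
; It tracks the occupying player to report locked state and exposes components for the lock parent and unlock teleport.
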(event Custom|CE_ActiveInteraction
  (params (IsActive :type Boolean))
  (bind _box (Variables|Default|GetBox))
  (if IsActive
    (Collision|SetCollisionEnabled _box "QueryAndPhysics")
    (Rendering|SetVisibility (Variables|Default|GetCube) true false)
    (else
      (Collision|SetCollisionEnabled _box "NoCollision")
      (Rendering|SetVisibility (Variables|Default|GetCube) false false))))

(event EventOnStartInteract
  (params (Player :type Character%20Player%20Object%20Reference) (InputID :type EInputID%20Enum :default "QTE1"))
  (Default|OnStartInteract (Variables|Default|GetSwing) Player InputID))

(event EventOnInteract
  (params (Player :type Character%20Player%20Object%20Reference) (InputID :type EInputID%20Enum :default "QTE1"))
  (Default|OnInteract (Variables|Default|GetSwing) Player InputID))

(event EventOnEndInteract
  (params (Player :type Character%20Player%20Object%20Reference) (InputID :type EInputID%20Enum :default "QTE1"))
  (Default|OnEndInteract (Variables|Default|GetSwing) Player InputID))

(event EventSetCharacterinInteract
  (params (Player :type Character%20Player%20Object%20Reference))
  (Variables|Default|SetPlayerIn Player))

(event EventEndInteract
  (params (Player :type Character%20Player%20Object%20Reference))
  (Variables|Default|SetPlayerIn 0))

(event EventBeginPlay
  (CallFunction|CEActiveInteraction false))

(fn ConstructionScript)

(fn GetCharacterinInteract
  (return (Variables|Default|GetPlayerIn)))

(fn GetInteractWidget
  (return 0))

(fn GetPlayerLockParent
  (return (Variables|Default|GetLockPlayer)))

(fn GetUnlockTP
  (return (Variables|Default|GetUnlockPlayer)))

(fn IsPlayerLocked
  (return (Utilities|IsValid (Variables|Default|GetPlayerIn))))

(fn LockedPlayer
  (return true))
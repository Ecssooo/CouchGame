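; BP_SwingTest is an interactable physics swing that a player can be locked to and push with a QTE input.
; On BeginPlay, the Lock component attaches to the seat bone of RigSwing so it follows the swing.
; The QTE1 input adds a fixed velocity-change impulse to that bone.
; Interaction functions store the player and expose the lock and unlock points, while the character and widget getters are empty.
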(event EventStartInteract
  (params (Player :type Character%20Player%20Object%20Reference))
  (Variables|Default|SetPlayerIn Player))

(event EventBeginPlay
  (Transformation|AttachComponentToComponent (Variables|Default|GetLock) (Variables|Default|GetRig_Swing) "BNS_Swing_Seat" "KeepWorld" "KeepWorld" "KeepWorld" true))

(event EventSetCharacterinInteract
  (params (Player :type Character%20Player%20Object%20Reference))
  (Variables|Default|SetPlayerIn Player))

(event EventOnStartInteract
  (params (Player :type Character%20Player%20Object%20Reference) (InputID :type EInputID%20Enum :default "QTE1"))
  (bind _rig_swing (Variables|Default|GetRig_Swing))
  (switch Utilities|FlowControl|Switch|SwitchonEInputID InputID
    (:QTE1
      (Class|PrimitiveComponent|AddVelocityChangeImpulseatLocation _rig_swing "0.000000,150.000000,0.000000" (Transformation|GetWorldLocation _rig_swing) "BNS_Swing_Seat"))))

(fn ConstructionScript)

(fn GetCharacterinInteract
  (return 0))

(fn GetInteractWidget
  (return 0))

(fn GetPlayerLockParent
  (return (Variables|Default|GetLock)))

(fn GetUnlockTP
  (return (Variables|Default|GetUnlock)))

(fn IsPlayerLocked
  (return (Utilities|IsValid (Variables|Default|GetPlayerIn))))

(fn LockedPlayer
  (return true))
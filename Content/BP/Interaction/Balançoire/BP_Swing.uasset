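; Playground swing that one player can sit on while another player, not seated, pushes it through the interaction system.
; An overlap box registers the swing as the player's current interact object, and entry interaction attaches or detaches the rider and toggles their movement.
; Start interaction loops a timeline that rolls the pivot and re-snaps the rider to the seat.
; Stopping halts it, then resumes without looping after a short delay.
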(event OnComponentBeginOverlap(Box_InteractionZone)
  (params (OverlappedComponent :type Primitive%20Component%20Object%20Reference) (OtherActor :type Actor%20Object%20Reference) (OtherComp :type Primitive%20Component%20Object%20Reference) (OtherBodyIndex :type Integer) (bFromSweep :type Boolean) (SweepResult :type Hit%20Result%20Structure%20%28by%20ref%29))
  ;[0.15 0.15 0.15 0.5] Overlap Player with Swing
  (bind _asbp_character_player (Utilities|Casting|CastToBP_CharacterPlayer OtherActor))
  (Utilities|Array|Add (Variables|Default|GetPlayer) _asbp_character_player)
  (Variables|/Game/BP/Player/BP_CharacterPlayer.BP_CharacterPlayer_C|SetCurrentInteractObject _asbp_character_player self))

(event OnComponentEndOverlap(Box_InteractionZone)
  (params (OverlappedComponent :type Primitive%20Component%20Object%20Reference) (OtherActor :type Actor%20Object%20Reference) (OtherComp :type Primitive%20Component%20Object%20Reference) (OtherBodyIndex :type Integer))
  ;[0.15 0.15 0.15 0.5] Overlap Player with Swing
  (bind _asbp_character_player (Utilities|Casting|CastToBP_CharacterPlayer OtherActor))
  (Utilities|Array|RemoveItem (Variables|Default|GetPlayer) _asbp_character_player)
  (Variables|/Game/BP/Player/BP_CharacterPlayer.BP_CharacterPlayer_C|SetCurrentInteractObject _asbp_character_player 0))

(event Custom|CE_Reverse
  ;[0.15 0.15 0.15 0.5] Launch / Stop Swing
  (Utilities|FlowControl|Delay 0.1)
  (Components|Timeline|SetLooping (Variables|Default|GetTimelineSwing) false)
  (bind _rotation_1 (Timeline|TimelineSwing Play)
    (:Update
      (Transformation|SetRelativeRotation (Variables|Default|GetPivot) (Math|Rotator|MakeRotator (* _rotation_1 (Variables|Default|GetValueRotation)) 0.0 0.0) false false)
      (CallFunction|SetPosPlayerSwing))
    (:Finished
      (Variables|Default|SetisOnSwing false))))

(event Custom|CE_Stop
  ;[0.15 0.15 0.15 0.5] Launch / Stop Swing
  (Development|PrintString "OFF Swing")
  (Variables|Default|SetisOnSwing false)
  (CallFunction|CEReverse)
  (bind _rotation_1 (Timeline|TimelineSwing Stop)
    (:Update
      (Transformation|SetRelativeRotation (Variables|Default|GetPivot) (Math|Rotator|MakeRotator (* _rotation_1 (Variables|Default|GetValueRotation)) 0.0 0.0) false false)
      (CallFunction|SetPosPlayerSwing))
    (:Finished
      (Variables|Default|SetisOnSwing false))))

(event EventEntryInteract
  (params (Player :type BP%20Character%20Player%20Object%20Reference))
  ;[0.15 0.15 0.15 0.5] Entry / Swing
  (bind _output_get (Variables|Default|SetPlayerActorTemporary Player))
  (if (Variables|Default|GetisPlayerIn)
    (if (Variables|/Game/BP/Player/BP_CharacterPlayer.BP_CharacterPlayer_C|GetIsInSwing (Variables|Default|GetPlayerInSwing))
      (if (== (Variables|Default|GetPlayerInSwing) _output_get)
        (Default|PlayerLeaveSwing (Variables|Default|GetPlayerInSwing))
        (CallFunction|UndoPosPlayerSwing))
      (else
        (Default|PlayerLeaveSwing (Variables|Default|GetPlayerActorTemporary))
        (CallFunction|UndoPosPlayerSwing)
        (Development|PrintString "Player Exit Swing" true true "(R=1.000000,G=0.000000,B=0.034294,A=1.000000)")))
    (else
      (Variables|Default|SetPlayerInSwing (Variables|Default|GetPlayerActorTemporary))
      (CallFunction|SetPosPlayerSwing)
      (Variables|Default|SetisPlayerIn true)
      (Variables|/Game/BP/Player/BP_CharacterPlayer.BP_CharacterPlayer_C|SetIsInSwing (Variables|Default|GetPlayerInSwing) true)
      (Development|PrintString "Player Entry in Swing" true true "(R=0.031144,G=1.000000,B=0.000000,A=1.000000)"))))

(event EventStartInteract
  (params (Player :type BP%20Character%20Player%20Object%20Reference))
  ;[0.15 0.15 0.15 0.5] Launch / Stop Swing
  (bind _output_get (Variables|Default|SetPlayerActivateSwing Player))
  (if (not (Variables|/Game/BP/Player/BP_CharacterPlayer.BP_CharacterPlayer_C|GetIsInSwing _output_get))
    (if (Variables|Default|GetisPlayerIn)
      (Development|PrintString "ON Launch")
      (Variables|Default|SetisOnSwing true)
      (Components|Timeline|SetLooping (Variables|Default|GetTimelineSwing) true)
      (bind _rotation_1 (Timeline|TimelineSwing Play)
        (:Update
          (Transformation|SetRelativeRotation (Variables|Default|GetPivot) (Math|Rotator|MakeRotator (* _rotation_1 (Variables|Default|GetValueRotation)) 0.0 0.0) false false)
          (CallFunction|SetPosPlayerSwing))
        (:Finished
          (Variables|Default|SetisOnSwing false)))
      (elif (Variables|Default|GetisOnSwing)
        (Development|PrintString "You can't launch")
        (CallFunction|CEStop)
        (else
          (Development|PrintString "You can't launch"))))))

(event EventStopInteract
  (params (Player :type BP%20Character%20Player%20Object%20Reference))
  ;[0.15 0.15 0.15 0.5] Launch / Stop Swing
  (if (not (Variables|/Game/BP/Player/BP_CharacterPlayer.BP_CharacterPlayer_C|GetIsInSwing (Variables|Default|GetPlayerActivateSwing)))
    (if (Variables|Default|GetisPlayerIn)
      (Development|PrintString "OFF Swing")
      (Variables|Default|SetisOnSwing false)
      (CallFunction|CEReverse)
      (bind _rotation_1 (Timeline|TimelineSwing Stop)
        (:Update
          (Transformation|SetRelativeRotation (Variables|Default|GetPivot) (Math|Rotator|MakeRotator (* _rotation_1 (Variables|Default|GetValueRotation)) 0.0 0.0) false false)
          (CallFunction|SetPosPlayerSwing))
        (:Finished
          (Variables|Default|SetisOnSwing false)))
      (else
        (Development|PrintString "can't SWING" true true "(R=1.000000,G=0.000000,B=0.047706,A=1.000000)")))))

(fn ConstructionScript)

(fn SetPosPlayerSwing
  (bind _playerinswing (Variables|Default|GetPlayerInSwing))
  (bind _setposplayer (Variables|Default|GetSetPosPlayer))
  (bind _returnvalue (Transformation|GetWorldLocation _setposplayer))
  (bind _rootcomponent (Variables|/Script/Engine.Actor|GetRootComponent _playerinswing))
  (bind _returnvalue_2 (Transformation|GetWorldRotation _rootcomponent))
  (bind (_roll _pitch _yaw) (Math|Rotator|BreakRotator _returnvalue_2))
  (Transformation|AttachActorToActor (Variables|Default|GetPlayerInSwing) self "" "KeepWorld" "KeepWorld" "KeepWorld" true)
  (Transformation|SetActorLocation (Variables|Default|GetPlayerInSwing) (Math|Vector|MakeVector (.x _returnvalue) (.y _returnvalue) (.z _returnvalue)) false false)
  (Transformation|SetActorRotation (Variables|Default|GetPlayerInSwing) (Math|Rotator|MakeRotator _roll _pitch _yaw))
  (Pawn|Components|CharacterMovement|SetMovementMode (Variables|/Script/Engine.Character|GetCharacterMovement (Variables|Default|GetPlayerInSwing)) "MOVE_None" 0))

(fn UndoPosPlayerSwing
  (Transformation|DetachFromActor (Variables|Default|GetPlayerInSwing) "KeepWorld" "KeepWorld" "KeepWorld")
  (Pawn|Components|CharacterMovement|SetMovementMode (Variables|/Script/Engine.Character|GetCharacterMovement (Variables|Default|GetPlayerInSwing)) "MOVE_Walking" 0)
  (Variables|Default|SetisPlayerIn false)
  (Variables|Default|SetPlayerInSwing 0))
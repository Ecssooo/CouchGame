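; BP_GoToFace3 is a trigger actor that completes the "GoToFace3" step of a step sequence when the player reaches it.
; On BeginPlay it finds and caches the level's BP_StepManager.
; When BP_Player1 overlaps its Box, it checks that the manager's current step is named "GoToFace3" and then calls NextStep to advance the sequence.
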(event OnComponentBeginOverlap(Box)
  (params (OverlappedComponent :type Primitive%20Component%20Object%20Reference) (OtherActor :type Actor%20Object%20Reference) (OtherComp :type Primitive%20Component%20Object%20Reference) (OtherBodyIndex :type Integer) (bFromSweep :type Boolean) (SweepResult :type Hit%20Result%20Structure%20%28by%20ref%29))
  (bind _stepmanager (Variables|Default|GetStepManager))
  (if (== OtherActor "/Game/BP/Player/BP_Player1.BP_Player1")
    (if (== (Variables|/Script/CouchGame.Step|GetStepName (Utilities|Array|Get(acopy) (Variables|/Script/CouchGame.StepManager|GetListStep _stepmanager) (Variables|/Script/CouchGame.StepManager|GetIndexStep _stepmanager))) "GoToFace3")
      (Class|StepManager|NextStep (Variables|Default|GetStepManager)))))

(event EventBeginPlay
  (bind _returnvalue (Actor|GetActorOfClass "/Game/BP/Steps/BP_StepManager.BP_StepManager_C"))
  (Variables|Default|SetStepManager _returnvalue))

(fn ConstructionScript)
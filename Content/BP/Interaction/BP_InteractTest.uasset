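; BP_InteractTest is a test interactable that exercises interaction start and end with debug prints.
; StartInteract stores the interacting player and prints a message, while EndInteract only prints, leaving that reference set.
; Query functions expose the stored player and the lock and unlock parents.
; LockedPlayer always returns true, and IsPlayerLocked simply checks whether the stored player is valid.
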(event EventBeginPlay)

(event Collision|EventActorBeginOverlap
  (params (OtherActor :type Actor%20Object%20Reference)))

(event EventTick
  (params (DeltaSeconds :type Float%20%28single-precision%29)))

(event EventStartInteract
  (params (Player :type Character%20Player%20Object%20Reference))
  (Variables|Default|SetPlayerInInteract Player)
  (Development|PrintString "StartInteractable"))

(event EventEndInteract
  (params (Player :type Character%20Player%20Object%20Reference))
  (Development|PrintString "EndInteract"))

(fn ConstructionScript)

(fn GetCharacterinInteract
  (return (Variables|Default|GetPlayerInInteract)))

(fn GetPlayerLockParent
  (return (Variables|Default|GetLockedParents)))

(fn GetUnlockTP
  (return (Variables|Default|GetUnlockParents)))

(fn IsPlayerLocked
  (return (Utilities|IsValid (Variables|Default|GetPlayerInInteract))))

(fn LockedPlayer
  (return true))
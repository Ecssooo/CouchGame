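; Physics football for the cage football interaction that resets itself when left untouched by a player for a set time.
; On BeginPlay it stores the Sphere's start position and starts a TimeBeforeTP timer, which restarts whenever a BP_CharacterPlayer overlaps the Box.
; The CE_TP event, apparently the timer's callback, moves the actor back to the start position and zeroes the Sphere's linear and angular velocity.
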(event OnComponentBeginOverlap(Box)
  (params (OverlappedComponent :type Primitive%20Component%20Object%20Reference) (OtherActor :type Actor%20Object%20Reference) (OtherComp :type Primitive%20Component%20Object%20Reference) (OtherBodyIndex :type Integer) (bFromSweep :type Boolean) (SweepResult :type Hit%20Result%20Structure%20%28by%20ref%29))
  ;[0.15 0.15 0.15 0.5] BEGIN OVERLAP
  (bind _asbp_character_player (Utilities|Casting|CastToBP_CharacterPlayer OtherActor))
  (Utilities|IsValid _asbp_character_player
    (:Is%20Valid
      (Utilities|Time|ClearandInvalidateTimerbyHandle (Variables|Default|GetTimerEventTP))
      (CallFunction|CETimer))))

(event Custom|CE_Timer
  ;[0.15 0.15 0.15 0.5] CE TIMER
  (bind _returnvalue (Utilities|Time|SetTimerbyEvent (EventDispatchers|CreateEvent :!event Custom|CE_TP) (Variables|Default|GetTimeBeforeTP)))
  (Variables|Default|SetTimerEventTP _returnvalue))

(event Custom|CE_TP
  (bind _sphere (Variables|Default|GetSphere))
  ;[0.15 0.15 0.15 0.5] CE TP
  (Transformation|SetActorLocation (Variables|Default|GetStartPos) false false)
  (Physics|SetPhysicsLinearVelocity _sphere "0, 0, 0" false "None")
  (Class|PrimitiveComponent|SetPhysicsAngularVelocityinDegrees _sphere "0, 0, 0" false "None")
  (Development|PrintString "BALL RESET"))

(event EventBeginPlay
  ;[0.15 0.15 0.15 0.5] BEGIN PLAY
  (Variables|Default|SetStartPos (Transformation|GetWorldLocation (Variables|Default|GetSphere)))
  (CallFunction|CETimer))

(fn ConstructionScript)
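; Football goal cage that detects when a BP_BallFOOT enters its BoxGOAL trigger and celebrates the goal.
; On overlap, it calls CETP on the ball, then fires its own goal event.
; That event prints "GOAL" and runs a particle effect for a few seconds before deactivating it.
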(event OnComponentBeginOverlap(BoxGOAL)
  (params (OverlappedComponent :type Primitive%20Component%20Object%20Reference) (OtherActor :type Actor%20Object%20Reference) (OtherComp :type Primitive%20Component%20Object%20Reference) (OtherBodyIndex :type Integer) (bFromSweep :type Boolean) (SweepResult :type Hit%20Result%20Structure%20%28by%20ref%29))
  (bind _asbp_ball_foot (Utilities|Casting|CastToBP_BallFOOT OtherActor))
  (Utilities|IsValid _asbp_ball_foot
    (:Is%20Valid
      (Default|CETP _asbp_ball_foot)
      (CallFunction|CEGOAL))))

(event Custom|CE_GOAL
  (Development|PrintString "GOAL")
  (Components|Activation|Activate (Variables|Default|GetPARTICLE_EFFECT) false)
  (Utilities|FlowControl|Delay 3.0)
  (Components|Activation|Deactivate (Variables|Default|GetPARTICLE_EFFECT)))

(fn ConstructionScript)
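; BP_Toboggan is an interactable slide that carries the player along a two-segment path.
; StartInteract snaps the player to TpLock, waits briefly, sends an interact animation message, then chains two timelines that lerp position from TpLock through Pos2 to Pos5 before setting Idle.
; EndInteract stops the animation and both timelines.
; Getter functions expose the interact widget, lock and unlock points, and current player to the interaction system.
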(event Custom|CE_StopTimeline2
  (bind _delta (Timeline|Timeline Stop)
    (:Update
      (bind _returnvalue (CallFunction|FCalculNewLocation (Variables|Default|GetPos2) (Variables|Default|GetPos5) _delta))
      (Transformation|SetActorLocation (Variables|Default|GetPlayerIn) _returnvalue false false))
    (:Finished
      (Class|PlayerStateMachine|ChangeState (Variables|/Script/CouchGame.CharacterPlayer|GetStateMachine (Variables|Default|GetPlayerIn)) "Idle"))))

(event Custom|CE_StopTimeline1
  (bind _delta (Timeline|Timeline%201%20a%202 Stop)
    (:Update
      (bind _returnvalue (CallFunction|FCalculNewLocation (Variables|Default|GetTpLock) (Variables|Default|GetPos2) _delta))
      (Transformation|SetActorLocation (Variables|Default|GetPlayerIn) _returnvalue false false))
    (:Finished
      (bind _delta_2 (Timeline|Timeline PlayFromStart)
        (:Update
          (bind _returnvalue_2 (CallFunction|FCalculNewLocation (Variables|Default|GetPos2) (Variables|Default|GetPos5) _delta_2))
          (Transformation|SetActorLocation (Variables|Default|GetPlayerIn) _returnvalue_2 false false))
        (:Finished
          (Class|PlayerStateMachine|ChangeState (Variables|/Script/CouchGame.CharacterPlayer|GetStateMachine (Variables|Default|GetPlayerIn)) "Idle"))))))

(event EventEndInteract
  (params (Player :type Character%20Player%20Object%20Reference))
  (bind _returnvalue (Class|CharacterPlayer|GetBlueprintAnim (Variables|Default|GetPlayerIn)))
  (Class|BPIAnim|StopInteract(Message) _returnvalue)
  (CallFunction|CEStopTimeline1)
  (CallFunction|CEStopTimeline2)
  (Variables|Default|SetPlayerIsIn false))

(event EventSetCharacterinInteract
  (params (Player :type Character%20Player%20Object%20Reference))
  (Variables|Default|SetPlayerIn Player))

(event EventStartInteract
  (params (Player :type Character%20Player%20Object%20Reference))
  (bind _output_get (Variables|Default|SetPlayerIn Player))
  (Variables|Default|SetPlayerIsIn true)
  (Transformation|SetActorLocation _output_get (Transformation|GetWorldLocation (Variables|Default|GetTpLock)) false false)
  (Utilities|FlowControl|Delay 0.5)
  (if (Variables|Default|GetPlayerIsIn)
    (bind _returnvalue (Class|CharacterPlayer|GetBlueprintAnim (Variables|Default|GetPlayerIn)))
    (Class|BPIAnim|PlayInteract(Message) _returnvalue "NewEnumerator0")
    (bind _delta (Timeline|Timeline%201%20a%202 PlayFromStart)
      (:Update
        (bind _returnvalue_2 (CallFunction|FCalculNewLocation (Variables|Default|GetTpLock) (Variables|Default|GetPos2) _delta))
        (Transformation|SetActorLocation (Variables|Default|GetPlayerIn) _returnvalue_2 false false))
      (:Finished
        (bind _delta_2 (Timeline|Timeline PlayFromStart)
          (:Update
            (bind _returnvalue_3 (CallFunction|FCalculNewLocation (Variables|Default|GetPos2) (Variables|Default|GetPos5) _delta_2))
            (Transformation|SetActorLocation (Variables|Default|GetPlayerIn) _returnvalue_3 false false))
          (:Finished
            (Class|PlayerStateMachine|ChangeState (Variables|/Script/CouchGame.CharacterPlayer|GetStateMachine (Variables|Default|GetPlayerIn)) "Idle")))))))

(fn ConstructionScript)

(fn FCalculNewLocation
  (params (TargetStart :type Scene%20Component%20Object%20Reference) (TargetEnd :type Scene%20Component%20Object%20Reference) (Delta :type Float%20%28double-precision%29))
  (bind _returnvalue (Transformation|GetWorldLocation TargetStart))
  (return (+ _returnvalue (* (- (Transformation|GetWorldLocation TargetEnd) _returnvalue) Delta))))

(fn GetCharacterinInteract
  (return (Variables|Default|GetPlayerIn)))

(fn GetInteractWidget
  (return "/Game/BP/Widget/WBP_InteractX.WBP_InteractX_C"))

(fn GetPlayerLockParent
  (return (Variables|Default|GetTpLock)))

(fn GetUnlockTP
  (return (Variables|Default|GetTpUnLock)))

(fn IsPlayerLocked
  (return (Utilities|IsValid (Variables|Default|GetPlayerIn))))

(fn LockedPlayer
  (return true))
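; Interactable "Tampon" actor that locks the player into an alternating down/up quick-time-event sequence until completed.
; StartInteract turns the world-space WBP_QTE widget toward BP_CameraActor, then delayed prompts alternate, with wrong inputs or failed clicks restarting from down.
; Tick also restarts timed-out prompts, checking completion through hard-coded interaction ID 203.
; Reaching MaxCount successful ups saves completion via SaveCubeSubsystem and returns the player's state machine to Idle.
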(event Custom|CEPlayQTETampon
  (params (TimerQTE :type Float%20%28double-precision%29) (IndexQTE :type Integer))
  ;[0.15 0.15 0.15 0.5] Play QTE Tampon
  (if (Variables|Default|GetIsPlayable)
    (CallFunction|FShowWidget)
    (Default|PlayQTE (Variables|Default|GetAs%20WBP%20QTE) TimerQTE IndexQTE)))

(event Custom|CE_ResetQTE
  ;[0.15 0.15 0.15 0.5] Reset QTE
  ;;[0.15 0.15 0.15 0.5] Reset Var Count
  (Variables|Default|SetCountUp 0)
  (Variables|Default|SetCountDown 0)
  ;;[0.15 0.15 0.15 0.5] Lancer le QTE down
  (Utilities|FlowControl|Delay (Variables|Default|GetTimeQTEForStart))
  (CallFunction|CEPlayQTETampon (Variables|Default|GetTimeQTEDuration) 2))

(event Custom|CE_RotationWidget
  (bind _worldcamera (Variables|Default|GetWorldCamera))
  (bind _widget (Variables|Default|GetWidget))
  (bind _returnvalue (Transformation|GetWorldLocation _widget))
  (bind _rootcomponent (Variables|/Script/Engine.Actor|GetRootComponent _worldcamera))
  (bind _returnvalue_2 (Transformation|GetWorldLocation _rootcomponent))
  (bind _returnvalue_3 (Math|Rotator|FindLookatRotation _returnvalue _returnvalue_2))
  ;[0.15 0.15 0.15 0.5] Rotation Widget
  (Transformation|SetWorldRotation (Variables|Default|GetWidget) (Math|Rotator|MakeRotator (.roll (Transformation|GetWorldRotation (Variables|Default|GetWidget))) (.pitch _returnvalue_3) (.yaw _returnvalue_3)) false false))

(event Custom|CE_Win
  ;[0.15 0.15 0.15 0.5] Win
  (Class|SaveCubeSubsystem|SaveInteractionData (Subsystems|GetSaveCubeSubsystem) (.interactionindex (Variables|Default|GetInteractionData)) true)
  (Class|PlayerStateMachine|ChangeState (Variables|/Script/CouchGame.CharacterPlayer|GetStateMachine (Variables|Default|GetPlayerIn)) "Idle"))

(event EventBeginPlay
  ;[0.15 0.15 0.15 0.5] Begin Play (Recuperation des var)
  (bind _aswbp_qte (Utilities|Casting|CastToWBP_QTE (UserInterface|GetUserWidgetObject (Variables|Default|GetWidget))))
  (Variables|Default|SetAs%20WBP%20QTE _aswbp_qte)
  (bind _returnvalue (Actor|GetActorOfClass "/Game/BP/Camera/BP_CameraActor.BP_CameraActor_C"))
  (Variables|Default|SetWorldCamera _returnvalue))

(event EventTick
  (params (DeltaSeconds :type Float%20%28single-precision%29))
  (bind _returnvalue (Class|SaveCubeSubsystem|GetInteractionsDatasfromID (Subsystems|GetSaveCubeSubsystem) 203))
  (if (not (.iscompleted _returnvalue))
    (if (Variables|Default|GetIsVisible)
      ;[0.15 0.15 0.15 0.5] If le QTE est fini
      (bind _isrunning (Default|FGetIsRunning (Variables|Default|GetAs%20WBP%20QTE)))
      (if (not _isrunning)
        ;[0.15 0.15 0.15 0.5] Hide & Reset Var Count
        (CallFunction|FHideWidget)
        (Variables|Default|SetCountDown 0)
        (Variables|Default|SetCountUp 0)
        ;[0.15 0.15 0.15 0.5] Lancer QTE down
        (Utilities|FlowControl|Delay (Variables|Default|GetTimeQTEForStart))
        (CallFunction|CEPlayQTETampon (Variables|Default|GetTimeQTEDuration) 2)))))

(event EventEndInteract
  (params (Player :type Character%20Player%20Object%20Reference))
  ;[0.15 0.15 0.15 0.5] End Interact
  (Variables|Default|SetIsPlayable false)
  (CallFunction|FHideWidget)
  (bind _returnvalue (Class|CharacterPlayer|GetBlueprintAnim (Variables|Default|GetPlayerIn)))
  (Class|BPIAnim|StopInteract(Message) _returnvalue))

(event EventSetCharacterinInteract
  (params (Player :type Character%20Player%20Object%20Reference))
  ;[0.15 0.15 0.15 0.5] Player In
  (Variables|Default|SetPlayerIn Player))

(event EventHighlightInteraction
  (params (IsHighlight :type Boolean))
  (Rendering|SetVisibility (Variables|Default|GetCylinder) IsHighlight false))

(event EventStartInteract
  (params (Player :type Character%20Player%20Object%20Reference))
  ;[0.15 0.15 0.15 0.5] StartInteract
  (bind _returnvalue (Class|SaveCubeSubsystem|GetInteractionsDatasfromID (Subsystems|GetSaveCubeSubsystem) (.interactionindex (Variables|Default|GetInteractionData))))
  (if (not (.iscompleted _returnvalue))
    (bind _returnvalue_2 (Class|CharacterPlayer|GetBlueprintAnim Player))
    (Class|BPIAnim|PlayInteract(Message) _returnvalue_2 "NewEnumerator3")
    (CallFunction|CERotationWidget)
    ;;[0.15 0.15 0.15 0.5] Reset Var
    (Variables|Default|SetCountUp 0)
    (Variables|Default|SetCountDown 0)
    (Variables|Default|SetIsPlayable true)
    ;;[0.15 0.15 0.15 0.5] Lancer QTE down
    (Utilities|FlowControl|Delay (Variables|Default|GetTimeQTEForStart))
    (CallFunction|CEPlayQTETampon (Variables|Default|GetTimeQTEDuration) 2)))

(event EventOnStartInteract
  (params (Player :type Character%20Player%20Object%20Reference) (InputID :type EInputID%20Enum :default "QTE1"))
  ;[0.15 0.15 0.15 0.5] OnStartInteract
  (switch Utilities|FlowControl|Switch|SwitchonEInputID InputID
    (:QTE1
      ;[0.15 0.15 0.15 0.5] Click Up
      (bind _win (Default|FClickQTE (Variables|Default|GetAs%20WBP%20QTE)))
      (CallFunction|FHideWidget)
      ;[0.15 0.15 0.15 0.5] If QTE win
      (if _win
        (Math|Integer|IncrementInt (Variables|Default|GetCountUp)
          (:%20%20
            ;[0.15 0.15 0.15 0.5] If QTE fini
            (if (== (Variables|Default|GetCountUp) (Variables|Default|GetMaxCount))
              ;[0.15 0.15 0.15 0.5] Win
              (Development|PrintString "WIN")
              (CallFunction|CEWin)
              (else
                ;[0.15 0.15 0.15 0.5] Lancer le QTE down
                (Utilities|FlowControl|Delay (Variables|Default|GetTimeBetween2Round))
                (CallFunction|CEPlayQTETampon (Variables|Default|GetTimeQTEDuration) 2)))))
        (else
          (CallFunction|CEResetQTE))))
    (:QTE2
      ;[0.15 0.15 0.15 0.5] Click Right
      (Default|FClickQTE (Variables|Default|GetAs%20WBP%20QTE) 1)
      (CallFunction|FHideWidget)
      (CallFunction|CEResetQTE))
    (:QTE3
      ;[0.15 0.15 0.15 0.5] Click Down
      (bind _win_2 (Default|FClickQTE (Variables|Default|GetAs%20WBP%20QTE) 2))
      (CallFunction|FHideWidget)
      ;[0.15 0.15 0.15 0.5] If QTE win
      (if _win_2
        (Math|Integer|IncrementInt (Variables|Default|GetCountDown)
          (:%20%20
            ;[0.15 0.15 0.15 0.5] Lancer le QTE Up
            (Utilities|FlowControl|Delay (Variables|Default|GetTimeBetween2QTE))
            (CallFunction|CEPlayQTETampon (Variables|Default|GetTimeQTEDuration))))
        (else
          ;[0.15 0.15 0.15 0.5] Reset Var Count
          (Variables|Default|SetCountUp 0)
          (Variables|Default|SetCountDown 0)
          ;[0.15 0.15 0.15 0.5] Lancer le QTE down
          (Utilities|FlowControl|Delay (Variables|Default|GetTimeQTEForStart))
          (CallFunction|CEPlayQTETampon (Variables|Default|GetTimeQTEDuration) 2))))
    (:QTE4
      ;[0.15 0.15 0.15 0.5] Click Left
      (Default|FClickQTE (Variables|Default|GetAs%20WBP%20QTE) 3)
      (CallFunction|FHideWidget)
      (CallFunction|CEResetQTE))))

(fn ConstructionScript)

(fn FShowWidget
  (Variables|Default|SetIsVisible true)
  (Rendering|SetVisibility (Variables|Default|GetWidget) true false))

(fn FHideWidget
  (Variables|Default|SetIsVisible false)
  (Rendering|SetVisibility (Variables|Default|GetWidget) false false))

(fn GetCharacterinInteract
  (return (Variables|Default|GetPlayerIn)))

(fn GetInteractWidget
  (return (Variables|Default|GetInteractWidget)))

(fn GetPlayerLockParent
  (return (Variables|Default|GetLockParent)))

(fn GetUnlockTP
  (return (Variables|Default|GetLockParent)))

(fn IsPlayerLocked
  (return (Utilities|IsValid (Variables|Default|GetPlayerIn))))

(fn LockedPlayer
  (return true))
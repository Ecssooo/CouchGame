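; BP_Bench is a bench interactable that answers interaction calls and declares that it locks the player.
; It stores the interacting player in PlayerIn and counts as occupied while that reference is valid.
; Getters expose TPLock as the player's lock parent and UnLock as the release point.
; StartInteract only prints a debug string, and GetInteractWidget returns no widget.
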(event EventStartInteract
  (params (Player :type Character%20Player%20Object%20Reference))
  (Development|PrintString "Interact_Bench"))

(event EventSetCharacterinInteract
  (params (Player :type Character%20Player%20Object%20Reference))
  (Variables|Default|SetPlayerIn Player))

(fn ConstructionScript)

(fn GetCharacterinInteract
  (return (Variables|Default|GetPlayerIn)))

(fn GetInteractWidget
  (return 0))

(fn GetPlayerLockParent
  (return (Variables|Default|GetTPLock)))

(fn GetUnlockTP
  (return (Variables|Default|GetUnLock)))

(fn IsPlayerLocked
  (return (Utilities|IsValid (Variables|Default|GetPlayerIn))))

(fn LockedPlayer
  (return true))
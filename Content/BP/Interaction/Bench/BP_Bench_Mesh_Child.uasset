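; Bench interactable Blueprint that implements interaction events and queries for a player using the bench.
; Start and end interact play and stop an interact message on the player's anim Blueprint, with a leftover debug print on start.
; It stores the interacting player, reports locked status from that reference's validity, and exposes TPLock and UnLock for lock and unlock.
; Delayed logic to attach and rotate the player is disconnected and never runs.
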(event EventEndInteract
  (params (Player :type Character%20Player%20Object%20Reference))
  (bind _returnvalue (Class|CharacterPlayer|GetBlueprintAnim Player))
  (Class|BPIAnim|StopInteract(Message) _returnvalue))

(event EventSetCharacterinInteract
  (params (Player :type Character%20Player%20Object%20Reference))
  (Variables|Default|SetPlayerIn Player))

(event EventStartInteract
  (params (Player :type Character%20Player%20Object%20Reference))
  (Development|PrintString "Hello")
  (bind _returnvalue (Class|CharacterPlayer|GetBlueprintAnim Player))
  (Class|BPIAnim|PlayInteract(Message) _returnvalue "NewEnumerator0"))

(fn ConstructionScript)

(fn GetCharacterinInteract
  (return (Variables|Default|GetPlayerIn)))

(fn GetInteractWidget
  (return 0))

(fn GetPlayerLockParent
  (return (Variables|Default|GetTPLock)))

(fn GetUnlockTP
  (return (Variables|Default|GetUnLock)))

(fn IsPlayerLocked
  (return (Utilities|IsValid (Variables|Default|GetPlayerIn))))

(fn LockedPlayer
  (return true))
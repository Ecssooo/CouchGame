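; Interactable bench actor that locks a player to it and triggers an interact animation, likely sitting.
; On interact start, after a short delay, it attaches the stored player to itself, yaws them 90 degrees from the bench mesh and messages their animation Blueprint.
; Ending interaction only stops that animation message, without detaching or clearing the stored player.
; Getters expose lock state and lock/unlock points; the widget getter is empty.
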(event EventEndInteract
  (params (Player :type Character%20Player%20Object%20Reference))
  (bind _returnvalue (Class|CharacterPlayer|GetBlueprintAnim Player))
  (Class|BPIAnim|StopInteract(Message) _returnvalue))

(event EventStartInteract
  (params (Player :type Character%20Player%20Object%20Reference))
  (Utilities|FlowControl|Delay 0.1)
  (Transformation|AttachActorToActor (Variables|Default|GetPlayerIn) self "None" "KeepWorld" "KeepWorld" "KeepWorld" true)
  (Transformation|SetActorRotation (Variables|Default|GetPlayerIn) (Math|Rotator|MakeRotator 0.0 0.0 (+ (.Yaw (Math|Rotator|BreakRotator (Transformation|GetWorldRotation (Variables|Default|GetBench)))) 9e+01)))
  (bind _returnvalue (Class|CharacterPlayer|GetBlueprintAnim (Variables|Default|GetPlayerIn)))
  (Class|BPIAnim|PlayInteract(Message) _returnvalue "NewEnumerator0"))

(event EventSetCharacterinInteract
  (params (Player :type Character%20Player%20Object%20Reference))
  (Variables|Default|SetPlayerIn Player))

(fn ConstructionScript)

(fn GetCharacterinInteract
  (return (Variables|Default|GetPlayerIn)))

(fn GetInteractWidget
  (return 0))

(fn GetPlayerLockParent
  (return (Variables|Default|GetTPLock)))

(fn GetUnlockTP
  (return (Variables|Default|GetUnLock)))

(fn IsPlayerLocked
  (return (Utilities|IsValid (Variables|Default|GetPlayerIn))))

(fn LockedPlayer
  (return true))
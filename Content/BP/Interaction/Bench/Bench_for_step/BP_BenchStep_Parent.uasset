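; Bench interaction parent that completes once two players have stayed on it together for a set time.
; On BeginPlay it registers itself with two child-actor bench steps and keeps a player count through add and remove events.
; At two players Tick runs a timer that any removal resets; winning saves interaction 501 as completed, blocking restarts, and stops both children.
; Highlighting toggles custom depth on the bench mesh.
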(event Custom|CE_AddPlayer
  (bind _returnvalue (Class|SaveCubeSubsystem|GetInteractionsDatasfromID (Subsystems|GetSaveCubeSubsystem) 501))
  (if (not (.iscompleted _returnvalue))
    (bind _result (Math|Integer|IncrementInt (Variables|Default|GetCountPlayerIn))
      (:%20%20
        (if (== _result 2)
          (CallFunction|CEStartInteract))))))

(event Custom|CE_RemovePlayer
  (bind _result (Math|Integer|DecrementInt (Variables|Default|GetCountPlayerIn))
    (:%20%20
      (Variables|Default|SetCountPlayerIn (Math|Integer|Clamp(Integer) _result 0 2))
      (CallFunction|CEStopInteract))))

(event Custom|CE_StartInteract
  (Variables|Default|SetIsInteractionStart true)
  (Variables|Default|SetCurrentTime 0.0))

(event Custom|CE_StopInteract
  (Variables|Default|SetIsInteractionStart false)
  (Variables|Default|SetCurrentTime 0.0))

(event Custom|CE_Win
  (CallFunction|CEStopInteract)
  (Class|SaveCubeSubsystem|SaveInteractionData (Subsystems|GetSaveCubeSubsystem) 501 true)
  (Default|CEStopInteract (Variables|Default|GetAs%20BP%20Bench%20Step%20Child))
  (Default|CEStopInteract (Variables|Default|GetAs%20BP%20Bench%20Step%20Child_0)))

(event EventBeginPlay
  (bind _asbp_bench_step_child (Utilities|Casting|CastToBP_BenchStep_Child (Variables|/Script/Engine.ChildActorComponent|GetChildActor (Variables|Default|GetBP_BenchStep_Child))))
  (bind _output_get (Variables|Default|SetAs%20BP%20Bench%20Step%20Child _asbp_bench_step_child))
  (Default|CESetBPBenchParent _output_get self)
  (bind _asbp_bench_step_child_2 (Utilities|Casting|CastToBP_BenchStep_Child (Variables|/Script/Engine.ChildActorComponent|GetChildActor (Variables|Default|GetBP_BenchStep_Child1))))
  (bind _output_get_2 (Variables|Default|SetAs%20BP%20Bench%20Step%20Child_0 _asbp_bench_step_child_2))
  (Default|CESetBPBenchParent _output_get_2 self))

(event EventTick
  (params (DeltaSeconds :type Float%20%28single-precision%29))
  (if (Variables|Default|GetIsInteractionStart)
    (bind _output_get (Variables|Default|SetCurrentTime (+ DeltaSeconds (Variables|Default|GetCurrentTime))))
    (if (>= _output_get (Variables|Default|GetTimeInteraction))
      (CallFunction|CEWin))))

(event EventHighlightInteraction
  (params (IsHighlight :type Boolean))
  (Rendering|SetRenderCustomDepth (Variables|Default|GetSM_Bench) IsHighlight))

(fn ConstructionScript)
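; BP_BenchStep_Child is an interactable player spot belonging to a parent bench, which is handed to it through an event.
; Starting or ending interaction plays or stops the player's interact animation message and adds or removes a player on the parent.
; A forced stop ends the animation and returns the player's state machine to Idle.
; It exposes lock and unlock points, and hides its interact widget once saved interaction data is completed.
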(event Custom|CE_SetBPBenchParent
  (params (BenchParent :type BP%20Bench%20Step%20Parent%20Object%20Reference))
  (Variables|Default|SetBenchParent BenchParent))

(event Custom|CE_StopInteract
  (bind _returnvalue (Class|CharacterPlayer|GetBlueprintAnim (Variables|Default|GetPlayerIn)))
  (Class|BPIAnim|StopInteract(Message) _returnvalue)
  (Class|PlayerStateMachine|ChangeState (Variables|/Script/CouchGame.CharacterPlayer|GetStateMachine (Variables|Default|GetPlayerIn)) "Idle"))

(event EventStartInteract
  (params (Player :type Character%20Player%20Object%20Reference))
  (Development|PrintString "AAAA")
  (bind _returnvalue (Class|CharacterPlayer|GetBlueprintAnim Player))
  (Class|BPIAnim|PlayInteract(Message) _returnvalue "NewEnumerator0")
  (Default|CEAddPlayer (Variables|Default|GetBenchParent)))

(event EventEndInteract
  (params (Player :type Character%20Player%20Object%20Reference))
  (Development|PrintString "BBBB")
  (Default|CERemovePlayer (Variables|Default|GetBenchParent))
  (bind _returnvalue (Class|CharacterPlayer|GetBlueprintAnim (Variables|Default|GetPlayerIn)))
  (Class|BPIAnim|StopInteract(Message) _returnvalue))

(event EventSetCharacterinInteract
  (params (Player :type Character%20Player%20Object%20Reference))
  (Variables|Default|SetPlayerIn Player))

(fn ConstructionScript)

(fn GetCharacterinInteract
  (return (Variables|Default|GetPlayerIn)))

(fn GetInteractWidget
  (bind _returnvalue (Class|SaveCubeSubsystem|GetInteractionsDatasfromID (Subsystems|GetSaveCubeSubsystem) (.interactionindex (Variables|Default|GetInteractionData))))
  (if (.iscompleted _returnvalue)
    (return 0)
    (else
      (return "/Game/BP/Widget/WBP_InteractX.WBP_InteractX_C"))))

(fn GetPlayerLockParent
  (return (Variables|Default|GetTPLock)))

(fn GetUnlockTP
  (return (Variables|Default|GetUnLock)))

(fn IsPlayerLocked
  (return (Utilities|IsValid (Variables|Default|GetPlayerIn))))

(fn LockedPlayer
  (return true))
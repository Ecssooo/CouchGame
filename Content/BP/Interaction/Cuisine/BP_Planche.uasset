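; Interactable cutting board station in the kitchen minigame, where a locked player cuts meat through timed QTEs while the fridge is also in play.
; Interacting flags the board active in BP_Cuisine and triggers a BP_Frigo QTE; board QTEs require both stations active.
; Correct inputs call CutMeat on BP_Cuisine; misses or timeouts (polled on Tick) roll a new random QTE.
; The QTE widget turns toward the camera when interaction starts.
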(event Custom|CE_PlayQTEPlanche
  (params (TimerQTE :type Float%20%28double-precision%29) (IndexQTE :type Integer))
  (if (Variables|/Game/BP/Interaction/Cuisine/BP_Cuisine.BP_Cuisine_C|GetIsPlanchePlaying (Variables|Default|GetCuisine))
    (if (Variables|/Game/BP/Interaction/Cuisine/BP_Cuisine.BP_Cuisine_C|GetIsFrigoPlaying (Variables|Default|GetCuisine))
      (CallFunction|FShowWBP)
      (Default|PlayQTE (Variables|Default|GetAs%20WBP%20QTE) TimerQTE IndexQTE)
      (Variables|/Game/BP/Interaction/Cuisine/BP_Cuisine.BP_Cuisine_C|SetIsQTEPlanche (Variables|Default|GetCuisine) true))))

(event Custom|CE_RotateWBP
  (bind _worldcamera (Variables|Default|GetWorldCamera))
  (bind _widget (Variables|Default|GetWidget))
  (bind _returnvalue (Transformation|GetWorldLocation _widget))
  (bind _rootcomponent (Variables|/Script/Engine.Actor|GetRootComponent _worldcamera))
  (bind _returnvalue_2 (Transformation|GetWorldLocation _rootcomponent))
  (bind _returnvalue_3 (Math|Rotator|FindLookatRotation _returnvalue _returnvalue_2))
  (Transformation|SetWorldRotation (Variables|Default|GetWidget) (Math|Rotator|MakeRotator (.roll (Transformation|GetWorldRotation (Variables|Default|GetWidget))) (.pitch _returnvalue_3) (.yaw _returnvalue_3)) false false))

(event Custom|CE_HighlightInteraction
  (params (InputPin :type Boolean))
  (Rendering|SetVisibility (Variables|Default|GetCylinder) InputPin false)
  (Rendering|SetRenderCustomDepth (Variables|Default|GetTable) InputPin)
  (Rendering|SetRenderCustomDepth (Variables|Default|Getplanche%20a%20decouper) InputPin))

(event Custom|CE_StartPlanche
  (if (Variables|/Game/BP/Interaction/Cuisine/BP_Cuisine.BP_Cuisine_C|GetIsPlanchePlaying (Variables|Default|GetCuisine))
    (if (Variables|/Game/BP/Interaction/Cuisine/BP_Cuisine.BP_Cuisine_C|GetIsFrigoPlaying (Variables|Default|GetCuisine))
      (CallFunction|CEPlayQTEPlanche 1.5 (Math|Random|RandomInteger 3)))))

(event EventBeginPlay
  (bind _aswbp_qte (Utilities|Casting|CastToWBP_QTE (UserInterface|GetUserWidgetObject (Variables|Default|GetWidget))))
  (Variables|Default|SetAs%20WBP%20QTE _aswbp_qte)
  (bind _returnvalue (Actor|GetActorOfClass "/Game/BP/Camera/BP_CameraActor.BP_CameraActor_C"))
  (Variables|Default|SetWorldCamera _returnvalue)
  (bind _returnvalue_2 (Actor|GetActorOfClass "/Game/BP/Interaction/Cuisine/BP_Frigo.BP_Frigo_C"))
  (Variables|Default|SetFrigo _returnvalue_2)
  (bind _returnvalue_3 (Actor|GetActorOfClass "/Game/BP/Interaction/Cuisine/BP_Cuisine.BP_Cuisine_C"))
  (Variables|Default|SetCuisine _returnvalue_3))

(event EventSetCharacterinInteract
  (params (Player :type Character%20Player%20Object%20Reference))
  (Variables|Default|SetPlayerIn Player))

(event EventTick
  (params (DeltaSeconds :type Float%20%28single-precision%29))
  (if (Variables|Default|GetIsVisible)
    (if (Variables|/Game/BP/Interaction/Cuisine/BP_Cuisine.BP_Cuisine_C|GetIsQTEPlanche (Variables|Default|GetCuisine))
      (bind _isrunning (Default|FGetIsRunning (Variables|Default|GetAs%20WBP%20QTE)))
      (if (not _isrunning)
        (CallFunction|FHideWBP)
        (Utilities|FlowControl|Delay 1.0)
        (CallFunction|CEPlayQTEPlanche 1.5 (Math|Random|RandomInteger 3))))))

(event EventOnStartInteract
  (params (Player :type Character%20Player%20Object%20Reference) (InputID :type EInputID%20Enum :default "QTE1"))
  (if (Variables|/Game/BP/Interaction/Cuisine/BP_Cuisine.BP_Cuisine_C|GetIsQTEPlanche (Variables|Default|GetCuisine))
    (switch Utilities|FlowControl|Switch|SwitchonEInputID InputID
      (:QTE1
        (Utilities|QTE1))
      (:QTE2
        (Utilities|QTE2))
      (:QTE3
        (Utilities|QTE3))
      (:QTE4
        (Utilities|QTE4)))
    (Variables|/Game/BP/Interaction/Cuisine/BP_Cuisine.BP_Cuisine_C|SetIsQTEPlanche (Variables|Default|GetCuisine) false)))

(event EventStartInteract
  (params (Player :type Character%20Player%20Object%20Reference))
  (Variables|/Game/BP/Interaction/Cuisine/BP_Cuisine.BP_Cuisine_C|SetIsPlanchePlaying (Variables|Default|GetCuisine) true)
  (Default|CEPlayQTEFrigo (Variables|Default|GetFrigo) 1.5 (Math|Random|RandomInteger 3))
  (CallFunction|CERotateWBP))

(event EventEndInteract
  (params (Player :type Character%20Player%20Object%20Reference))
  (Variables|/Game/BP/Interaction/Cuisine/BP_Cuisine.BP_Cuisine_C|SetIsPlanchePlaying (Variables|Default|GetCuisine) false)
  (if (Variables|/Game/BP/Interaction/Cuisine/BP_Cuisine.BP_Cuisine_C|GetIsQTEPlanche (Variables|Default|GetCuisine))
    (CallFunction|FHideWBP)
    (elif (Variables|/Game/BP/Interaction/Cuisine/BP_Cuisine.BP_Cuisine_C|GetIsQTEFrigo (Variables|Default|GetCuisine))
      (Default|FHideWBP (Variables|Default|GetFrigo))
      (Variables|/Game/BP/Interaction/Cuisine/BP_Cuisine.BP_Cuisine_C|SetIsQTEFrigo (Variables|Default|GetCuisine) false))))

(fn ConstructionScript)

(fn FShowWBP
  (Variables|Default|SetIsVisible true)
  (Rendering|SetVisibility (Variables|Default|GetWidget) true false))

(fn FHideWBP
  (Variables|Default|SetIsVisible false)
  (Rendering|SetVisibility (Variables|Default|GetWidget) false false))

(fn GetCharacterinInteract
  (return (Variables|Default|GetPlayerIn)))

(fn GetInteractWidget
  (return 0))

(fn GetPlayerLockParent
  (return (Variables|Default|GetPlayerPos1)))

(fn GetUnlockTP
  (return (Variables|Default|GetPlayerPos1)))

(fn IsPlayerLocked
  (return (Utilities|IsValid (Variables|Default|GetPlayerIn))))

(fn LockedPlayer
  (return true))
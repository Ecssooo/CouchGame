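; BP_Cuisine is the kitchen interaction actor coordinating a fridge (BP_Frigo) and a cutting board (BP_Planche) around a soy steak.
; It finds both stations at BeginPlay, then on request spawns one steak, slides it between two points with a timeline and starts the board.
; Cutting destroys the steak after a delay, resets the state flags and returns both stations' players to Idle.
; Its interaction functions are empty stubs.
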(event Custom|CE_SpawnSteack
  (if (not (Variables|Default|GetIsSteackSpawn))
    (Variables|Default|SetIsSteackSpawn true)
    (bind _returnvalue (Game|SpawnActorfromClass "/Game/BP/Interaction/Cuisine/BP_SteackDeSoja.BP_SteackDeSoja_C" (Math|Transform|MakeTransform (Transformation|GetWorldLocation (Variables|Components|GetSteackPos1)) "0, 0, 0" "0.400000,0.400000,0.100000") "Undefined" "MultiplyWithRoot" 0 0))
    (Variables|Default|SetSteackDeSoja _returnvalue)
    (bind _1 (Timeline|steack PlayFromStart)
      (:Update
        (Transformation|SetWorldLocation (Variables|/Game/BP/Interaction/Cuisine/BP_SteackDeSoja.BP_SteackDeSoja_C|GetSteackDeSoja _returnvalue) (Math|Vector|Lerp(Vector) (Transformation|GetWorldLocation (Variables|Components|GetSteackPos1)) (Transformation|GetWorldLocation (Variables|Components|GetSteackPos2)) _1) false false))
      (:Finished
        (Variables|Default|SetSteackOnPlanch true)
        (Default|CEStartPlanche (Variables|Default|GetPlanche))))))

(event Custom|CE_CutMeat
  (Utilities|FlowControl|Delay 1.0)
  (Actor|DestroyActor (Variables|Default|GetSteackDeSoja))
  (Utilities|FlowControl|Sequence
    (:then_0
      (Variables|Default|SetIsSteackSpawn false))
    (:then_1
      (Variables|Default|SetSteackOnPlanch false))
    (:then_2
      (Variables|Default|SetIsPlanchePlaying false))
    (:then_3
      (Variables|Default|SetIsFrigoPlaying false))
    (:then_4
      (Variables|Default|SetIsQTEFrigo false))
    (:then_5
      (Variables|Default|SetIsQTEPlanche false))
    (:then_6
      (Class|PlayerStateMachine|ChangeState (Variables|/Script/CouchGame.CharacterPlayer|GetStateMachine (Variables|/Game/BP/Interaction/Cuisine/BP_Frigo.BP_Frigo_C|GetPlayerIn (Variables|Default|GetFrigo))) "Idle")
      (Class|PlayerStateMachine|ChangeState (Variables|/Script/CouchGame.CharacterPlayer|GetStateMachine (Variables|/Game/BP/Interaction/Cuisine/BP_Planche.BP_Planche_C|GetPlayerIn (Variables|Default|GetPlanche))) "Idle"))))

(event EventBeginPlay
  (bind _returnvalue (Actor|GetActorOfClass "/Game/BP/Interaction/Cuisine/BP_Planche.BP_Planche_C"))
  (Variables|Default|SetPlanche _returnvalue)
  (bind _returnvalue_2 (Actor|GetActorOfClass "/Game/BP/Interaction/Cuisine/BP_Frigo.BP_Frigo_C"))
  (Variables|Default|SetFrigo _returnvalue_2))

(fn ConstructionScript)

(fn GetCharacterinInteract
  (return 0))

(fn GetInteractWidget
  (return 0))

(fn GetPlayerLockParent
  (return 0))

(fn GetUnlockTP
  (return 0))

(fn IsPlayerLocked
  (return false))

(fn LockedPlayer
  (return false))
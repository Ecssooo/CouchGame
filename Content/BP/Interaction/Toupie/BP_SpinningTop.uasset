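; Interactable spinning top that one player rides while another player spins it, launching the rider once spin speed passes a limit.
; An overlap box sets it as the player's current interact object, and EntryInteract attaches the rider with movement disabled or lets them exit.
; Each StartInteract call from a non-rider compounds the yaw step using delta time and re-snaps the rider.
; Stopping, exiting or launching resets the speed; the latter two also detach the rider.
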(event OnComponentBeginOverlap(Box_InteractionZone)
  (params (OverlappedComponent :type Primitive%20Component%20Object%20Reference) (OtherActor :type Actor%20Object%20Reference) (OtherComp :type Primitive%20Component%20Object%20Reference) (OtherBodyIndex :type Integer) (bFromSweep :type Boolean) (SweepResult :type Hit%20Result%20Structure%20%28by%20ref%29))
  ;[0.15 0.15 0.15 0.5] Overlap Player with SpinningTop
  (bind _asbp_character_player (Utilities|Casting|CastToBP_CharacterPlayer OtherActor))
  (bind _output_get (Variables|Default|SetPlayer _asbp_character_player))
  (Variables|/Game/BP/Player/BP_CharacterPlayer.BP_CharacterPlayer_C|SetCurrentInteractObject _output_get self))

(event OnComponentEndOverlap(Box_InteractionZone)
  (params (OverlappedComponent :type Primitive%20Component%20Object%20Reference) (OtherActor :type Actor%20Object%20Reference) (OtherComp :type Primitive%20Component%20Object%20Reference) (OtherBodyIndex :type Integer))
  ;[0.15 0.15 0.15 0.5] Overlap Player with SpinningTop
  (bind _asbp_character_player (Utilities|Casting|CastToBP_CharacterPlayer OtherActor))
  (bind _output_get (Variables|Default|SetPlayer _asbp_character_player))
  (Variables|/Game/BP/Player/BP_CharacterPlayer.BP_CharacterPlayer_C|SetCurrentInteractObject _output_get 0))

(event Custom|CE_StopSpinning
  ;[0.15 0.15 0.15 0.5] Launch / Stop SpinningTop
  (Development|PrintString "Rotate OFF" true true "(R=1.000000,G=0.000000,B=0.016047,A=1.000000)")
  (Variables|Default|SetValueRotation (Variables|Default|GetDefaultValueRotation)))

(event EventBeginPlay
  ;[0.15 0.15 0.15 0.5] Set Value In Start
  (Variables|Default|SetDefaultValueRotation (Variables|Default|GetValueRotation)))

(event EventStopInteract
  (params (Player :type BP%20Character%20Player%20Object%20Reference))
  ;[0.15 0.15 0.15 0.5] Launch / Stop SpinningTop
  (Development|PrintString "Rotate OFF" true true "(R=1.000000,G=0.000000,B=0.016047,A=1.000000)")
  (Variables|Default|SetValueRotation (Variables|Default|GetDefaultValueRotation)))

(event EventStartInteract
  (params (Player :type BP%20Character%20Player%20Object%20Reference))
  ;[0.15 0.15 0.15 0.5] Launch / Stop SpinningTop
  (bind _output_get (Variables|Default|SetPlayerActivateSpinningTop Player))
  (if (not (Variables|/Game/BP/Player/BP_CharacterPlayer.BP_CharacterPlayer_C|GetIsInSpinningTop _output_get))
    (if (Variables|Default|GetisPlayerIn)
      (Development|PrintString "Rotate On" true true "(R=0.000000,G=1.000000,B=0.123024,A=1.000000)")
      (bind _output_get_2 (Variables|Default|SetValueRotation (+ (* (* (Variables|Default|GetValueRotation) (Utilities|Time|GetWorldDeltaSeconds)) (Variables|Default|GetVitesseRotation)) (Variables|Default|GetValueRotation))))
      (Transformation|AddRelativeRotation (Variables|Default|GetParent_Cube_Center) (Math|Rotator|MakeRotator 0.0 0.0 _output_get_2) false false)
      (CallFunction|SetPosPlayerSpinningTop)
      (if (> (Variables|Default|GetValueRotation) (Variables|Default|GetValueLimitAfterLaunch))
        (Development|PrintString "Launch")
        (Character|LaunchCharacter (Variables|Default|GetPlayerInSpinningTop) (Math|Conversions|ToVector(Float) (Variables|Default|GetValueLaunchCharacter)) false false)
        (Default|PlayerLeaveSpinningTop (Variables|Default|GetPlayerInSpinningTop))
        (CallFunction|UndoPosPlayerSpinningTop))
      (else
        (Development|PrintString "You Can't Rotate" true true "(R=1.000000,G=0.037429,B=0.000000,A=1.000000)")
        (CallFunction|CEStopSpinning)))))

(event EventEntryInteract
  (params (Player :type BP%20Character%20Player%20Object%20Reference))
  ;[0.15 0.15 0.15 0.5] Entry / SpinningTop
  (Variables|Default|SetPlayerActorTemporary Player)
  (if (Variables|Default|GetisPlayerIn)
    (if (Variables|/Game/BP/Player/BP_CharacterPlayer.BP_CharacterPlayer_C|GetIsInSpinningTop (Variables|Default|GetPlayerInSpinningTop))
      (Default|PlayerLeaveSpinningTop (Variables|Default|GetPlayerInSpinningTop))
      (CallFunction|UndoPosPlayerSpinningTop)
      (Development|PrintString "Player Exit Spinning TOP" true true "(R=1.000000,G=0.000000,B=0.034294,A=1.000000)")
      (else
        (Development|PrintString "Can't Entry in Spinning TOP" true true "(R=1.000000,G=0.033577,B=0.000000,A=1.000000)")))
    (else
      (Variables|Default|SetPlayerInSpinningTop (Variables|Default|GetPlayerActorTemporary))
      (CallFunction|SetPosPlayerSpinningTop)
      (Variables|Default|SetisPlayerIn true)
      (Variables|/Game/BP/Player/BP_CharacterPlayer.BP_CharacterPlayer_C|SetIsInSpinningTop (Variables|Default|GetPlayerInSpinningTop) true)
      (Development|PrintString "Player Entry in Spinning TOP" true true "(R=0.031144,G=1.000000,B=0.000000,A=1.000000)"))))

(fn ConstructionScript)

(fn SetPosPlayerSpinningTop
  (bind _playerinspinningtop (Variables|Default|GetPlayerInSpinningTop))
  (bind _posplayer1 (Variables|Default|GetPosPlayer1))
  (bind _posplayer1_2 (Variables|Default|GetPosPlayer1))
  (bind _returnvalue (Transformation|GetWorldLocation _posplayer1))
  (bind _returnvalue_2 (Transformation|GetWorldRotation _posplayer1_2))
  (bind (_roll _pitch _yaw) (Math|Rotator|BreakRotator _returnvalue_2))
  (Transformation|AttachActorToActor (Variables|Default|GetPlayerInSpinningTop) self "" "KeepWorld" "KeepWorld" "KeepWorld" true)
  (Transformation|SetActorLocation (Variables|Default|GetPlayerInSpinningTop) (Math|Vector|MakeVector (.x _returnvalue) (.y _returnvalue) (.z _returnvalue)) false false)
  (Transformation|SetActorRotation _playerinspinningtop (Math|Rotator|MakeRotator _roll _pitch _yaw))
  (Pawn|Components|CharacterMovement|SetMovementMode (Variables|/Script/Engine.Character|GetCharacterMovement _playerinspinningtop) "MOVE_None" 0))

(fn UndoPosPlayerSpinningTop
  (Transformation|DetachFromActor (Variables|Default|GetPlayerInSpinningTop) "KeepWorld" "KeepWorld" "KeepWorld")
  (Pawn|Components|CharacterMovement|SetMovementMode (Variables|/Script/Engine.Character|GetCharacterMovement (Variables|Default|GetPlayerInSpinningTop)) "MOVE_Walking" 0)
  (Variables|Default|SetisPlayerIn false)
  (Variables|Default|SetPlayerInSpinningTop 0)
  (Variables|Default|SetValueRotation (Variables|Default|GetDefaultValueRotation)))
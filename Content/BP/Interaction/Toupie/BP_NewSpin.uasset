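; BP_NewSpin is an interactable spinner that locks one player onto it and lets another player spin it up with a QTE input.
; The rider is snapped to the Lock component each tick, and the interact widget changes while the spinner is occupied.
; Held input accelerates RotatingMovement yaw up to MaxSpeed, and releasing it decelerates.
; While accelerating past a speed threshold, it reports a sublevel as discovered through LevelComunicationSubsystem.
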(event EventStartInteract
  (params (Player :type Character%20Player%20Object%20Reference))
  (bind _returnvalue (CallFunction|IsPlayerLocked))
  (if (not _returnvalue)
    (bind _output_get (Variables|Default|SetPlayerIn Player))
    (bind _returnvalue_2 (Class|CharacterPlayer|GetBlueprintAnim _output_get))
    (Class|BPIAnim|PlayAnim(Message) _returnvalue_2 "FishPull" "NewEnumerator1")))

(event EventTick
  (params (DeltaSeconds :type Float%20%28single-precision%29))
  (bind _returnvalue (CallFunction|IsPlayerLocked))
  (if _returnvalue
    (CallFunction|FixPlayer)
    (if (Variables|Default|GetIsTakingSpeed)
      (if (> (.yaw (Variables|/Script/Engine.RotatingMovementComponent|GetRotationRate (Variables|Default|GetRotatingMovement))) 5e+01)
        (Class|LevelComunicationSubsystem|DiscoveredSubLevel (Subsystems|GetLevelComunicationSubsystem) 1 1))
      (else
        (Variables|/Script/Engine.RotatingMovementComponent|SetRotationRate (Variables|Default|GetRotatingMovement) (Math|Rotator|MakeRotator 0.0 0.0 (Math|Float|Clamp(Float) (- (.yaw (Variables|/Script/Engine.RotatingMovementComponent|GetRotationRate (Variables|Default|GetRotatingMovement))) (* (Utilities|Time|GetWorldDeltaSeconds) (Variables|Default|GetAccelerationRate))) 0.0 (Variables|Default|GetMaxSpeed))))))))

(event EventOnInteract
  (params (Player :type Character%20Player%20Object%20Reference) (InputID :type EInputID%20Enum :default "QTE1"))
  (if (and (not (== Player (Variables|Default|GetPlayerIn))) (Utilities|Enum|Equal(Enum) InputID "QTE1"))
    (bind _returnvalue (CallFunction|IsPlayerLocked))
    (if _returnvalue
      (Variables|Default|SetIsTakingSpeed true)
      (Variables|/Script/Engine.RotatingMovementComponent|SetRotationRate (Variables|Default|GetRotatingMovement) (Math|Rotator|MakeRotator 0.0 0.0 (Math|Float|Clamp(Float) (+ (.yaw (Variables|/Script/Engine.RotatingMovementComponent|GetRotationRate (Variables|Default|GetRotatingMovement))) (* (Utilities|Time|GetWorldDeltaSeconds) (Variables|Default|GetAccelerationRate))) 0.0 (Variables|Default|GetMaxSpeed))))
      (CallFunction|FixPlayer))))

(event EventEndInteract
  (params (Player :type Character%20Player%20Object%20Reference))
  (bind _returnvalue (Class|CharacterPlayer|GetBlueprintAnim Player))
  (Class|BPIAnim|StopAnim(Message) _returnvalue))

(event EventSetCharacterinInteract
  (params (Player :type Character%20Player%20Object%20Reference))
  (Variables|Default|SetPlayerIn Player))

(event EventOnEndInteract
  (params (Player :type Character%20Player%20Object%20Reference) (InputID :type EInputID%20Enum :default "QTE1"))
  (Variables|Default|SetIsTakingSpeed false))

(fn ConstructionScript)

(fn FixPlayer
  (bind _playerin (Variables|Default|GetPlayerIn))
  (bind _lock (Variables|Default|GetLock))
  (Transformation|SetActorLocation _playerin (Transformation|GetWorldLocation _lock) false false)
  (Transformation|SetActorRotation _playerin (Transformation|GetWorldRotation _lock)))

(fn GetCharacterinInteract
  (return (Variables|Default|GetPlayerIn)))

(fn GetInteractWidget
  (bind _returnvalue (CallFunction|IsPlayerLocked))
  (if _returnvalue
    (return "/Game/BP/Widget/WBP_InteractY.WBP_InteractY_C")
    (else
      (return (Variables|Default|GetInteractWidget)))))

(fn GetPlayerLockParent
  (return (Variables|Default|GetLock)))

(fn GetUnlockTP
  (return (Variables|Default|GetOutTP)))

(fn IsPlayerLocked
  (return (Utilities|IsValid (Variables|Default|GetPlayerIn))))

(fn LockedPlayer
  (return true))
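; BP_Graine is an interactable seed spot where the player plants a small tree, which starts hidden.
; It implements interaction functions that store the player and supply lock and unlock points.
; The first QTE1 input triggers, after a short delay, an interact animation message on the player's anim blueprint and reveals PetitArbus.
; Logic to find and activate BP_Arbre is present but unconnected.
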(event Custom|CE_PLayAnim
  ;[0.15 0.15 0.15 0.5] Play Anim et event pour relier l'arbre
  (Utilities|FlowControl|Delay 0.2)
  (bind _returnvalue (Class|CharacterPlayer|GetBlueprintAnim (Variables|Default|GetPlayerIn)))
  (Class|BPIAnim|PlayInteract(Message) _returnvalue "NewEnumerator6")
  (Rendering|SetVisibility (Variables|Default|GetPetitArbus) true false))

(event EventStartInteract
  (params (Player :type Character%20Player%20Object%20Reference))
  (Variables|Default|SetPlayerIn Player))

(event EventSetCharacterinInteract
  (params (Player :type Character%20Player%20Object%20Reference))
  (Variables|Default|SetPlayerIn Player))

(event EventOnStartInteract
  (params (Player :type Character%20Player%20Object%20Reference) (InputID :type EInputID%20Enum :default "QTE1"))
  ;[0.15 0.15 0.15 0.5] OnStartInteract
  (if (Variables|Default|GetisFirstTime)
    (switch Utilities|FlowControl|Switch|SwitchonEInputID InputID
      (:QTE1
        (Variables|Default|SetisFirstTime false)
        (CallFunction|CEPLayAnim)))))

(event EventBeginPlay
  ;[0.15 0.15 0.15 0.5] EVENT BEGIN PLAY
  (Rendering|SetVisibility (Variables|Default|GetPetitArbus) false false))

(fn ConstructionScript)

(fn GetCharacterinInteract
  (return 0))

(fn GetInteractWidget
  (return 0))

(fn GetPlayerLockParent
  (return (Variables|Default|GetTpLock)))

(fn GetUnlockTP
  (return (Variables|Default|GetUnLock)))

(fn IsPlayerLocked
  (return (Utilities|IsValid (Variables|Default|GetPlayerIn))))

(fn LockedPlayer
  (return true))
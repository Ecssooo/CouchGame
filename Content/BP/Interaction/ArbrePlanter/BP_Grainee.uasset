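; BP_Grainee is an interactable seed, apparently part of tree planting, that locks the player during use.
; It stores the interacting player, treats a valid reference as locked, and exposes lock and unlock teleport points through interaction functions.
; On the QTE1 input it swaps the Graine material and plays an interact message on the player's anim Blueprint.
; StartInteract only prints a debug string, and no interact widget is provided.
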(event EventStartInteract
  (params (Player :type Character%20Player%20Object%20Reference))
  (bind _returnvalue (CallFunction|IsPlayerLocked))
  (if (not _returnvalue)
    (Development|PrintString "PlayerEntre")))

(event EventSetCharacterinInteract
  (params (Player :type Character%20Player%20Object%20Reference))
  (Variables|Default|SetPlayerIn Player))

(event EventOnStartInteract
  (params (Player :type Character%20Player%20Object%20Reference) (InputID :type EInputID%20Enum :default "QTE1"))
  (switch Utilities|FlowControl|Switch|SwitchonEInputID InputID
    (:QTE1
      (Rendering|Material|SetMaterial (Variables|Default|GetGraine) 0 "/Game/BP/Interaction/ArbrePlanter/M_Graine.M_Graine")
      (bind _returnvalue (Class|CharacterPlayer|GetBlueprintAnim (Variables|Default|GetPlayerIn)))
      (Class|BPIAnim|PlayInteract(Message) _returnvalue "NewEnumerator6"))))

(fn ConstructionScript)

(fn GetCharacterinInteract
  (return (Variables|Default|GetPlayerIn)))

(fn GetInteractWidget
  (return 0))

(fn GetPlayerLockParent
  (return (Variables|Default|GetTpLock)))

(fn GetUnlockTP
  (return (Variables|Default|GetUnLock)))

(fn IsPlayerLocked
  (return (Utilities|IsValid (Variables|Default|GetPlayerIn))))

(fn LockedPlayer
  (return true))
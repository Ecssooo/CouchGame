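; Two-player fishing minigame controller that pits two BP_NewPecheChild child actors against each other.
; Children report ready or unready; with both players in, it plays their interact animations, waits briefly, then shows QTEs and starts the Fishing timeline.
; Any other player count stops the QTEs and timeline.
; When the timeline finishes, the higher score wins, non-zero ties go to the second child, and both lose if neither scored.
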(event Custom|CE_PlayerReady
  ;[0.15 0.15 0.15 0.5] Player Ready
  (Math|Integer|IncrementInt (Variables|Default|GetPlayerCount)
    (:%20%20
      (CallFunction|CELaunchFIshing))))

(event Custom|CE_PlayerUnReady
  ;[0.15 0.15 0.15 0.5] Player unready
  (Math|Integer|DecrementInt (Variables|Default|GetPlayerCount)
    (:%20%20
      (CallFunction|CELaunchFIshing))))

(event Custom|CE_LaunchFIshing
  ;[0.15 0.15 0.15 0.5] Launch Fishing
  (Utilities|FlowControl|DelayUntilNextTick)
  (if (== (Variables|Default|GetPlayerCount) 2)
    (Variables|Default|SetIsPlay true)
    (bind _returnvalue (Class|CharacterPlayer|GetBlueprintAnim (Variables|/Game/BP/Interaction/Peche/BP_NewPecheChild.BP_NewPecheChild_C|GetPlayerIn (Variables|Default|GetFishChild1))))
    (Class|BPIAnim|PlayInteract(Message) _returnvalue "NewEnumerator5")
    (bind _returnvalue_2 (Class|CharacterPlayer|GetBlueprintAnim (Variables|/Game/BP/Interaction/Peche/BP_NewPecheChild.BP_NewPecheChild_C|GetPlayerIn (Variables|Default|GetFishChild2))))
    (Class|BPIAnim|PlayInteract(Message) _returnvalue_2 "NewEnumerator5")
    (Utilities|FlowControl|Delay 2.0)
    (if (Variables|Default|GetIsPlay)
      (Default|ShowQTE (Variables|Default|GetFishChild1))
      (Default|ShowQTE (Variables|Default|GetFishChild2))
      (CallFunction|CEStartFishing))
    (else
      (Variables|Default|SetIsPlay false)
      (Default|CEStopQTE (Variables|Default|GetFishChild1))
      (Default|CEStopQTE (Variables|Default|GetFishChild2))
      (CallFunction|CEStopFishing))))

(event Custom|CE_EndFish
  ;[0.15 0.15 0.15 0.5] CE EndFishing
  (if (Variables|Default|GetIsPlay)
    (if (!= (+ (Variables|/Game/BP/Interaction/Peche/BP_NewPecheChild.BP_NewPecheChild_C|GetPlayerScore (Variables|Default|GetFishChild1)) (Variables|/Game/BP/Interaction/Peche/BP_NewPecheChild.BP_NewPecheChild_C|GetPlayerScore (Variables|Default|GetFishChild2))) 0)
      (Variables|Default|SetIsPlay false)
      (if (> (Variables|/Game/BP/Interaction/Peche/BP_NewPecheChild.BP_NewPecheChild_C|GetPlayerScore (Variables|Default|GetFishChild1)) (Variables|/Game/BP/Interaction/Peche/BP_NewPecheChild.BP_NewPecheChild_C|GetPlayerScore (Variables|Default|GetFishChild2)))
        (Default|CEWin (Variables|Default|GetFishChild1))
        (Default|CELose (Variables|Default|GetFishChild2))
        (else
          (Default|CEWin (Variables|Default|GetFishChild2))
          (Default|CELose (Variables|Default|GetFishChild1))))
      (else
        (Default|CELose (Variables|Default|GetFishChild1))
        (Default|CELose (Variables|Default|GetFishChild2))))))

(event Custom|CE_StartFishing
  ;[0.15 0.15 0.15 0.5] CE Fishing (timeline)
  (Timeline|Fishing PlayFromStart
    (:Finished
      (CallFunction|CEEndFish))))

(event Custom|CE_StopFishing
  ;[0.15 0.15 0.15 0.5] CE Fishing (timeline)
  (Timeline|Fishing Stop
    (:Finished
      (CallFunction|CEEndFish))))

(event EventBeginPlay
  ;[0.15 0.15 0.15 0.5] Begin Play
  (bind _asbp_new_peche_child (Utilities|Casting|CastToBP_NewPecheChild (Variables|/Script/Engine.ChildActorComponent|GetChildActor (Variables|Default|GetBP_NewPecheChild1))))
  (Variables|Default|SetFishChild1 _asbp_new_peche_child)
  (bind _asbp_new_peche_child_2 (Utilities|Casting|CastToBP_NewPecheChild (Variables|/Script/Engine.ChildActorComponent|GetChildActor (Variables|Default|GetBP_NewPecheChild2))))
  (Variables|Default|SetFishChild2 _asbp_new_peche_child_2))

(fn ConstructionScript)
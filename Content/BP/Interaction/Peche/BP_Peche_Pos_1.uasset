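; Interactable player position for the fishing minigame, where a locked player presses a QTE input while a fish is present.
; Joining or leaving updates BP_Peche's player count and state; valid presses increment CounterPlayer and blink the prompt.
; Custom events handle start, stop, animations, outline and turning both widgets toward the world camera.
; CE_ShowWin stops play, briefly shows any win widget, returns the player to Idle and saves the interaction as completed.
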(event Custom|PlayQTE
  ;[0.15 0.15 0.15 0.5] QTE Play
  (CallFunction|HideQTE)
  (if (Variables|Default|GetIsPlay)
    (Utilities|FlowControl|Delay 0.1)
    (CallFunction|ShowQTE)))

(event Custom|CE_SetOutline
  (params (Isenable :type Boolean))
  (Rendering|SetRenderCustomDepth (Variables|Default|GetCube) Isenable))

(event Custom|CE_ShowWin
  (params (IsWin :type Boolean))
  (CallFunction|CEStop IsWin)
  (if IsWin
    (Rendering|SetVisibility (Variables|Default|GetWidget_WIN) true false))
  (Utilities|FlowControl|Delay 5.0)
  (Rendering|SetVisibility (Variables|Default|GetWidget_WIN) false false)
  (Class|PlayerStateMachine|ChangeState (Variables|/Script/CouchGame.CharacterPlayer|GetStateMachine (Variables|Default|GetPlayer%20In)) "Idle")
  (bind _returnvalue (Class|CharacterPlayer|GetBlueprintAnim (Variables|Default|GetPlayer%20In)))
  (Class|BPIAnim|StopInteract(Message) _returnvalue)
  (Class|SaveCubeSubsystem|SaveInteractionData (Subsystems|GetSaveCubeSubsystem) 102 true))

(event Custom|CE_RotationWidget
  (params (World%20camera :type Camera%20Actor%20Object%20Reference))
  (bind _rootcomponent (Variables|/Script/Engine.Actor|GetRootComponent World%20camera))
  (bind _widget (Variables|Default|GetWidget))
  (bind _widget_win (Variables|Default|GetWidget_WIN))
  (bind _rootcomponent_2 (Variables|/Script/Engine.Actor|GetRootComponent World%20camera))
  (bind _returnvalue (Transformation|GetWorldLocation _widget))
  (bind _returnvalue_2 (Transformation|GetWorldLocation _rootcomponent))
  (bind _returnvalue_3 (Transformation|GetWorldLocation _widget_win))
  (bind _returnvalue_4 (Transformation|GetWorldLocation _rootcomponent_2))
  (bind _returnvalue_5 (Math|Rotator|FindLookatRotation _returnvalue _returnvalue_2))
  (bind _returnvalue_6 (Math|Rotator|FindLookatRotation _returnvalue_3 _returnvalue_4))
  ;[0.15 0.15 0.15 0.5] Rotation widget
  (Transformation|SetWorldRotation (Variables|Default|GetWidget) (Math|Rotator|MakeRotator (.roll (Transformation|GetWorldRotation _widget)) (.pitch _returnvalue_5) (.yaw _returnvalue_5)) false false)
  (Transformation|SetWorldRotation (Variables|Default|GetWidget_WIN) (Math|Rotator|MakeRotator (.roll (Transformation|GetWorldRotation _widget_win)) (.pitch _returnvalue_6) (.yaw _returnvalue_6)) false false))

(event Custom|CE_PlayAnimStopPeche
  (params (IsWin :type Boolean))
  (if IsWin
    (bind _returnvalue (Class|CharacterPlayer|GetBlueprintAnim (Variables|Default|GetPlayer%20In)))
    (Class|BPIAnim|PlayInteract(Message) _returnvalue "NewEnumerator1")))

(event Custom|CE_Start
  (Variables|Default|SetIsPlay true)
  (CallFunction|ShowQTE))

(event Custom|CE_Stop
  (params (IsWin :type Boolean))
  (Variables|Default|SetIsPlay false)
  (CallFunction|HideQTE)
  (CallFunction|CEPlayAnimStopPeche IsWin))

(event Custom|CE_PlayAnimStartPeche
  (bind _returnvalue (Class|CharacterPlayer|GetBlueprintAnim (Variables|Default|GetPlayer%20In)))
  (Class|BPIAnim|PlayInteract(Message) _returnvalue "NewEnumerator5"))

(event EventBeginPlay
  (bind _returnvalue (Actor|GetActorOfClass "/Game/BP/Interaction/Peche/BP_Peche.BP_Peche_C"))
  (Variables|Default|SetBP_Peche _returnvalue)
  (bind _returnvalue_2 (Actor|GetActorOfClass "/Game/BP/Camera/BP_CameraActor.BP_CameraActor_C"))
  (Variables|Default|SetWorldCamera _returnvalue_2))

(event EventEndInteract
  (params (Player :type Character%20Player%20Object%20Reference))
  (bind _bp_peche (Variables|Default|GetBP_Peche))
  ;[0.15 0.15 0.15 0.5] ENDInteract
  (Development|PrintString "StopInteract" true true "(R=1.000000,G=0.000000,B=0.027276,A=1.000000)")
  (Math|Integer|DecrementInt (Variables|/Game/BP/Interaction/Peche/BP_Peche.BP_Peche_C|GetNumberPlayer _bp_peche)
    (:%20%20
      (Default|StateInteraction _bp_peche)
      (CallFunction|CEStop false)
      (Class|PlayerStateMachine|ChangeState (Variables|/Script/CouchGame.CharacterPlayer|GetStateMachine (Variables|Default|GetPlayer%20In)) "Idle")
      (bind _returnvalue (Class|CharacterPlayer|GetBlueprintAnim (Variables|Default|GetPlayer%20In)))
      (Class|BPIAnim|StopInteract(Message) _returnvalue))))

(event EventOnStartInteract
  (params (Player :type Character%20Player%20Object%20Reference) (InputID :type EInputID%20Enum :default "QTE1"))
  ;[0.15 0.15 0.15 0.5] OnStartInteract
  (if (Variables|Default|GetIsPlay)
    (switch Utilities|FlowControl|Switch|SwitchonEInputID InputID
      (:QTE1
        (if (Variables|/Game/BP/Interaction/Peche/BP_Peche.BP_Peche_C|GetIsFish (Variables|Default|GetBP_Peche))
          (Math|Integer|IncrementInt (Variables|Default|GetCounterPlayer)
            (:%20%20
              (Development|PrintString "OK")
              (CallFunction|PlayQTE))))))))

(event EventStartInteract
  (params (Player :type Character%20Player%20Object%20Reference))
  (bind _bp_peche (Variables|Default|GetBP_Peche))
  ;[0.15 0.15 0.15 0.5] StartInteract
  (Variables|Default|SetPlayer%20In Player)
  (Development|PrintString "Interact_Peche" true true "(R=0.000000,G=1.000000,B=0.017657,A=1.000000)")
  (Math|Integer|IncrementInt (Variables|/Game/BP/Interaction/Peche/BP_Peche.BP_Peche_C|GetNumberPlayer _bp_peche)
    (:%20%20
      (Default|StateInteraction _bp_peche))))

(event EventSetCharacterinInteract
  (params (Player :type Character%20Player%20Object%20Reference))
  ;[0.15 0.15 0.15 0.5] SET Character Interact
  (Variables|Default|SetPlayer%20In Player))

(fn ConstructionScript)

(fn StartPeche)

(fn ShowQTE
  (if (Variables|Default|GetIsPlay)
    (Rendering|SetVisibility (Variables|Default|GetWidget) true false)))

(fn HideQTE
  (Rendering|SetVisibility (Variables|Default|GetWidget) false false))

(fn GetCharacterinInteract
  (return 0))

(fn GetInteractWidget
  (return (Variables|Default|GetInteractWidget)))

(fn GetPlayerLockParent
  (return (Variables|Default|GetTpLock)))

(fn GetUnlockTP
  (return (Variables|Default|GetTpUnLock)))

(fn IsPlayerLocked
  (return (Utilities|IsValid 0)))

(fn LockedPlayer
  (return true))
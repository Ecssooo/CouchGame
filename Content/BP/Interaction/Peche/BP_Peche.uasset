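; BP_Peche runs a two-player fishing minigame, coordinating the BP_Peche_Pos_1 and BP_Peche_Pos_2 actors found at BeginPlay.
; With two players, it plays start animations, waits for the fish, then opens a timed catch window.
; Tick declares the first position reaching NumberForWin the winner and prints a fish drawn by Percentage from FishStruct.
; A timeout ends the round as a defeat, and outline highlights forward to both positions.
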(event Custom|CE_StartInteraction
  ;[0.15 0.15 0.15 0.5] Start Interaction
  (CallFunction|CERotationWidget)
  (Variables|Default|SetisEnd true)
  (Default|CEPlayAnimStartPeche (Variables|Default|GetBP_Peche_Pos_1))
  (Default|CEPlayAnimStartPeche (Variables|Default|GetBP_Peche_Pos_2))
  (Development|PrintString "PoissonArrive")
  (Utilities|FlowControl|Delay (Variables|Default|GetDelayFishStart))
  (if (Variables|Default|GetIsGamePeche)
    (Variables|Default|SetIsFish true)
    (Development|PrintString "PoissonEstLa")
    (Default|CEStart (Variables|Default|GetBP_Peche_Pos_1))
    (Default|CEStart (Variables|Default|GetBP_Peche_Pos_2))
    (Utilities|FlowControl|Delay (Variables|Default|GetDelayFishEnd))
    (if (Variables|Default|GetIsGamePeche)
      (CallFunction|CEEndInteraction)
      (elif (Variables|Default|GetisEnd)
        (CallFunction|CEENGAME)))
    (elif (Variables|Default|GetisEnd)
      (CallFunction|CEENGAME))))

(event Custom|CE_RotationWidget
  ;[0.15 0.15 0.15 0.5] Rotation Widget
  (Default|CERotationWidget (Variables|Default|GetBP_Peche_Pos_1) (Variables|Default|GetWorldCamera))
  (Default|CERotationWidget (Variables|Default|GetBP_Peche_Pos_2) (Variables|Default|GetWorldCamera)))

(event Custom|CE_ENGAME
  ;[0.15 0.15 0.15 0.5] END_Game
  (Development|PrintString "END Game")
  (Variables|Default|SetisEnd false)
  (Variables|Default|SetIsGamePeche false)
  (Variables|Default|SetIsFish false)
  (Variables|/Game/BP/Interaction/Peche/BP_Peche_Pos_1.BP_Peche_Pos_1_C|SetCounterPlayer (Variables|Default|GetBP_Peche_Pos_1) 0)
  (Variables|/Game/BP/Interaction/Peche/BP_Peche_Pos_2.BP_Peche_Pos_2_C|SetCounterPlayer (Variables|Default|GetBP_Peche_Pos_2) 0)
  (Default|CEShowWin (Variables|Default|GetBP_Peche_Pos_2) false)
  (Default|CEShowWin (Variables|Default|GetBP_Peche_Pos_1) false))

(event Custom|CE_EndInteraction
  ;[0.15 0.15 0.15 0.5] END Interaction
  (Development|PrintString "Interaction Fini / defaite")
  (CallFunction|CEENGAME))

(event Custom|CE_Pos2_Player_Win
  ;[0.15 0.15 0.15 0.5] PlayerWin_2
  (Development|PrintString "GAME REUSSIE" true true "(R=0.019072,G=1.000000,B=0.000000,A=1.000000)")
  (Development|PrintString "Player 2 WIN")
  (bind _fishdrop (CallFunction|GetRandomFish))
  (Development|PrintString (Utilities|String|Append "Pos 2 : " (Utilities|String|ToString(Name) _fishdrop)))
  (Default|CEShowWin (Variables|Default|GetBP_Peche_Pos_2) true)
  (Default|CEShowWin (Variables|Default|GetBP_Peche_Pos_1) false)
  (Development|PrintString "END Game")
  (Variables|Default|SetisEnd false)
  (Variables|Default|SetIsGamePeche false)
  (Variables|Default|SetIsFish false)
  (Variables|/Game/BP/Interaction/Peche/BP_Peche_Pos_1.BP_Peche_Pos_1_C|SetCounterPlayer (Variables|Default|GetBP_Peche_Pos_1) 0)
  (Variables|/Game/BP/Interaction/Peche/BP_Peche_Pos_2.BP_Peche_Pos_2_C|SetCounterPlayer (Variables|Default|GetBP_Peche_Pos_2) 0))

(event Custom|CE_SpawnResult
  (params (FishPack :type String))
  (bind _widget_fish_pack (Variables|Default|GetWidget_Fish_Pack))
  ;[0.15 0.15 0.15 0.5] Spawn Result
  (Rendering|SetVisibility _widget_fish_pack true true)
  (bind _aswbp_peche_fish_pack (Utilities|Casting|CastToWBP_Peche_FishPack (UserInterface|GetWidget _widget_fish_pack)))
  (Variables|/Game/BP/Interaction/Peche/WBP_Peche_FishPack.WBP_Peche_FishPack_C|SetMyText _aswbp_peche_fish_pack (Utilities|String|ToString(Text) (Utilities|Text|ToText(String) FishPack)))
  (Utilities|FlowControl|Delay 5.0)
  (Rendering|SetVisibility (Variables|Default|GetWidget_Fish_Pack) false false))

(event Custom|CE_Pos1_Player_Win
  ;[0.15 0.15 0.15 0.5] PlayerWin_1
  (Development|PrintString "GAME REUSSIE" true true "(R=0.019072,G=1.000000,B=0.000000,A=1.000000)")
  (Development|PrintString "Player 1 WIN")
  (bind _fishdrop (CallFunction|GetRandomFish))
  (Development|PrintString (Utilities|String|Append "Pos 1 : " (Utilities|String|ToString(Name) _fishdrop)))
  (Default|CEShowWin (Variables|Default|GetBP_Peche_Pos_1) true)
  (Default|CEShowWin (Variables|Default|GetBP_Peche_Pos_2) false)
  (Development|PrintString "END Game")
  (Variables|Default|SetisEnd false)
  (Variables|Default|SetIsGamePeche false)
  (Variables|Default|SetIsFish false)
  (Variables|/Game/BP/Interaction/Peche/BP_Peche_Pos_1.BP_Peche_Pos_1_C|SetCounterPlayer (Variables|Default|GetBP_Peche_Pos_1) 0)
  (Variables|/Game/BP/Interaction/Peche/BP_Peche_Pos_2.BP_Peche_Pos_2_C|SetCounterPlayer (Variables|Default|GetBP_Peche_Pos_2) 0))

(event EventTick
  (params (DeltaSeconds :type Float%20%28single-precision%29))
  ;[0.15 0.15 0.15 0.5] Event Tick
  (if (Variables|Default|GetIsGamePeche)
    (if (Variables|Default|GetIsFish)
      (Utilities|FlowControl|Sequence
        (:then_0
          (if (>= (Variables|/Game/BP/Interaction/Peche/BP_Peche_Pos_1.BP_Peche_Pos_1_C|GetCounterPlayer (Variables|Default|GetBP_Peche_Pos_1)) (Variables|Default|GetNumberForWin))
            (CallFunction|CEPos1PlayerWin)))
        (:then_1
          (if (>= (Variables|/Game/BP/Interaction/Peche/BP_Peche_Pos_2.BP_Peche_Pos_2_C|GetCounterPlayer (Variables|Default|GetBP_Peche_Pos_2)) (Variables|Default|GetNumberForWin))
            (CallFunction|CEPos2PlayerWin)))))))

(event EventHighlightInteraction
  (params (IsHighlight :type Boolean))
  ;[0.15 0.15 0.15 0.5] Highlight
  (Default|CESetOutline (Variables|Default|GetBP_Peche_Pos_1) IsHighlight)
  (Default|CESetOutline (Variables|Default|GetBP_Peche_Pos_2) IsHighlight))

(event EventBeginPlay
  ;[0.15 0.15 0.15 0.5] Begin Play
  (bind _returnvalue (Actor|GetActorOfClass "/Game/BP/Interaction/Peche/BP_Peche_Pos_1.BP_Peche_Pos_1_C"))
  (Variables|Default|SetBP_Peche_Pos_1 _returnvalue)
  (bind _returnvalue_2 (Actor|GetActorOfClass "/Game/BP/Interaction/Peche/BP_Peche_Pos_2.BP_Peche_Pos_2_C"))
  (Variables|Default|SetBP_Peche_Pos_2 _returnvalue_2)
  (bind _returnvalue_3 (Actor|GetActorOfClass "/Script/Engine.CameraActor"))
  (Variables|Default|SetWorldCamera _returnvalue_3)
  (bind _returnvalue_4 (UserInterface|CreateWidget "/Game/BP/Interaction/Peche/WBP_Peche_FishPack.WBP_Peche_FishPack_C"))
  (Variables|Default|SetFishPack _returnvalue_4))

(fn ConstructionScript)

(fn StateInteraction
  (if (== (Variables|Default|GetNumberPlayer) 2)
    (Variables|Default|SetIsGamePeche true)
    (CallFunction|CEStartInteraction)
    (else
      (Variables|Default|SetIsGamePeche false)
      (Variables|Default|SetIsFish false))))

(fn GetRandomFish
  (for _array_element (Variables|Default|GetFishStruct)
    (Variables|Default|SetTotalChance (+ (.Percentage (Utilities|Struct|BreakS_Fish _array_element)) (Variables|Default|GetTotalChance)))
    (Variables|Default|SetRandomValue (Math|Random|RandomFloatinRange 0.0 (Variables|Default|GetTotalChance)))
    (for _array_element_2 (Variables|Default|GetFishStruct)
      (if (<= (Variables|Default|GetRandomValue) (.Percentage (Utilities|Struct|BreakS_Fish _array_element_2)))
        (return (Utilities|String|StringToName (.Name (Utilities|Struct|BreakS_Fish _array_element_2))))
        (else
          (Variables|Default|SetRandomValue (- (Variables|Default|GetRandomValue) (.Percentage (Utilities|Struct|BreakS_Fish _array_element_2)))))))))
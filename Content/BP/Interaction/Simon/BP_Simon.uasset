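; Interactable Simon memory minigame where the player repeats a growing random sequence of four colors with QTE inputs.
; Interacting swaps input mapping contexts and shows a camera-facing WBP_Simon widget.
; A delayed recursive event plays the sequence with sounds while input is blocked, then checks each press, restarting on mistakes.
; Reaching maximum length saves interaction 202 as completed and returns the player to Idle; once completed, replays grow without limit.
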(event Custom|ShowSolution
  ;[0.15 0.15 0.15 0.5] Show Solution
  (Development|PrintString "Enter ShowSolution")
  (Variables|Default|SetIndexList 0)
  (Utilities|FlowControl|Delay 1.0)
  (CallFunction|BoucleShowSolution))

(event Custom|BoucleShowSolution
  ;[0.15 0.15 0.15 0.5] Boucle de Show Solution
  (Utilities|FlowControl|Sequence
    (:then_0
      (switch int (Utilities|Array|Get(acopy) (Variables|Default|GetListSolution) (Variables|Default|GetIndexList))
        (:0
          (Default|FGreenClick (Variables|Default|GetAs%20WBP%20Simon) (Variables|Default|GetTimeClick) true)
          (Class|SoundManager|PlaySound (Subsystems|GetSoundManager) "SFX_Color_Switch_01" (Variables|Default|GetAudio)))
        (:1
          (Default|FRedClick (Variables|Default|GetAs%20WBP%20Simon) (Variables|Default|GetTimeClick) true)
          (Class|SoundManager|PlaySound (Subsystems|GetSoundManager) "SFX_Color_Switch_02" (Variables|Default|GetAudio)))
        (:2
          (Default|FBlueClick (Variables|Default|GetAs%20WBP%20Simon) (Variables|Default|GetTimeClick) true)
          (Class|SoundManager|PlaySound (Subsystems|GetSoundManager) "SFX_Color_Switch_03" (Variables|Default|GetAudio)))
        (:3
          (Default|FYellowClick (Variables|Default|GetAs%20WBP%20Simon) (Variables|Default|GetTimeClick) true)
          (Class|SoundManager|PlaySound (Subsystems|GetSoundManager) "SFX_Color_Switch_04" (Variables|Default|GetAudio)))))
    (:then_1
      (Utilities|FlowControl|Delay 0.5)
      (Math|Integer|IncrementInt (Variables|Default|GetIndexList)
        (:%20%20
          (if (>= (Variables|Default|GetIndexList) (Utilities|Array|Length (Variables|Default|GetListSolution)))
            (Variables|Default|SetListen false)
            (Variables|Default|SetIndexList 0)
            (Development|PrintString "Exit ShowSolution")
            (else
              (CallFunction|BoucleShowSolution))))))))

(event EventSetCharacterinInteract
  (params (Player :type Character%20Player%20Object%20Reference))
  ;[0.15 0.15 0.15 0.5] Start Set Character Interact
  (Variables|Default|SetPlayerIn Player))

(event EventTick
  (params (DeltaSeconds :type Float%20%28single-precision%29))
  (bind _worldcamera (Variables|Default|GetWorldCamera))
  (bind _widget (Variables|Default|GetWidget))
  (bind _returnvalue (Transformation|GetWorldLocation _widget))
  (bind _rootcomponent (Variables|/Script/Engine.Actor|GetRootComponent _worldcamera))
  (bind _returnvalue_2 (Transformation|GetWorldLocation _rootcomponent))
  (bind _returnvalue_3 (Math|Rotator|FindLookatRotation _returnvalue _returnvalue_2))
  ;[0.15 0.15 0.15 0.5] Rotation Widget
  (if (Variables|Default|GetIsInInteract)
    (Transformation|SetWorldRotation (Variables|Default|GetWidget) (Math|Rotator|MakeRotator (.roll (Transformation|GetWorldRotation (Variables|Default|GetWidget))) (.pitch _returnvalue_3) (.yaw _returnvalue_3)) false false)))

(event EventBeginPlay
  ;[0.15 0.15 0.15 0.5] Begin Play
  (bind _returnvalue (Actor|GetActorOfClass "/Game/BP/Camera/BP_CameraActor.BP_CameraActor_C"))
  (Variables|Default|SetWorldCamera _returnvalue))

(event EventStartInteract
  (params (Player :type Character%20Player%20Object%20Reference))
  ;[0.15 0.15 0.15 0.5] Start Interact
  ;;[0.15 0.15 0.15 0.5] Get WBP_Simon
  (bind _aswbp_simon (Utilities|Casting|CastToWBP_Simon (UserInterface|GetUserWidgetObject (Variables|Default|GetWidget))))
  (Variables|Default|SetAs%20WBP%20Simon _aswbp_simon)
  (CallFunction|FInitListSolution)
  (CallFunction|FClearListPlayer)
  (Variables|Default|SetListen true)
  (CallFunction|ShowSolution)
  (Variables|Default|SetIsInInteract true)
  (Rendering|SetVisibility (Variables|Default|GetWidget) true false)
  (if (not (Utilities|GetClassDefaults "/Script/CouchGame.CharacterSettings"))
    (bind _playerindex (Class|BPIPlayer|GetPlayerIndex(Message) Player))
    (Input|RemoveMappingContext (PlayerController|LocalPlayerSubsystems|GetEnhancedInputLocalPlayerSubsystem (Game|GetPlayerController _playerindex)) "/Game/Input/IMC_Player.IMC_Player" "(bIgnoreAllPressedKeysUntilRelease=True,bForceImmediately=False,bNotifyUserSettings=False)")
    (Input|AddMappingContext (PlayerController|LocalPlayerSubsystems|GetEnhancedInputLocalPlayerSubsystem (Game|GetPlayerController _playerindex)) "/Game/Input/IMC_Simon.IMC_Simon" 0 "(bIgnoreAllPressedKeysUntilRelease=True,bForceImmediately=False,bNotifyUserSettings=False)")))

(event EventHighlightInteraction
  (params (IsHighlight :type Boolean))
  (Rendering|SetVisibility (Variables|Default|GetCylinder) IsHighlight false))

(event EventOnStartInteract
  (params (Player :type Character%20Player%20Object%20Reference) (InputID :type EInputID%20Enum :default "QTE1"))
  ;[0.15 0.15 0.15 0.5] Interact
  (if (not (Variables|Default|GetListen))
    (switch Utilities|FlowControl|Switch|SwitchonEInputID InputID
      (:QTE1
        (Class|SoundManager|PlaySound (Subsystems|GetSoundManager) "SFX_Color_Switch_01" (Variables|Default|GetAudio))
        (bind _iscorrect (CallFunction|FIsCorrectNote))
        (if _iscorrect
          (CallFunction|FAddNotePlayer)
          (Default|FGreenClick (Variables|Default|GetAs%20WBP%20Simon) (Variables|Default|GetTimeClick) false)
          (if (== (Utilities|Array|Length (Variables|Default|GetListSolution)) (Utilities|Array|Length (Variables|Default|GetListPlayer))) :!label _label
            (bind _returnvalue (Class|SaveCubeSubsystem|GetInteractionsDatasfromID (Subsystems|GetSaveCubeSubsystem) 202))
            (if (.iscompleted _returnvalue)
              (Variables|Default|SetListen true :!label _label_2)
              (CallFunction|FClearListPlayer)
              (Utilities|FlowControl|Delay 1.0)
              (CallFunction|FAddNewNoteListSolution)
              (CallFunction|ShowSolution)
              (elif (== (Utilities|Array|Length (Variables|Default|GetListSolution)) (Variables|Default|GetListeSizeMax))
                (Rendering|SetVisibility (Variables|Default|GetWidget) false false)
                (Class|SaveCubeSubsystem|SaveInteractionData (Subsystems|GetSaveCubeSubsystem) 202 true)
                (Class|PlayerStateMachine|ChangeState (Variables|/Script/CouchGame.CharacterPlayer|GetStateMachine (Variables|Default|GetPlayerIn)) "Idle")
                (else
                  (goto _label_2)))))
          (else
            (Default|FAnimDeath (Variables|Default|GetAs%20WBP%20Simon))
            (Utilities|FlowControl|Delay 2.0)
            (Variables|Default|SetListen true)
            (CallFunction|FClearListPlayer)
            (CallFunction|FInitListSolution)
            (CallFunction|ShowSolution))))
      (:QTE2
        (Class|SoundManager|PlaySound (Subsystems|GetSoundManager) "SFX_Color_Switch_02" (Variables|Default|GetAudio))
        (bind _iscorrect_2 (CallFunction|FIsCorrectNote 1))
        (if _iscorrect_2
          (CallFunction|FAddNotePlayer 1)
          (Default|FRedClick (Variables|Default|GetAs%20WBP%20Simon) (Variables|Default|GetTimeClick) false)
          (goto _label)
          (else
            (Default|FAnimDeath (Variables|Default|GetAs%20WBP%20Simon))
            (Utilities|FlowControl|Delay 2.0)
            (Variables|Default|SetListen true)
            (CallFunction|FClearListPlayer)
            (CallFunction|FInitListSolution)
            (CallFunction|ShowSolution))))
      (:QTE3
        (Class|SoundManager|PlaySound (Subsystems|GetSoundManager) "SFX_Color_Switch_03" (Variables|Default|GetAudio))
        (bind _iscorrect_3 (CallFunction|FIsCorrectNote 2))
        (if _iscorrect_3
          (CallFunction|FAddNotePlayer 2)
          (Default|FBlueClick (Variables|Default|GetAs%20WBP%20Simon) (Variables|Default|GetTimeClick) false)
          (goto _label)
          (else
            (Default|FAnimDeath (Variables|Default|GetAs%20WBP%20Simon))
            (Utilities|FlowControl|Delay 2.0)
            (Variables|Default|SetListen true)
            (CallFunction|FClearListPlayer)
            (CallFunction|FInitListSolution)
            (CallFunction|ShowSolution))))
      (:QTE4
        (Class|SoundManager|PlaySound (Subsystems|GetSoundManager) "SFX_Color_Switch_04" (Variables|Default|GetAudio))
        (bind _iscorrect_4 (CallFunction|FIsCorrectNote 3))
        (if _iscorrect_4
          (CallFunction|FAddNotePlayer 3)
          (Default|FYellowClick (Variables|Default|GetAs%20WBP%20Simon) (Variables|Default|GetTimeClick) false)
          (goto _label)
          (else
            (Default|FAnimDeath (Variables|Default|GetAs%20WBP%20Simon))
            (Utilities|FlowControl|Delay 2.0)
            (Variables|Default|SetListen true)
            (CallFunction|FClearListPlayer)
            (CallFunction|FInitListSolution)
            (CallFunction|ShowSolution)))))))

(event EventEndInteract
  (params (Player :type Character%20Player%20Object%20Reference))
  ;[0.15 0.15 0.15 0.5] End Interact
  (Variables|Default|SetIsInInteract false)
  (Rendering|SetVisibility (Variables|Default|GetWidget) false false)
  (if (not (Utilities|GetClassDefaults "/Script/CouchGame.CharacterSettings"))
    (bind _playerindex (Class|BPIPlayer|GetPlayerIndex(Message) Player))
    (Input|RemoveMappingContext (PlayerController|LocalPlayerSubsystems|GetEnhancedInputLocalPlayerSubsystem (Game|GetPlayerController _playerindex)) "/Game/Input/IMC_Simon.IMC_Simon" "(bIgnoreAllPressedKeysUntilRelease=True,bForceImmediately=False,bNotifyUserSettings=False)")
    (Input|AddMappingContext (PlayerController|LocalPlayerSubsystems|GetEnhancedInputLocalPlayerSubsystem (Game|GetPlayerController _playerindex)) "/Game/Input/IMC_Player.IMC_Player" 0 "(bIgnoreAllPressedKeysUntilRelease=True,bForceImmediately=False,bNotifyUserSettings=False)")))

(fn ConstructionScript)

(fn FInitListSolution
  (Utilities|Array|Clear (Variables|Default|GetListSolution))
  (for _index (range 0 (Variables|Default|GetListeSizeStart))
    (CallFunction|FAddNewNoteListSolution)))

(fn FAddNewNoteListSolution
  (Utilities|Array|Add (Variables|Default|GetListSolution) (Math|Random|RandomInteger 4))
  (return))

(fn FClearListPlayer
  (Utilities|Array|Clear (Variables|Default|GetListPlayer)))

(fn FIsCorrectNote
  (params (Note :type Integer))
  (return (== Note (Utilities|Array|Get(acopy) (Variables|Default|GetListSolution) (Variables|Default|GetIndexList)))))

(fn FAddNotePlayer
  (params (Note :type Integer))
  (Utilities|Array|Add (Variables|Default|GetListPlayer) Note)
  (Math|Integer|IncrementInt (Variables|Default|GetIndexList)
    (:%20%20
      (return))))

(fn GetCharacterinInteract
  (return (Variables|Default|GetPlayerIn)))

(fn GetInteractWidget
  (return 0))

(fn GetPlayerLockParent
  (return (Variables|Default|GetLockParent)))

(fn GetUnlockTP
  (return (Variables|Default|GetLockParent)))

(fn IsPlayerLocked
  (return (Utilities|IsValid (Variables|Default|GetPlayerIn))))

(fn LockedPlayer
  (return true))
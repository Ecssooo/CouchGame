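; Two-player cooperative hut-building interaction, completed through a series of simultaneous QTEs.
; Two BP_Cabane0 child actors report ready, unready and QTE results; once both players are ready, both QTEs start together.
; Each joint success hides another group of construction-site props, revealing the hut at step five, and reaching the max count locks the interaction.
; A failure or a player leaving resets progress and visuals, with failures retrying after a delay.
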(event Custom|CE_PlayerUnready
  (params (Player :type BP%20Character%20Player%20Object%20Reference))
  (Variables|Default|SetCountQTE 0)
  (Math|Integer|DecrementInt (Variables|Default|GetCountPlayerReady)
    (:%20%20
      (CallFunction|CEStopQTE)
      (if (<= (Variables|Default|GetCountPlayerReady) 0)
        (Variables|Default|SetCountPlayerReady 0)))))

(event Custom|CE_PlayerReady
  (params (Player :type BP%20Character%20Player%20Object%20Reference))
  (if (not (Variables|Default|GetInteractCheck))
    (CallFunction|FResetAffichage)
    (bind _result (Math|Integer|IncrementInt (Variables|Default|GetCountPlayerReady))
      (:%20%20
        (if (>= _result 2)
          (Variables|Default|SetCountPlayerReady 2)
          (CallFunction|CEPlayQTE))))))

(event Custom|CE_IsEnd
  (CallFunction|FNextAffichage)
  (if (== (Variables|Default|GetCountQTE) (Variables|Default|GetCountMaxQTE))
    (Variables|Default|SetCountQTE 0)
    (Variables|Default|SetInteractCheck true)
    (Development|PrintString "WIN")
    (else
      (Utilities|FlowControl|Delay (Variables|Default|GetTimeBetween2QTE))
      (Utilities|IsPlayable
        (:true
          (Development|PrintString "5555")
          (CallFunction|CEPlayQTE))))))

(event Custom|CE_PlayQTE
  (Development|PrintString (Utilities|String|ToString(Integer) (Variables|Default|GetCountQTE)))
  (if (not (Variables|Default|GetInteractCheck))
    (Utilities|IsPlayable
      (:true
        (if true
          (Default|CEPlayQTE (Variables|Default|GetAs%20BP%20Cabane%200) (Variables|Default|GetTimeQTEDuration))
          (Default|CEPlayQTE (Variables|Default|GetAs%20BP%20Cabane%201) (Variables|Default|GetTimeQTEDuration))
          (Variables|Default|SetCanClick true))))))

(event Custom|CE_StopQTE
  (if (not (Variables|Default|GetInteractCheck))
    (CallFunction|FResetAffichage)
    (Variables|Default|SetCountQTE 0)
    (Default|CEStopQTE (Variables|Default|GetAs%20BP%20Cabane%200))
    (Default|CEStopQTE (Variables|Default|GetAs%20BP%20Cabane%201))))

(event Custom|CE_IsQTEWin
  (params (IsWin :type Boolean))
  (if (Variables|Default|GetCanClick)
    (if IsWin
      (Math|Integer|IncrementInt (Variables|Default|GetCountQTEWin)
        (:%20%20
          _)))
    (Math|Integer|IncrementInt (Variables|Default|GetCountPlayerInQTE)
      (:%20%20
        (if (== (Variables|Default|GetCountPlayerInQTE) 2)
          (Variables|Default|SetCountPlayerInQTE 0)
          (if (== (Variables|Default|GetCountQTEWin) 2)
            (Variables|Default|SetCountQTEWin 0)
            (Math|Integer|IncrementInt (Variables|Default|GetCountQTE)
              (:%20%20
                (Development|PrintString "TRUUUUUUE" true true "(R=0.000000,G=0.000000,B=0.000000,A=1.000000)")
                (CallFunction|CEIsEnd)))
            (else
              (Variables|Default|SetCountQTEWin 0)
              (Variables|Default|SetCanClick false)
              (CallFunction|CEStopQTE)
              (Utilities|FlowControl|Delay (Variables|Default|GetTimeQTEForStart))
              (Utilities|IsPlayable
                (:true
                  (Development|PrintString "66666")
                  (CallFunction|CEPlayQTE))))))))))

(event EventBeginPlay
  (Utilities|FlowControl|Sequence
    (:then_0
      (bind _asbp_cabane_0 (Utilities|Casting|CastToBP_Cabane0 (Variables|/Script/Engine.ChildActorComponent|GetChildActor (Variables|Default|GetBP_Cabane0))))
      (bind _output_get (Variables|Default|SetAs%20BP%20Cabane%200 _asbp_cabane_0))
      (EventDispatchers|BindEventtoEDPlayerReady _output_get (EventDispatchers|CreateEvent :!event Custom|CE_PlayerReady))
      (EventDispatchers|BindEventtoEDPlayerUnready (Variables|Default|GetAs%20BP%20Cabane%200) (EventDispatchers|CreateEvent :!event Custom|CE_PlayerUnready))
      (EventDispatchers|BindEventtoEDIsQTEWin (Variables|Default|GetAs%20BP%20Cabane%200) (EventDispatchers|CreateEvent :!event Custom|CE_IsQTEWin)))
    (:then_1
      (bind _asbp_cabane_0_2 (Utilities|Casting|CastToBP_Cabane0 (Variables|/Script/Engine.ChildActorComponent|GetChildActor (Variables|Default|GetBP_Cabane1))))
      (bind _output_get_2 (Variables|Default|SetAs%20BP%20Cabane%201 _asbp_cabane_0_2))
      (EventDispatchers|BindEventtoEDPlayerReady _output_get_2 (EventDispatchers|CreateEvent :!event Custom|CE_PlayerReady))
      (EventDispatchers|BindEventtoEDPlayerUnready (Variables|Default|GetAs%20BP%20Cabane%201) (EventDispatchers|CreateEvent :!event Custom|CE_PlayerUnready))
      (EventDispatchers|BindEventtoEDIsQTEWin (Variables|Default|GetAs%20BP%20Cabane%201) (EventDispatchers|CreateEvent :!event Custom|CE_IsQTEWin)))))

(fn ConstructionScript)

(fn FNextAffichage
  (switch int (Variables|Default|GetCountQTE)
    (:1
      (Utilities|Show1))
    (:2
      (Utilities|Show2))
    (:3
      (Utilities|Show3))
    (:4
      (Utilities|Show4))
    (:5
      (Rendering|SetVisibility (Variables|Default|GetSM_Hut) true false))))

(fn FResetAffichage
  (Rendering|SetVisibility (Variables|Default|GetSM_Hut) false false)
  (for _array_element (Components|GetChildrenComponents (Variables|Default|GetChantier) false)
    (Rendering|SetVisibility _array_element true false)))
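; Interactable cabin (Cabane) station that locks the player and runs a directional quick-time event.
; PlayQTE shows a world-space WBP_QTE widget with a random prompt and plays the player's interact animation.
; Four inputs check the answer, Tick fails it when the widget stops running, and dispatchers report readiness and results.
; The widget turns toward BP_CameraActor on interact start; BeginPlay seeds IsVisible from saved interaction 503's completion.
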(event Custom|CE_PlayQTE
  (params (TimerQTE :type Float%20%28double-precision%29))
  (Variables|Default|SetIsPlayable true)
  (CallFunction|FShowWidget)
  (Default|PlayQTE (Variables|Default|GetAs%20WBP%20QTE) TimerQTE (Math|Random|RandomInteger 3))
  (bind _returnvalue (Class|CharacterPlayer|GetBlueprintAnim (Variables|Default|GetPlayerIn)))
  (Class|BPIAnim|PlayInteract(Message) _returnvalue "NewEnumerator2"))

(event Custom|CE_StopInteract
  (bind _returnvalue (Class|CharacterPlayer|GetBlueprintAnim (Variables|Default|GetPlayerIn)))
  (Class|BPIAnim|StopInteract(Message) _returnvalue)
  (Class|PlayerStateMachine|ChangeState (Variables|/Script/CouchGame.CharacterPlayer|GetStateMachine (Variables|Default|GetPlayerIn)) "Idle"))

(event Custom|CE_RotationWidget
  (bind _worldcamera (Variables|Default|GetWorldCamera))
  (bind _widget (Variables|Default|GetWidget))
  (bind _returnvalue (Transformation|GetWorldLocation _widget))
  (bind _rootcomponent (Variables|/Script/Engine.Actor|GetRootComponent _worldcamera))
  (bind _returnvalue_2 (Transformation|GetWorldLocation _rootcomponent))
  (bind _returnvalue_3 (Math|Rotator|FindLookatRotation _returnvalue _returnvalue_2))
  ;[0.15 0.15 0.15 0.5] Rotation Widget
  (Transformation|SetWorldRotation (Variables|Default|GetWidget) (Math|Rotator|MakeRotator (.roll (Transformation|GetWorldRotation (Variables|Default|GetWidget))) (.pitch _returnvalue_3) (.yaw _returnvalue_3)) false false))

(event Custom|CE_Highlight
  (params (bNewVisibility :type Boolean))
  (Rendering|SetVisibility (Variables|Default|GetCylinder) bNewVisibility false))

(event Custom|CE_StopQTE
  (Variables|Default|SetIsPlayable false)
  (CallFunction|FHideWidget)
  (Default|FClickQTE (Variables|Default|GetAs%20WBP%20QTE))
  (bind _returnvalue (Class|CharacterPlayer|GetBlueprintAnim (Variables|Default|GetPlayerIn)))
  (Class|BPIAnim|StopInteract(Message) _returnvalue))

(event EventBeginPlay
  ;[0.15 0.15 0.15 0.5] Begin Play (Recuperation des var)
  (bind _aswbp_qte (Utilities|Casting|CastToWBP_QTE (UserInterface|GetUserWidgetObject (Variables|Default|GetWidget))))
  (Variables|Default|SetAs%20WBP%20QTE _aswbp_qte)
  (bind _returnvalue (Actor|GetActorOfClass "/Game/BP/Camera/BP_CameraActor.BP_CameraActor_C"))
  (Variables|Default|SetWorldCamera _returnvalue)
  (bind _returnvalue_2 (Class|SaveCubeSubsystem|GetInteractionsDatasfromID (Subsystems|GetSaveCubeSubsystem) 503))
  (Variables|Default|SetIsVisible (.iscompleted _returnvalue_2)))

(event EventTick
  (params (DeltaSeconds :type Float%20%28single-precision%29))
  (if (Variables|Default|GetIsVisible)
    ;[0.15 0.15 0.15 0.5] If le QTE est fini
    (bind _isrunning (Default|FGetIsRunning (Variables|Default|GetAs%20WBP%20QTE)))
    (if (not _isrunning)
      ;[0.15 0.15 0.15 0.5] Hide & Reset Var Count
      (CallFunction|FHideWidget)
      (Default|CallEDIsQTEWin false))))

(event EventEndInteract
  (params (Player :type Character%20Player%20Object%20Reference))
  ;[0.15 0.15 0.15 0.5] End Interact
  (Default|CallEDPlayerUnready)
  (CallFunction|CEStopQTE))

(event EventSetCharacterinInteract
  (params (Player :type Character%20Player%20Object%20Reference))
  ;[0.15 0.15 0.15 0.5] Player In
  (Variables|Default|SetPlayerIn Player))

(event EventOnStartInteract
  (params (Player :type Character%20Player%20Object%20Reference) (InputID :type EInputID%20Enum :default "QTE1"))
  ;[0.15 0.15 0.15 0.5] OnStartInteract
  (if (Variables|Default|GetIsPlayable)
    (switch Utilities|FlowControl|Switch|SwitchonEInputID InputID
      (:QTE1
        ;[0.15 0.15 0.15 0.5] Click Up
        (bind _win (Default|FClickQTE (Variables|Default|GetAs%20WBP%20QTE)))
        (CallFunction|FHideWidget)
        (Default|CallEDIsQTEWin _win))
      (:QTE2
        ;[0.15 0.15 0.15 0.5] Click Right
        (bind _win_2 (Default|FClickQTE (Variables|Default|GetAs%20WBP%20QTE) 1))
        (CallFunction|FHideWidget)
        (Default|CallEDIsQTEWin _win_2))
      (:QTE3
        ;[0.15 0.15 0.15 0.5] Click Down
        (bind _win_3 (Default|FClickQTE (Variables|Default|GetAs%20WBP%20QTE) 2))
        (CallFunction|FHideWidget)
        (Default|CallEDIsQTEWin _win_3))
      (:QTE4
        ;[0.15 0.15 0.15 0.5] Click Left
        (bind _win_4 (Default|FClickQTE (Variables|Default|GetAs%20WBP%20QTE) 3))
        (CallFunction|FHideWidget)
        (Default|CallEDIsQTEWin _win_4)))))

(event EventStartInteract
  (params (Player :type Character%20Player%20Object%20Reference))
  ;[0.15 0.15 0.15 0.5] StartInteract
  (Default|CallEDPlayerReady)
  (Variables|Default|SetIsPlayable true)
  (CallFunction|CERotationWidget))

(fn ConstructionScript)

(fn FShowWidget
  (Variables|Default|SetIsVisible true)
  (Rendering|SetVisibility (Variables|Default|GetWidget) true false))

(fn FHideWidget
  (Variables|Default|SetIsVisible false)
  (Rendering|SetVisibility (Variables|Default|GetWidget) false false))

(fn GetCharacterinInteract
  (return (Variables|Default|GetPlayerIn)))

(fn GetInteractWidget
  (return 0))

(fn GetPlayerLockParent
  (return (Variables|Default|GetLockParent)))

(fn GetUnlockTP
  (return (Variables|Default|GetLockParent)))

(fn IsPlayerLocked
  (return (Utilities|IsValid (Variables|Default|GetPlayerIn))))

(fn LockedPlayer
  (return true))
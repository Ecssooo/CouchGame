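; Audio Blueprint that smoothly switches music and ambient sound between six level "faces", starting with face 1 on BeginPlay.
; CE_ChangeSound plays a timeline whose Alpha drives the volume multiplier of both audio components.
; The timeline's Change Sound event track picks the face's music and ambience and plays them through SoundManager.
; GetColor returns black for every face and is not called in this Blueprint.
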(event Custom|CE_ChangeSound
  (params (LevelLoad :type Integer))
  (bind _alpha (Timeline|ChangeSound PlayFromStart)
    (:Update
      (Audio|Components|Audio|SetVolumeMultiplier (Variables|Default|GetMusic) _alpha :!class /Script/Engine.AudioComponent)
      (Audio|Components|Audio|SetVolumeMultiplier (Variables|Default|GetAmbient) _alpha :!class /Script/Engine.AudioComponent))
    (:ChangeSound
      (switch int LevelLoad
        (:1
          (CallFunction|PlayMusic "MUS_face_1")
          (CallFunction|PlayAmbient "AMB_Face1"))
        (:2
          (CallFunction|PlayMusic "MUS_face_2")
          (CallFunction|PlayAmbient "AMB_Face2"))
        (:3
          (CallFunction|PlayMusic "MUS_face_3")
          (CallFunction|PlayAmbient "AMB_Face3"))
        (:4
          (CallFunction|PlayMusic "MUS_face_4")
          (CallFunction|PlayAmbient "AMB_Face4"))
        (:5
          (CallFunction|PlayMusic "MUS_face_5")
          (CallFunction|PlayAmbient "AMB_Face5"))
        (:6
          (CallFunction|PlayMusic "MUS_face_6")
          (CallFunction|PlayAmbient "AMB_Face6"))))))

(event EventBeginPlay
  (CallFunction|CEChangeSound 1))

(fn ConstructionScript)

(fn GetColor
  (params (LevelLoad :type Integer))
  (switch int LevelLoad
    (:1
      (return ""))
    (:2
      (return ""))
    (:3
      (return ""))
    (:4
      (return ""))
    (:5
      (return ""))
    (:6
      (return ""))))

(fn PlayMusic
  (params (SoundName :type Name))
  (Class|SoundManager|PlaySound (Subsystems|GetSoundManager) SoundName (Variables|Default|GetMusic)))

(fn PlayAmbient
  (params (SoundName :type Name))
  (Class|SoundManager|PlaySound (Subsystems|GetSoundManager) SoundName (Variables|Default|GetAmbient)))
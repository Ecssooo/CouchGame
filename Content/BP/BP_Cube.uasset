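; BP_Cube is a cube actor that animates quarter-turn rotations in four directions for a TP manager.
; Custom events play two timelines forward or in reverse, lerping roll for right/left and pitch for up/down.
; On finish, rotation snaps back to zero and the manager's load function runs by timeline direction.
; Up and down call FLoadUp and FLoadDown, while right and left both call FLoadRight.
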(event Custom|CE_RotateLeft
  (bind (_direction _newtrack_0) (Timeline|Timeline ReverseFromEnd)
    (:Update
      (Transformation|SetActorRotation (Math|Rotator|MakeRotator (Math|Float|Lerp 0.0 9e+01 _newtrack_0) (Math|Float|Lerp 0.0 0.0 _newtrack_0) (Math|Float|Lerp 0.0 0.0 _newtrack_0))))
    (:Finished
      (Transformation|SetActorRotation "0, 0, 0")
      (switch Utilities|FlowControl|Switch|SwitchonETimelineDirection _direction
        (:Forward
          (Default|FLoadRight (Variables|Default|GetAs%20BP%20TPManager)))
        (:Backward
          (Default|FLoadRight (Variables|Default|GetAs%20BP%20TPManager)))))))

(event Custom|CE_RotateRight
  (bind (_direction _newtrack_0) (Timeline|Timeline PlayFromStart)
    (:Update
      (Transformation|SetActorRotation (Math|Rotator|MakeRotator (Math|Float|Lerp 0.0 9e+01 _newtrack_0) (Math|Float|Lerp 0.0 0.0 _newtrack_0) (Math|Float|Lerp 0.0 0.0 _newtrack_0))))
    (:Finished
      (Transformation|SetActorRotation "0, 0, 0")
      (switch Utilities|FlowControl|Switch|SwitchonETimelineDirection _direction
        (:Forward
          (Default|FLoadRight (Variables|Default|GetAs%20BP%20TPManager)))
        (:Backward
          (Default|FLoadRight (Variables|Default|GetAs%20BP%20TPManager)))))))

(event Custom|CE_RotateDown
  (bind (_direction _newtrack_0) (Timeline|Timeline_0 ReverseFromEnd)
    (:Update
      (Transformation|SetActorRotation (Math|Rotator|MakeRotator (Math|Float|Lerp 0.0 0.0 _newtrack_0) (Math|Float|Lerp 0.0 -9e+01 _newtrack_0) (Math|Float|Lerp 0.0 0.0 _newtrack_0))))
    (:Finished
      (Transformation|SetActorRotation "0, 0, 0")
      (switch Utilities|FlowControl|Switch|SwitchonETimelineDirection _direction
        (:Forward
          (Default|FLoadUp (Variables|Default|GetAs%20BP%20TPManager)))
        (:Backward
          (Default|FLoadDown (Variables|Default|GetAs%20BP%20TPManager)))))))

(event Custom|CE_RotateUp
  (bind (_direction _newtrack_0) (Timeline|Timeline_0 PlayFromStart)
    (:Update
      (Transformation|SetActorRotation (Math|Rotator|MakeRotator (Math|Float|Lerp 0.0 0.0 _newtrack_0) (Math|Float|Lerp 0.0 -9e+01 _newtrack_0) (Math|Float|Lerp 0.0 0.0 _newtrack_0))))
    (:Finished
      (Transformation|SetActorRotation "0, 0, 0")
      (switch Utilities|FlowControl|Switch|SwitchonETimelineDirection _direction
        (:Forward
          (Default|FLoadUp (Variables|Default|GetAs%20BP%20TPManager)))
        (:Backward
          (Default|FLoadDown (Variables|Default|GetAs%20BP%20TPManager)))))))

(event Collision|EventActorBeginOverlap
  (params (OtherActor :type Actor%20Object%20Reference)))

(event EventTick
  (params (DeltaSeconds :type Float%20%28single-precision%29)))

(event EventBeginPlay)

(fn ConstructionScript)
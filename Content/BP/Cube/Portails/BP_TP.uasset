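; Cube portal that, while enabled, counts overlapping players and starts the level transition once two stand inside.
; It plays a sound per arrival, then undiscovers all sublevels, teleports characters out and blends the camera, separated by timeline-setting delays.
; It then rotates BP_Cube from Direction to DirectionArrive and passes the neighbor level's name suffix, as an integer, to skybox color and audio changers.
; External events toggle its plane and highlight effect.
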(event OnComponentBeginOverlap(Trigger)
  (params (OverlappedComponent :type Primitive%20Component%20Object%20Reference) (OtherActor :type Actor%20Object%20Reference) (OtherComp :type Primitive%20Component%20Object%20Reference) (OtherBodyIndex :type Integer) (bFromSweep :type Boolean) (SweepResult :type Hit%20Result%20Structure%20%28by%20ref%29))
  (bind (_swingduration _slideduration _sublevelupduration _subleveldownduration _skyboxfadeduration _blendcamerainduration _blendcameraoutduration _waitforblendout _waitforrotationstart) (Utilities|GetClassDefaults "/Script/CouchGame.TimelineSettings"))
  (if (Utilities|DoesObjectImplementInterface OtherActor "/Game/BP/BPI/BPI_Player.BPI_Player_C")
    (if (Variables|Default|GetIs%20Enable)
      (Math|Integer|IncrementInt (Variables|Default|GetNbPlayerHir)
        (:%20%20
          (if (== (Variables|Default|GetNbPlayerHir) 1)
            (Class|SoundManager|PlaySound (Subsystems|GetSoundManager) "SFX_Portal_Player_1" (Variables|Default|GetAudio)))
          (if (== (Variables|Default|GetNbPlayerHir) 2)
            (Class|SoundManager|PlaySound (Subsystems|GetSoundManager) "SFX_Portal_Player_2" (Variables|Default|GetAudio))
            (bind _returnvalue (Actor|GetActorOfClass "/Game/BP/Systems/BP_SaveSubLevelManager.BP_SaveSubLevelManager_C"))
            (Class|SaveSubLevelManager|UndiscoverAllSubLevel _returnvalue)
            (Class|CubeGameMode|TeleportCharacterOut (Variables|Default|GetAs%20Cube%20Game%20Mode))
            (Utilities|FlowControl|Delay _waitforblendout)
            (bind _returnvalue_2 (Actor|GetActorOfClass "/Game/BP/Camera/BP_BlendCameraForTransition.BP_BlendCameraForTransition_C"))
            (bind _output_get (Variables|Default|SetBlendCamera _returnvalue_2))
            (Default|CEBlendOut _output_get)
            (Utilities|FlowControl|Delay _waitforrotationstart)
            (CallFunction|FTryTP)))))))

(event OnComponentEndOverlap(Trigger)
  (params (OverlappedComponent :type Primitive%20Component%20Object%20Reference) (OtherActor :type Actor%20Object%20Reference) (OtherComp :type Primitive%20Component%20Object%20Reference) (OtherBodyIndex :type Integer))
  (if (Utilities|DoesObjectImplementInterface OtherActor "/Game/BP/BPI/BPI_Player.BPI_Player_C")
    (if (Variables|Default|GetIs%20Enable)
      (Math|Integer|DecrementInt (Variables|Default|GetNbPlayerHir)))))

(event Custom|CE_EnableTP
  (params (IsEnable :type Boolean))
  (bind _output_get (Variables|Default|SetIs%20Enable IsEnable))
  (Rendering|SetVisibility (Variables|Default|GetPlane) _output_get false))

(event EventBeginPlay
  (Utilities|FlowControl|Sequence
    (:then_0
      (bind _returnvalue (Actor|GetActorOfClass "/Game/BP/Cube/BP_Cube.BP_Cube_C"))
      (Variables|Default|SetBP_Cube _returnvalue))
    (:then_1
      (bind _ascube_game_mode (Utilities|Casting|CastToCubeGameMode (Game|GetGameMode)))
      (Variables|Default|SetAs%20Cube%20Game%20Mode _ascube_game_mode))))

(event EventHighlightTeleporter
  (params (IsHighlight :type Boolean))
  (Rendering|SetVisibility (Variables|Default|GetNS_Portal_Bleue) IsHighlight false))

(fn ConstructionScript)

(fn FTryTP
  (switch Utilities|FlowControl|Switch|SwitchonELevelDir (Variables|Default|GetDirection)
    (:Up
      (Class|CubeController|StartRotationQuat (Variables|Default|GetBP_Cube) (Variables|Default|GetDirection) (Variables|Default|GetDirectionArrive)))
    (:Down
      (Class|CubeController|StartRotationQuat (Variables|Default|GetBP_Cube) (Variables|Default|GetDirection) (Variables|Default|GetDirectionArrive)))
    (:Left
      (Class|CubeController|StartRotationQuat (Variables|Default|GetBP_Cube) (Variables|Default|GetDirection) (Variables|Default|GetDirectionArrive)))
    (:Right
      (Class|CubeController|StartRotationQuat (Variables|Default|GetBP_Cube) (Variables|Default|GetDirection) (Variables|Default|GetDirectionArrive))))
  (bind _returnvalue (Actor|GetActorOfClass "/Script/CouchGame.LevelStreamerActor"))
  (bind _returnvalue_2 (Actor|GetActorOfClass "/Game/Assets3D/skybox/Dynamic_Skybox/BP_SkyboxChangeColor.BP_SkyboxChangeColor_C"))
  (Default|CEChangeColor _returnvalue_2 (Math|Conversions|ToInteger(Byte) (.RightS (Utilities|String|Split (Utilities|String|ToString(Name) (Class|LevelStreamerActor|GetNeighborLevel _returnvalue (Variables|/Script/CouchGame.LevelStreamerActor|GetCurrentLevel _returnvalue) (Variables|Default|GetDirection))) "_"))))
  (bind _returnvalue_3 (Actor|GetActorOfClass "/Game/BP/SoundSystem/BP_AudioSmoothChange.BP_AudioSmoothChange_C"))
  (Default|CEChangeSound _returnvalue_3 (Math|Conversions|ToInteger(Byte) (.RightS (Utilities|String|Split (Utilities|String|ToString(Name) (Class|LevelStreamerActor|GetNeighborLevel _returnvalue (Variables|/Script/CouchGame.LevelStreamerActor|GetCurrentLevel _returnvalue) (Variables|Default|GetDirection))) "_")))))
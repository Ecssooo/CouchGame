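; Cube actor that turns in 90-degree steps through right, left, up and down events.
; Two timelines drive roll and pitch, playing forward or reversed, with Finished updating the wrapped 0-360 angle and snapping to it.
; The animated axis lerps between zero and 90 degrees in magnitude, independent of its stored angle.
; Delayed CubeGameMode calls to spawn the character in a streamed level with DirectionTP are disconnected and never run.
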(event Custom|CE_RotateLeft
  (params (DirectionTP :type ELevelDir%20Enum :default "Up"))
  ;[0 0.1011 0.2083 0.5] Rotate Horizontale
  (Variables|Default|SetDirectionTP DirectionTP)
  (bind (_direction _newtrack_0) (Timeline|Timeline ReverseFromEnd)
    (:Update
      ;;[0.15 0.15 0.15 0.5] In Boucle
      (Transformation|SetActorRelativeRotation (Math|Rotator|MakeRotator (Math|Float|Lerp 0.0 -9e+01 _newtrack_0) (Variables|Default|GetCurrentPitch) 0.0)))
    (:Finished
      (switch Utilities|FlowControl|Switch|SwitchonETimelineDirection _direction
        (:Forward
          (bind _newrotation (CallFunction|ClampRotation (- (Variables|Default|GetCurrentRoll) 9e+01)))
          (bind _output_get (Variables|Default|SetCurrentRoll _newrotation))
          ;;[0.15 0.15 0.15 0.5] End Boucle
          (Transformation|SetActorRelativeRotation (Math|Rotator|MakeRotator _output_get (Variables|Default|GetCurrentPitch) 0.0)))
        (:Backward
          (bind _newrotation_2 (CallFunction|ClampRotation (+ (Variables|Default|GetCurrentRoll) 9e+01)))
          (bind _output_get_2 (Variables|Default|SetCurrentRoll _newrotation_2))
          (Transformation|SetActorRelativeRotation (Math|Rotator|MakeRotator _output_get_2 (Variables|Default|GetCurrentPitch) 0.0)))))))

(event Custom|CE_RotateRight
  (params (DirectionTP :type ELevelDir%20Enum :default "Up"))
  ;[0 0.1011 0.2083 0.5] Rotate Horizontale
  (Variables|Default|SetDirectionTP DirectionTP)
  (bind (_direction _newtrack_0) (Timeline|Timeline PlayFromStart)
    (:Update
      ;;[0.15 0.15 0.15 0.5] In Boucle
      (Transformation|SetActorRelativeRotation (Math|Rotator|MakeRotator (Math|Float|Lerp 0.0 -9e+01 _newtrack_0) (Variables|Default|GetCurrentPitch) 0.0)))
    (:Finished
      (switch Utilities|FlowControl|Switch|SwitchonETimelineDirection _direction
        (:Forward
          (bind _newrotation (CallFunction|ClampRotation (- (Variables|Default|GetCurrentRoll) 9e+01)))
          (bind _output_get (Variables|Default|SetCurrentRoll _newrotation))
          ;;[0.15 0.15 0.15 0.5] End Boucle
          (Transformation|SetActorRelativeRotation (Math|Rotator|MakeRotator _output_get (Variables|Default|GetCurrentPitch) 0.0)))
        (:Backward
          (bind _newrotation_2 (CallFunction|ClampRotation (+ (Variables|Default|GetCurrentRoll) 9e+01)))
          (bind _output_get_2 (Variables|Default|SetCurrentRoll _newrotation_2))
          (Transformation|SetActorRelativeRotation (Math|Rotator|MakeRotator _output_get_2 (Variables|Default|GetCurrentPitch) 0.0)))))))

(event Custom|CE_RotateDown
  (params (DirectionTP :type ELevelDir%20Enum :default "Up"))
  ;[0.002553 0.0278 0.15 0.5] Rotate Verticale
  (Variables|Default|SetDirectionTP DirectionTP)
  (bind (_direction _newtrack_0) (Timeline|Timeline_0 ReverseFromEnd)
    (:Update
      ;;[0.15 0.15 0.15 0.5] In Boucle
      (Transformation|SetActorRelativeRotation (Math|Rotator|MakeRotator (Variables|Default|GetCurrentRoll) (Math|Float|Lerp 0.0 9e+01 _newtrack_0) 0.0)))
    (:Finished
      (switch Utilities|FlowControl|Switch|SwitchonETimelineDirection _direction
        (:Forward
          (bind _newrotation (CallFunction|ClampRotation (+ 9e+01 (Variables|Default|GetCurrentPitch))))
          (bind _output_get (Variables|Default|SetCurrentPitch _newrotation))
          ;;[0.15 0.15 0.15 0.5] End Boucle
          (Transformation|SetActorRelativeRotation (Math|Rotator|MakeRotator (Variables|Default|GetCurrentRoll) _output_get 0.0)))
        (:Backward
          (bind _newrotation_2 (CallFunction|ClampRotation (- (Variables|Default|GetCurrentPitch) 9e+01)))
          (bind _output_get_2 (Variables|Default|SetCurrentPitch _newrotation_2))
          (Transformation|SetActorRelativeRotation (Math|Rotator|MakeRotator (Variables|Default|GetCurrentRoll) _output_get_2 0.0)))))))

(event Custom|CE_RotateUp
  (params (DirectionTP :type ELevelDir%20Enum :default "Up"))
  ;[0.002553 0.0278 0.15 0.5] Rotate Verticale
  (Variables|Default|SetDirectionTP DirectionTP)
  (bind (_direction _newtrack_0) (Timeline|Timeline_0 PlayFromStart)
    (:Update
      ;;[0.15 0.15 0.15 0.5] In Boucle
      (Transformation|SetActorRelativeRotation (Math|Rotator|MakeRotator (Variables|Default|GetCurrentRoll) (Math|Float|Lerp 0.0 9e+01 _newtrack_0) 0.0)))
    (:Finished
      (switch Utilities|FlowControl|Switch|SwitchonETimelineDirection _direction
        (:Forward
          (bind _newrotation (CallFunction|ClampRotation (+ 9e+01 (Variables|Default|GetCurrentPitch))))
          (bind _output_get (Variables|Default|SetCurrentPitch _newrotation))
          ;;[0.15 0.15 0.15 0.5] End Boucle
          (Transformation|SetActorRelativeRotation (Math|Rotator|MakeRotator (Variables|Default|GetCurrentRoll) _output_get 0.0)))
        (:Backward
          (bind _newrotation_2 (CallFunction|ClampRotation (- (Variables|Default|GetCurrentPitch) 9e+01)))
          (bind _output_get_2 (Variables|Default|SetCurrentPitch _newrotation_2))
          (Transformation|SetActorRelativeRotation (Math|Rotator|MakeRotator (Variables|Default|GetCurrentRoll) _output_get_2 0.0)))))))

(event EventBeginPlay
  (bind _ascube_game_mode (Utilities|Casting|CastToCubeGameMode (Game|GetGameMode)))
  (Variables|Default|SetAs%20Cube%20Game%20Mode _ascube_game_mode)
  (Variables|Default|SetCurrentRoll 0.0)
  (Variables|Default|SetCurrentPitch 0.0))

(fn ConstructionScript)

(fn ClampRotation
  (params (Roation :type Float%20%28double-precision%29))
  (if (< Roation 0.0)
    (return (+ Roation 3.6e+02))
    (elif (>= Roation 3.6e+02)
      (return (- Roation 3.6e+02))
      (else
        (return Roation)))))
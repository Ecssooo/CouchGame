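; BP_TP is a toggleable teleporter that sends players out and rotates the cube once two players stand in its trigger.
; While enabled, it counts overlapping BPI_Player actors as they enter and leave, testing the count on each entry.
; At exactly two, it calls TeleportCharacterOut on CubeGameMode and starts BP_Cube's quaternion rotation from Direction to DirectionArrive.
; Separate events toggle its enabled state with trigger visibility, and its custom-depth highlight.
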(event OnComponentBeginOverlap(Trigger)
  (params (OverlappedComponent :type Primitive%20Component%20Object%20Reference) (OtherActor :type Actor%20Object%20Reference) (OtherComp :type Primitive%20Component%20Object%20Reference) (OtherBodyIndex :type Integer) (bFromSweep :type Boolean) (SweepResult :type Hit%20Result%20Structure%20%28by%20ref%29))
  (if (Utilities|DoesObjectImplementInterface OtherActor "/Game/BP/BPI/BPI_Player.BPI_Player_C")
    (if (Variables|Default|GetIs%20Enable)
      (Math|Integer|IncrementInt (Variables|Default|GetNbPlayerHir)
        (:%20%20
          (CallFunction|FTryTP))))))

(event OnComponentEndOverlap(Trigger)
  (params (OverlappedComponent :type Primitive%20Component%20Object%20Reference) (OtherActor :type Actor%20Object%20Reference) (OtherComp :type Primitive%20Component%20Object%20Reference) (OtherBodyIndex :type Integer))
  (if (Utilities|DoesObjectImplementInterface OtherActor "/Game/BP/BPI/BPI_Player.BPI_Player_C")
    (if (Variables|Default|GetIs%20Enable)
      (Math|Integer|DecrementInt (Variables|Default|GetNbPlayerHir)))))

(event Custom|CE_EnableTP
  (params (IsEnable :type Boolean))
  (bind _output_get (Variables|Default|SetIs%20Enable IsEnable))
  (Rendering|SetVisibility (Variables|Default|GetTrigger) _output_get false))

(event EventBeginPlay
  (Utilities|FlowControl|Sequence
    (:then_0
      (bind _returnvalue (Actor|GetActorOfClass "/Game/BP/Cube/BP_Cube.BP_Cube_C"))
      (Variables|Default|SetBP_Cube _returnvalue))
    (:then_1
      (bind _ascube_game_mode (Utilities|Casting|CastToCubeGameMode (Game|GetGameMode)))
      (Variables|Default|SetAs%20Cube%20Game%20Mode _ascube_game_mode))))

(event EventHighlightTeleporter
  (params (IsHighlight :type Boolean))
  (Rendering|SetRenderCustomDepth (Variables|Default|GetTrigger) IsHighlight))

(fn ConstructionScript)

(fn FTryTP
  (if (== (Variables|Default|GetNbPlayerHir) 2)
    (Class|CubeGameMode|TeleportCharacterOut (Variables|Default|GetAs%20Cube%20Game%20Mode))
    (switch Utilities|FlowControl|Switch|SwitchonELevelDir (Variables|Default|GetDirection)
      (:Up
        (Class|CubeController|StartRotationQuat (Variables|Default|GetBP_Cube) (Variables|Default|GetDirection) (Variables|Default|GetDirectionArrive)))
      (:Down
        (Class|CubeController|StartRotationQuat (Variables|Default|GetBP_Cube) (Variables|Default|GetDirection) (Variables|Default|GetDirectionArrive)))
      (:Left
        (Class|CubeController|StartRotationQuat (Variables|Default|GetBP_Cube) (Variables|Default|GetDirection) (Variables|Default|GetDirectionArrive)))
      (:Right
        (Class|CubeController|StartRotationQuat (Variables|Default|GetBP_Cube) (Variables|Default|GetDirection) (Variables|Default|GetDirectionArrive))))))
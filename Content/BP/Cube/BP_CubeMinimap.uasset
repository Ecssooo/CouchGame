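; BP_CubeMinimap is an actor that represents a cube minimap with six cube components, one per face.
; FEnableFace takes a face number and a flag, then switches on the number to set visibility of the matching Cube1 to Cube6 component and its children.
; On BeginPlay it turns face 4 on; Tick and overlap events are unused.
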(event EventBeginPlay
  (CallFunction|FEnableFace 4 true))

(event Collision|EventActorBeginOverlap
  (params (OtherActor :type Actor%20Object%20Reference)))

(event EventTick
  (params (DeltaSeconds :type Float%20%28single-precision%29)))

(fn ConstructionScript)

(fn FEnableFace
  (params (NumFace :type Integer) (Enabled :type Boolean))
  (Variables|Default|SetEnabled Enabled)
  (switch int NumFace
    (:1
      (Rendering|SetVisibility (Variables|Default|GetCube_1) (Variables|Default|GetEnabled) true))
    (:2
      (Rendering|SetVisibility (Variables|Default|GetCube_2) (Variables|Default|GetEnabled) true))
    (:3
      (Rendering|SetVisibility (Variables|Default|GetCube_3) (Variables|Default|GetEnabled) true))
    (:4
      (Rendering|SetVisibility (Variables|Default|GetCube_4) (Variables|Default|GetEnabled) true))
    (:5
      (Rendering|SetVisibility (Variables|Default|GetCube_5) (Variables|Default|GetEnabled) true))
    (:6
      (Rendering|SetVisibility (Variables|Default|GetCube_6) (Variables|Default|GetEnabled) true))))
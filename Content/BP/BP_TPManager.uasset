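; BP_TPManager is a Blueprint wrapper around a TPManager object that handles directional level loading and unloading.
; Its functions forward up, down, left and right load requests and an unload request to TPManager, and a getter exposes that object.
; The event graph holds no active logic, only empty events and an unconnected test call.
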(event Collision|EventActorBeginOverlap
  (params (OtherActor :type Actor%20Object%20Reference)))

(event EventTick
  (params (DeltaSeconds :type Float%20%28single-precision%29)))

(event EventBeginPlay)

(fn ConstructionScript)

(fn FGetTPManager
  (return (Variables|Default|GetTPManager)))

(fn FLoadUp
  (Class|TPManager|OnUpPressed (Variables|Default|GetTPManager)))

(fn FUnloadLevel
  (Class|TPManager|UnloadLevel (Variables|Default|GetTPManager)))

(fn FLoadDown
  (Class|TPManager|OnDownPressed (Variables|Default|GetTPManager)))

(fn FLoadLeft
  (Class|TPManager|OnLeftPressed (Variables|Default|GetTPManager)))

(fn FLoadRight
  (Class|TPManager|OnRightPressed (Variables|Default|GetTPManager)))
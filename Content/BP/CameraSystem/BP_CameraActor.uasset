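; Two-player camera actor that glides between its start position and a target point as the players advance along the X axis.
; After a short delay, BeginPlay caches both players, the start location and the CameraTargetPos component's world location.
; Each Tick, forward and back flags drive a VInterpTo move.
; It advances when both players pass the target's X plus a margin, otherwise it returns.
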(event EventBeginPlay
  (Utilities|FlowControl|Delay 1.0)
  (Variables|Default|SetPlayer_1 (Game|GetPlayerCharacter 0))
  (Variables|Default|SetPlayer_2 (Game|GetPlayerCharacter 1))
  (Variables|Default|SetCamStartPos (Transformation|GetActorLocation))
  (Variables|Default|SetTargetPos (Transformation|GetWorldLocation (Variables|Default|GetCameraTargetPos)))
  (Components|Activation|SetAutoActivate (Variables|Default|GetCameraTargetPos) false))

(event EventTick
  (params (DeltaSeconds :type Float%20%28single-precision%29))
  (bind _targetpos (Variables|Default|GetTargetPos))
  (Variables|Default|SetDelta%20Seconds DeltaSeconds)
  (Utilities|IsValid (Variables|Default|GetPlayer_1)
    (:Is%20Valid
      (Utilities|IsValid (Variables|Default|GetPlayer_2)
        (:Is%20Valid
          (Utilities|FlowControl|Sequence
            (:then_0
              (if (Variables|Default|GetIsForward)
                (bind _returnvalue (Math|Interpolation|VInterpTo (Transformation|GetActorLocation) (Variables|Default|GetTargetPos) (Variables|Default|GetDelta%20Seconds) (Variables|Default|GetSpeedMovementCamera)))
                (Transformation|SetActorLocation _returnvalue false false)
                (Development|PrintString "CAM Avance" true true "(R=0.101540,G=0.000000,B=1.000000,A=1.000000)")))
            (:then_1
              (if (Variables|Default|GetIsBack)
                (bind _returnvalue_2 (Math|Interpolation|VInterpTo (Transformation|GetActorLocation) (Variables|Default|GetCamStartPos) (Variables|Default|GetDelta%20Seconds) (Variables|Default|GetSpeedMovementCamera)))
                (Transformation|SetActorLocation _returnvalue_2 false false)
                (Development|PrintString "CAM Recule" true true "(R=0.115642,G=0.000000,B=1.000000,A=1.000000)")))
            (:then_2
              (if (and (>= (.x (Transformation|GetActorLocation (Variables|Default|GetPlayer_2))) (+ (.x _targetpos) (Variables|Default|GetMargeCamera))) (>= (.x (Transformation|GetActorLocation (Variables|Default|GetPlayer_1))) (+ (.x _targetpos) (Variables|Default|GetMargeCamera))))
                (if (not (Variables|Default|GetIsForward))
                  (Development|PrintString "SUPERIEUR" true true "(R=0.000000,G=1.000000,B=0.065019,A=1.000000)" 4.0)
                  (Variables|Default|SetIsForward true)
                  (Variables|Default|SetIsBack false))
                (elif (not (Variables|Default|GetIsBack))
                  (Development|PrintString "Inferieur")
                  (Variables|Default|SetIsForward false)
                  (Variables|Default|SetIsBack true))))))))))

(fn ConstructionScript)
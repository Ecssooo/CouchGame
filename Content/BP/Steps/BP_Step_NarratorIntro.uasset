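; BP_Step_NarratorIntro is a step that plays the narrator introduction, then advances the StepManager.
; On step start it creates a WBP_Naration widget, shows its text, and plays the VOC_Narrator_Start voice line through the SoundManager after a delay.
; Chained delays then hide the text, call NextStep, and fade out the background before removing the widget, so the next step begins while the overlay is still closing.
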(event EventOnStartStep
  (bind _returnvalue (UserInterface|CreateWidget "/Game/UI/WBP_Naration.WBP_Naration_C"))
  (bind _output_get (Variables|Default|SetWBP%20Naration _returnvalue))
  (UserInterface|Viewport|AddtoViewport _output_get 0)
  (Default|CESetText (Variables|Default|GetWBP%20Naration) (Variables|Default|GetText))
  (Default|CEShowText (Variables|Default|GetWBP%20Naration))
  (Utilities|FlowControl|Delay 2.0)
  (Class|SoundManager|PlaySound (Subsystems|GetSoundManager) "VOC_Narrator_Start" (Variables|Default|GetAudio))
  (Utilities|FlowControl|Delay 3.0)
  (Default|CEHideText (Variables|Default|GetWBP%20Naration))
  (Utilities|FlowControl|Delay 2.0)
  (Class|StepManager|NextStep (Variables|Default|GetStepManager))
  (Default|CEHideBG (Variables|Default|GetWBP%20Naration))
  (Utilities|FlowControl|Delay 2.0)
  (Widget|RemovefromParent (Variables|Default|GetWBP%20Naration)))

(fn ConstructionScript)
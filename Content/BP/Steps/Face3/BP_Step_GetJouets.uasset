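; Tutorial-style step for cube face 3 that waits until four toy objects (IDs 301-304) are placed in their sockets.
; On start it highlights the objects and the face's teleporters through SaveCubeSubsystem.
; Tick polls each object's state, clears its highlight once socketed, then calls StepManager.NextStep when all four are in.
; Ending the step clears all highlights, and auto-step forces the objects into their sockets.
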(event EventOnStartStep
  (Variables|Default|SetIsReady true)
  (Class|SaveCubeSubsystem|SetObjectHighlight (Subsystems|GetSaveCubeSubsystem) 301 true)
  (Class|SaveCubeSubsystem|SetObjectHighlight (Subsystems|GetSaveCubeSubsystem) 302 true)
  (Class|SaveCubeSubsystem|SetObjectHighlight (Subsystems|GetSaveCubeSubsystem) 303 true)
  (Class|SaveCubeSubsystem|SetObjectHighlight (Subsystems|GetSaveCubeSubsystem) 304 true)
  (Class|SaveCubeSubsystem|SetTeleporterHighlightforFace (Subsystems|GetSaveCubeSubsystem) 3))

(event EventTick
  (params (DeltaSeconds :type Float%20%28single-precision%29))
  (if (Variables|Default|GetIsReady)
    (bind _returnvalue (Class|SaveCubeSubsystem|GetGrabObjectfromID (Subsystems|GetSaveCubeSubsystem) 304))
    (bind _returnvalue_2 (Class|SaveCubeSubsystem|GetGrabObjectfromID (Subsystems|GetSaveCubeSubsystem) 303))
    (bind _returnvalue_3 (Class|SaveCubeSubsystem|GetGrabObjectfromID (Subsystems|GetSaveCubeSubsystem) 301))
    (bind _returnvalue_4 (Class|SaveCubeSubsystem|GetGrabObjectfromID (Subsystems|GetSaveCubeSubsystem) 302))
    (Utilities|FlowControl|Sequence
      (:then_0
        (if (not (Variables|Default|Get302IsInSocket))
          (if (Utilities|Enum|Equal(Enum) (.objectstate _returnvalue_4) "InSocket")
            (Variables|Default|Set302IsInSocket true)
            (Class|SaveCubeSubsystem|SetObjectHighlight (Subsystems|GetSaveCubeSubsystem) 302 false))))
      (:then_1
        (if (not (Variables|Default|Get301IsInSocket))
          (if (Utilities|Enum|Equal(Enum) (.objectstate _returnvalue_3) "InSocket")
            (Variables|Default|Set301IsInSocket true)
            (Class|SaveCubeSubsystem|SetObjectHighlight (Subsystems|GetSaveCubeSubsystem) 301 false))))
      (:then_2
        (if (not (Variables|Default|Get303IsInSocket))
          (if (Utilities|Enum|Equal(Enum) (.objectstate _returnvalue_2) "InSocket")
            (Variables|Default|Set303IsInSocket true)
            (Class|SaveCubeSubsystem|SetObjectHighlight (Subsystems|GetSaveCubeSubsystem) 303 false))))
      (:then_3
        (if (not (Variables|Default|Get304IsInSocket))
          (if (Utilities|Enum|Equal(Enum) (.objectstate _returnvalue) "InSocket")
            (Variables|Default|Set304IsInSocket true)
            (Class|SaveCubeSubsystem|SetObjectHighlight (Subsystems|GetSaveCubeSubsystem) 304 false))))
      (:then_4
        (if (Math|Boolean|ANDBoolean (Variables|Default|Get303IsInSocket) (Variables|Default|Get301IsInSocket) (Variables|Default|Get302IsInSocket) (Variables|Default|Get304IsInSocket))
          (Variables|Default|SetIsReady false)
          (Class|StepManager|NextStep (Variables|Default|GetStepManager)))))))

(event EventOnEndStep
  (Class|SaveCubeSubsystem|SetObjectHighlight (Subsystems|GetSaveCubeSubsystem) 301 false)
  (Class|SaveCubeSubsystem|SetObjectHighlight (Subsystems|GetSaveCubeSubsystem) 302 false)
  (Class|SaveCubeSubsystem|SetObjectHighlight (Subsystems|GetSaveCubeSubsystem) 303 false)
  (Class|SaveCubeSubsystem|SetObjectHighlight (Subsystems|GetSaveCubeSubsystem) 304 false)
  (Class|SaveCubeSubsystem|ResetAllTeleporterHighlight (Subsystems|GetSaveCubeSubsystem)))

(event EventOnAutoStep
  (Variables|Default|SetIsReady false)
  (Class|SaveCubeSubsystem|SetObjectState (Subsystems|GetSaveCubeSubsystem) 301 "InSocket" 301)
  (Class|SaveCubeSubsystem|SetObjectState (Subsystems|GetSaveCubeSubsystem) 302 "InSocket" 302)
  (Class|SaveCubeSubsystem|SetObjectState (Subsystems|GetSaveCubeSubsystem) 303 "InSocket" 303)
  (Class|SaveCubeSubsystem|SetObjectState (Subsystems|GetSaveCubeSubsystem) 304 "InSocket" 304))

(fn ConstructionScript)
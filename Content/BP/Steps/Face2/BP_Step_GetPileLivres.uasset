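; Tutorial-style step Blueprint for Face 2 that waits for the book pile (object 203) to reach its socketed state.
; On start it highlights the object and Face 1's teleporters through SaveCubeSubsystem.
; Tick polls the object's state, clears its highlight, then calls StepManager.NextStep a tick later.
; Step end re-enables the object highlight and resets teleporters, while auto-step forces the object into its socket.
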(event EventOnStartStep
  (Variables|Default|SetIsReady true)
  (Class|SaveCubeSubsystem|SetObjectHighlight (Subsystems|GetSaveCubeSubsystem) 203 true)
  (Class|SaveCubeSubsystem|SetTeleporterHighlightforFace (Subsystems|GetSaveCubeSubsystem) 1))

(event EventTick
  (params (DeltaSeconds :type Float%20%28single-precision%29))
  (if (Variables|Default|GetIsReady)
    (bind _returnvalue (Class|SaveCubeSubsystem|GetGrabObjectfromID (Subsystems|GetSaveCubeSubsystem) 203))
    (if (Variables|Default|Get203IsInSocket)
      (Variables|Default|SetIsReady false)
      (Class|StepManager|NextStep (Variables|Default|GetStepManager))
      (elif (== (.objectstate _returnvalue) 0)
        (Variables|Default|Set203IsInSocket true)
        (Class|SaveCubeSubsystem|SetObjectHighlight (Subsystems|GetSaveCubeSubsystem) 203 false)))))

(event EventOnEndStep
  (Class|SaveCubeSubsystem|SetObjectHighlight (Subsystems|GetSaveCubeSubsystem) 203 true)
  (Class|SaveCubeSubsystem|ResetAllTeleporterHighlight (Subsystems|GetSaveCubeSubsystem)))

(event EventOnAutoStep
  (Variables|Default|SetIsReady false)
  (Class|SaveCubeSubsystem|SetObjectState (Subsystems|GetSaveCubeSubsystem) 203 "InSocket" 203))

(fn ConstructionScript)
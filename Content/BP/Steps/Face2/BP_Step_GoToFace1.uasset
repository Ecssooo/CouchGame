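; Step in the Face 2 sequence that waits for the player to reach Face 1.
; On start it highlights the Face 1 teleporter through the SaveCube subsystem and refreshes all teleporter states through BP_SaveSubLevelManager.
; Tick polls the LevelStreamerActor's current level and advances the StepManager once it is Face_1.
; Ending the step resets the highlights, while auto-step only stops the polling.
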(event EventOnStartStep
  (bind _returnvalue (Actor|GetActorOfClass "/Script/CouchGame.LevelStreamerActor"))
  (Variables|Default|SetLevelStreamerActor _returnvalue)
  (Variables|Default|SetIsReady true)
  (Class|SaveCubeSubsystem|SetTeleporterHighlightforFace (Subsystems|GetSaveCubeSubsystem) 1)
  (bind _returnvalue_2 (Actor|GetActorOfClass "/Game/BP/Systems/BP_SaveSubLevelManager.BP_SaveSubLevelManager_C"))
  (Class|SaveSubLevelManager|UpdateAllTeleporterState _returnvalue_2))

(event EventOnEndStep
  (Class|SaveCubeSubsystem|ResetAllTeleporterHighlight (Subsystems|GetSaveCubeSubsystem)))

(event EventTick
  (params (DeltaSeconds :type Float%20%28single-precision%29))
  (if (Variables|Default|GetIsReady)
    (if (== (Variables|/Script/CouchGame.LevelStreamerActor|GetCurrentLevel (Variables|Default|GetLevelStreamerActor)) "Face_1")
      (Class|StepManager|NextStep (Variables|Default|GetStepManager))
      (Variables|Default|SetIsReady false))))

(event EventOnAutoStep
  (Variables|Default|SetIsReady false))

(fn ConstructionScript)
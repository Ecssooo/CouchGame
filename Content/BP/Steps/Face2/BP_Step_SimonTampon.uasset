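; BP_Step_SimonTampon is a Face2 step that waits for two cube interactions, 202 and 203, to be completed in any order.
; On start it highlights both through the SaveCube subsystem, then polls their saved data every Tick, clearing each highlight upon completion.
; When both are finished it tells the StepManager to advance.
; Auto-step saves both as completed and stops polling, without clearing highlights or advancing itself.
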(event EventOnStartStep
  (Class|SaveCubeSubsystem|SetInteractionHighlight (Subsystems|GetSaveCubeSubsystem) 202 true)
  (Class|SaveCubeSubsystem|SetInteractionHighlight (Subsystems|GetSaveCubeSubsystem) 203 true)
  (Variables|Default|SetIsReady true))

(event EventOnAutoStep
  (Class|SaveCubeSubsystem|SaveInteractionData (Subsystems|GetSaveCubeSubsystem) 202 true)
  (Class|SaveCubeSubsystem|SaveInteractionData (Subsystems|GetSaveCubeSubsystem) 203 true)
  (Variables|Default|SetIsReady false))

(event EventTick
  (params (DeltaSeconds :type Float%20%28single-precision%29))
  (if (Variables|Default|GetIsReady)
    (Utilities|FlowControl|Sequence
      (:then_0
        (if (not (Variables|Default|Get202Finish))
          (bind _returnvalue (Class|SaveCubeSubsystem|GetInteractionsDatasfromID (Subsystems|GetSaveCubeSubsystem) 202))
          (if (.iscompleted _returnvalue)
            (Variables|Default|Set202Finish true)
            (Class|SaveCubeSubsystem|SetInteractionHighlight (Subsystems|GetSaveCubeSubsystem) 202 false))))
      (:then_1
        (if (not (Variables|Default|Get203Finish))
          (bind _returnvalue_2 (Class|SaveCubeSubsystem|GetInteractionsDatasfromID (Subsystems|GetSaveCubeSubsystem) 203))
          (if (.iscompleted _returnvalue_2)
            (Variables|Default|Set203Finish true)
            (Class|SaveCubeSubsystem|SetInteractionHighlight (Subsystems|GetSaveCubeSubsystem) 203 false))))
      (:then_2
        (if (and (Variables|Default|Get202Finish) (Variables|Default|Get203Finish))
          (Variables|Default|SetIsReady false)
          (Class|StepManager|NextStep (Variables|Default|GetStepManager)))))))

(fn ConstructionScript)
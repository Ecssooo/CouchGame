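; Tutorial-style step for face 2 that has the player socket two grab objects, 201 and 202, apparently the computer and briefcase.
; On start it highlights both objects and that face's teleporters through SaveCubeSubsystem.
; Tick polls each object's state, clears its highlight once socketed, then advances StepManager when both are done.
; Ending the step clears all highlights, while auto-step stops polling and forces both objects into their sockets.
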(event EventOnStartStep
  (Variables|Default|SetIsReady true)
  (Class|SaveCubeSubsystem|SetObjectHighlight (Subsystems|GetSaveCubeSubsystem) 201 true)
  (Class|SaveCubeSubsystem|SetObjectHighlight (Subsystems|GetSaveCubeSubsystem) 202 true)
  (Class|SaveCubeSubsystem|SetTeleporterHighlightforFace (Subsystems|GetSaveCubeSubsystem) 2))

(event EventTick
  (params (DeltaSeconds :type Float%20%28single-precision%29))
  (if (Variables|Default|GetIsReady)
    (bind _returnvalue (Class|SaveCubeSubsystem|GetGrabObjectfromID (Subsystems|GetSaveCubeSubsystem) 201))
    (bind _returnvalue_2 (Class|SaveCubeSubsystem|GetGrabObjectfromID (Subsystems|GetSaveCubeSubsystem) 202))
    (Utilities|FlowControl|Sequence
      (:then_0
        (if (not (Variables|Default|Get202IsInSocket))
          (if (== (.objectstate _returnvalue_2) 0)
            (Variables|Default|Set202IsInSocket true)
            (Class|SaveCubeSubsystem|SetObjectHighlight (Subsystems|GetSaveCubeSubsystem) 202 false))))
      (:then_1
        (if (not (Variables|Default|Get201IsInSocket))
          (if (== (.objectstate _returnvalue) 0)
            (Variables|Default|Set201IsInSocket true)
            (Class|SaveCubeSubsystem|SetObjectHighlight (Subsystems|GetSaveCubeSubsystem) 201 false))))
      (:then_2
        (if (Variables|Default|Get202IsInSocket)
          (if (Variables|Default|Get201IsInSocket)
            (Variables|Default|SetIsReady false)
            (Class|StepManager|NextStep (Variables|Default|GetStepManager))))))))

(event EventOnEndStep
  (Class|SaveCubeSubsystem|SetObjectHighlight (Subsystems|GetSaveCubeSubsystem) 201 false)
  (Class|SaveCubeSubsystem|SetObjectHighlight (Subsystems|GetSaveCubeSubsystem) 202 false)
  (Class|SaveCubeSubsystem|ResetAllTeleporterHighlight (Subsystems|GetSaveCubeSubsystem)))

(event EventOnAutoStep
  (Variables|Default|SetIsReady false)
  (Class|SaveCubeSubsystem|SetObjectState (Subsystems|GetSaveCubeSubsystem) 201 "InSocket" 201)
  (Class|SaveCubeSubsystem|SetObjectState (Subsystems|GetSaveCubeSubsystem) 202 "InSocket" 202))

(fn ConstructionScript)
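; Tutorial-style step Blueprint for fetching the fishing rods (cannes à pêche), grab objects 103 and 104.
; On start it highlights both objects and the face 1 teleporter through SaveCubeSubsystem.
; Tick polls their ObjectState, latches each as socketed at state 0 (103 before 104), clears its highlight, then calls StepManager.NextStep.
; Step end resets teleporter highlights and un-highlights 101 and 102, rather than this step's objects.
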(event EventOnStartStep
  (Variables|Default|SetIsReady true)
  (Class|SaveCubeSubsystem|SetObjectHighlight (Subsystems|GetSaveCubeSubsystem) 103 true)
  (Class|SaveCubeSubsystem|SetObjectHighlight (Subsystems|GetSaveCubeSubsystem) 104 true)
  (Class|SaveCubeSubsystem|SetTeleporterHighlightforFace (Subsystems|GetSaveCubeSubsystem) 1))

(event EventTick
  (params (DeltaSeconds :type Float%20%28single-precision%29))
  (if (Variables|Default|GetIsReady)
    (bind _returnvalue (Class|SaveCubeSubsystem|GetGrabObjectfromID (Subsystems|GetSaveCubeSubsystem) 103))
    (bind _returnvalue_2 (Class|SaveCubeSubsystem|GetGrabObjectfromID (Subsystems|GetSaveCubeSubsystem) 104))
    (if (Variables|Default|Get103IsInSocket)
      (if (Variables|Default|Get104IsInSocket)
        (Variables|Default|SetIsReady false)
        (Class|StepManager|NextStep (Variables|Default|GetStepManager))
        (elif (== (.objectstate _returnvalue_2) 0)
          (Variables|Default|Set104IsInSocket true)
          (Class|SaveCubeSubsystem|SetObjectHighlight (Subsystems|GetSaveCubeSubsystem) 104 false)))
      (elif (== (.objectstate _returnvalue) 0)
        (Variables|Default|Set103IsInSocket true)
        (Class|SaveCubeSubsystem|SetObjectHighlight (Subsystems|GetSaveCubeSubsystem) 103 false)))))

(event EventOnEndStep
  (Class|SaveCubeSubsystem|SetObjectHighlight (Subsystems|GetSaveCubeSubsystem) 101 false)
  (Class|SaveCubeSubsystem|SetObjectHighlight (Subsystems|GetSaveCubeSubsystem) 102 false)
  (Class|SaveCubeSubsystem|ResetAllTeleporterHighlight (Subsystems|GetSaveCubeSubsystem)))

(fn ConstructionScript)
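; Step Blueprint for the toolbox and paint pot (objects 101 and 102) that completes once both count as socketed.
; On start it highlights both objects and the teleporter for face 1 through SaveCubeSubsystem.
; Tick polls ObjectState, latching and un-highlighting each object at state 0, checking 102 only after 101 is latched, then calls StepManager.NextStep.
; Ending the step clears all these highlights.
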(event EventOnStartStep
  (Variables|Default|SetIsReady true)
  (Class|SaveCubeSubsystem|SetObjectHighlight (Subsystems|GetSaveCubeSubsystem) 101 true)
  (Class|SaveCubeSubsystem|SetObjectHighlight (Subsystems|GetSaveCubeSubsystem) 102 true)
  (Class|SaveCubeSubsystem|SetTeleporterHighlightforFace (Subsystems|GetSaveCubeSubsystem) 1))

(event EventTick
  (params (DeltaSeconds :type Float%20%28single-precision%29))
  (if (Variables|Default|GetIsReady)
    (bind _returnvalue (Class|SaveCubeSubsystem|GetGrabObjectfromID (Subsystems|GetSaveCubeSubsystem) 101))
    (bind _returnvalue_2 (Class|SaveCubeSubsystem|GetGrabObjectfromID (Subsystems|GetSaveCubeSubsystem) 102))
    (if (Variables|Default|Get101IsInSocket)
      (if (Variables|Default|Get102IsInSocket)
        (Variables|Default|SetIsReady false)
        (Class|StepManager|NextStep (Variables|Default|GetStepManager))
        (elif (== (.objectstate _returnvalue_2) 0)
          (Variables|Default|Set102IsInSocket true)
          (Class|SaveCubeSubsystem|SetObjectHighlight (Subsystems|GetSaveCubeSubsystem) 102 false)))
      (elif (== (.objectstate _returnvalue) 0)
        (Variables|Default|Set101IsInSocket true)
        (Class|SaveCubeSubsystem|SetObjectHighlight (Subsystems|GetSaveCubeSubsystem) 101 false)))))

(event EventOnEndStep
  (Class|SaveCubeSubsystem|SetObjectHighlight (Subsystems|GetSaveCubeSubsystem) 101 false)
  (Class|SaveCubeSubsystem|SetObjectHighlight (Subsystems|GetSaveCubeSubsystem) 102 false)
  (Class|SaveCubeSubsystem|ResetAllTeleporterHighlight (Subsystems|GetSaveCubeSubsystem)))

(fn ConstructionScript)
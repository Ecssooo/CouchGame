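; A scripted step that disables the teleporters registered in the level's BP_SaveSubLevelManager.
; On start, it waits briefly, calls CEEnableTP(false) on each BP_TP in the manager's TeleporterReferences, then tells the StepManager to advance.
; The auto-step path repeats the same delayed disable but does not call NextStep itself.
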(event EventOnAutoStep
  (Utilities|FlowControl|Delay 1.0)
  (bind _returnvalue (Actor|GetActorOfClass "/Game/BP/Systems/BP_SaveSubLevelManager.BP_SaveSubLevelManager_C"))
  (for _array_element (Variables|/Script/CouchGame.SaveSubLevelManager|GetTeleporterReferences _returnvalue)
    (bind _asbp_tp (Utilities|Casting|CastToBP_TP _array_element))
    (Default|CEEnableTP _asbp_tp false)))

(event EventOnStartStep
  (Utilities|FlowControl|Delay 1.0)
  (bind _returnvalue (Actor|GetActorOfClass "/Game/BP/Systems/BP_SaveSubLevelManager.BP_SaveSubLevelManager_C"))
  (for _array_element (Variables|/Script/CouchGame.SaveSubLevelManager|GetTeleporterReferences _returnvalue)
    (bind _asbp_tp (Utilities|Casting|CastToBP_TP _array_element))
    (Default|CEEnableTP _asbp_tp false))
  (Class|StepManager|NextStep (Variables|Default|GetStepManager)))

(fn ConstructionScript)
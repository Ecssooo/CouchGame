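; BP_Step_Peche is a step, apparently for fishing, that waits for the player to complete a specific interaction.
; On start it highlights that interaction through the SaveCube subsystem and arms a ready flag.
; Tick then polls the interaction's data and, once completed, clears the flag and tells the StepManager to advance.
; Ending the step removes the highlight.
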(event EventOnStartStep
  (Class|SaveCubeSubsystem|SetInteractionHighlight (Subsystems|GetSaveCubeSubsystem) 102 true)
  (Variables|Default|SetIsReady true))

(event EventTick
  (params (DeltaSeconds :type Float%20%28single-precision%29))
  (if (Variables|Default|GetIsReady)
    (bind _returnvalue (Class|SaveCubeSubsystem|GetInteractionsDatasfromID (Subsystems|GetSaveCubeSubsystem) 102))
    (if (.iscompleted _returnvalue)
      (Variables|Default|SetIsReady false)
      (Class|StepManager|NextStep (Variables|Default|GetStepManager)))))

(event EventOnEndStep
  (Class|SaveCubeSubsystem|SetInteractionHighlight (Subsystems|GetSaveCubeSubsystem) 102 false))

(fn ConstructionScript)
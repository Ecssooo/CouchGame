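; Step Blueprint for a face 4 placement puzzle step, completed when three grab objects (IDs 404–406) are all in their sockets.
; On start it highlights the objects through the SaveCubeSubsystem, then polls their states every Tick.
; Once all are socketed, it clears the highlights and calls NextStep on the StepManager.
; Auto-step forces all three into InSocket, and ending the step resets teleporter highlights.
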(event EventOnEndStep
  (Class|SaveCubeSubsystem|ResetAllTeleporterHighlight (Subsystems|GetSaveCubeSubsystem)))

(event EventOnStartStep
  (bind _returnvalue (Subsystems|GetSaveCubeSubsystem))
  (Variables|Default|SetIs%20Ready true)
  (Class|SaveCubeSubsystem|SetObjectHighlight _returnvalue 404 true)
  (Class|SaveCubeSubsystem|SetObjectHighlight _returnvalue 405 true)
  (Class|SaveCubeSubsystem|SetObjectHighlight _returnvalue 406 true))

(event EventTick
  (params (DeltaSeconds :type Float%20%28single-precision%29))
  (bind _returnvalue (Subsystems|GetSaveCubeSubsystem))
  (if (Variables|Default|GetIs%20Ready)
    (bind _returnvalue_2 (CallFunction|GetGrabStateIsinSocket))
    (if _returnvalue_2
      (Class|SaveCubeSubsystem|SetObjectHighlight _returnvalue 404 false)
      (Class|SaveCubeSubsystem|SetObjectHighlight _returnvalue 405 false)
      (Class|SaveCubeSubsystem|SetObjectHighlight _returnvalue 406 false)
      (Variables|Default|SetIs%20Ready false)
      (Class|StepManager|NextStep (Variables|Default|GetStepManager)))))

(event EventOnAutoStep
  (bind _returnvalue (Subsystems|GetSaveCubeSubsystem))
  (Class|SaveCubeSubsystem|SetObjectState _returnvalue 404 "InSocket" 404)
  (Class|SaveCubeSubsystem|SetObjectState _returnvalue 405 "InSocket" 405)
  (Class|SaveCubeSubsystem|SetObjectState _returnvalue 406 "InSocket" 406)
  (Variables|Default|SetIs%20Ready false))

(fn ConstructionScript)

(fn GetGrabStateIsinSocket
  (bind _returnvalue (Subsystems|GetSaveCubeSubsystem))
  (Utilities|FlowControl|Sequence
    (:then_0
      (bind _returnvalue_2 (Class|SaveCubeSubsystem|GetGrabObjectfromID _returnvalue 404)))
    (:then_1
      (bind _returnvalue_3 (Class|SaveCubeSubsystem|GetGrabObjectfromID _returnvalue 405)))
    (:then_2
      (bind _returnvalue_4 (Class|SaveCubeSubsystem|GetGrabObjectfromID _returnvalue 406)))
    (:then_3
      (return (Math|Boolean|ANDBoolean (Utilities|Enum|Equal(Enum) (.objectstate _returnvalue_2) "InSocket") (Utilities|Enum|Equal(Enum) (.objectstate _returnvalue_3) "InSocket") (Utilities|Enum|Equal(Enum) (.objectstate _returnvalue_4) "InSocket"))))))
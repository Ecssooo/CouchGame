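; Step Blueprint for the Face 4 suitcase stage, which waits until three grab objects (IDs 407–409) are placed in their sockets.
; On start it highlights the objects through the SaveCube subsystem, then polls their states on Tick.
; Once all are InSocket, it clears the highlights and advances the StepManager.
; Auto-step forces all three into the socket state, and step end resets teleporter highlights.
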(event EventOnAutoStep
  (bind _returnvalue (Subsystems|GetSaveCubeSubsystem))
  (Class|SaveCubeSubsystem|SetObjectState _returnvalue 407 "InSocket" 407)
  (Class|SaveCubeSubsystem|SetObjectState _returnvalue 408 "InSocket" 408)
  (Class|SaveCubeSubsystem|SetObjectState _returnvalue 409 "InSocket" 409)
  (Variables|Default|SetIs%20Ready false))

(event EventOnEndStep
  (Class|SaveCubeSubsystem|ResetAllTeleporterHighlight (Subsystems|GetSaveCubeSubsystem)))

(event EventOnStartStep
  (bind _returnvalue (Subsystems|GetSaveCubeSubsystem))
  (Variables|Default|SetIs%20Ready true)
  (Class|SaveCubeSubsystem|SetObjectHighlight _returnvalue 407 true)
  (Class|SaveCubeSubsystem|SetObjectHighlight _returnvalue 408 true)
  (Class|SaveCubeSubsystem|SetObjectHighlight _returnvalue 409 true))

(event EventTick
  (params (DeltaSeconds :type Float%20%28single-precision%29))
  (bind _returnvalue (Subsystems|GetSaveCubeSubsystem))
  (if (Variables|Default|GetIs%20Ready)
    (bind _returnvalue_2 (CallFunction|GetGrabStateIsinSocket))
    (if _returnvalue_2
      (Class|SaveCubeSubsystem|SetObjectHighlight _returnvalue 407 false)
      (Class|SaveCubeSubsystem|SetObjectHighlight _returnvalue 408 false)
      (Class|SaveCubeSubsystem|SetObjectHighlight _returnvalue 409 false)
      (Variables|Default|SetIs%20Ready false)
      (Class|StepManager|NextStep (Variables|Default|GetStepManager)))))

(fn ConstructionScript)

(fn GetGrabStateIsinSocket
  (bind _returnvalue (Subsystems|GetSaveCubeSubsystem))
  (Utilities|FlowControl|Sequence
    (:then_0
      (bind _returnvalue_2 (Class|SaveCubeSubsystem|GetGrabObjectfromID _returnvalue 407)))
    (:then_1
      (bind _returnvalue_3 (Class|SaveCubeSubsystem|GetGrabObjectfromID _returnvalue 408)))
    (:then_2
      (bind _returnvalue_4 (Class|SaveCubeSubsystem|GetGrabObjectfromID _returnvalue 409)))
    (:then_3
      (return (Math|Boolean|ANDBoolean (Utilities|Enum|Equal(Enum) (.objectstate _returnvalue_2) "InSocket") (Utilities|Enum|Equal(Enum) (.objectstate _returnvalue_3) "InSocket") (Utilities|Enum|Equal(Enum) (.objectstate _returnvalue_4) "InSocket"))))))
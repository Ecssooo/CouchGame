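; Tutorial or sequence step Blueprint that asks the player to get bear object 403 and place it in its socket.
; On start it highlights the object and the face 3 teleporter through SaveCubeSubsystem.
; Tick polls the object's state and calls StepManager.NextStep once it is InSocket.
; Ending clears highlights, and auto-step forces the object into its socket without player action.
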(event EventOnEndStep
  (Class|SaveCubeSubsystem|SetObjectHighlight (Subsystems|GetSaveCubeSubsystem) 403 false)
  (Class|SaveCubeSubsystem|ResetAllTeleporterHighlight (Subsystems|GetSaveCubeSubsystem)))

(event EventOnStartStep
  (Variables|Default|SetIs%20Ready true)
  (Class|SaveCubeSubsystem|SetObjectHighlight (Subsystems|GetSaveCubeSubsystem) 403 true)
  (Class|SaveCubeSubsystem|SetTeleporterHighlightforFace (Subsystems|GetSaveCubeSubsystem) 3))

(event EventTick
  (params (DeltaSeconds :type Float%20%28single-precision%29))
  (if (Variables|Default|GetIs%20Ready)
    (bind _returnvalue (Class|SaveCubeSubsystem|GetGrabObjectfromID (Subsystems|GetSaveCubeSubsystem) 403))
    (if (Utilities|Enum|Equal(Enum) (.objectstate _returnvalue) "InSocket")
      (Class|SaveCubeSubsystem|SetObjectHighlight (Subsystems|GetSaveCubeSubsystem) 403 false)
      (Variables|Default|SetIs%20Ready false)
      (Class|StepManager|NextStep (Variables|Default|GetStepManager)))))

(event EventOnAutoStep
  (Class|SaveCubeSubsystem|SetObjectState (Subsystems|GetSaveCubeSubsystem) 403 "InSocket" 403)
  (Variables|Default|SetIs%20Ready false))

(fn ConstructionScript)
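; Step Blueprint that plays the Face1 narrator line in a tutorial or sequence of steps.
; On step start it creates a WBP_Naration widget, adds it to the viewport and starts narration with the step's text, audio component and the VOC_Narrator_Face1 voice name.
; On auto step it stops the narrator and removes the widget from its parent.
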(event EventOnAutoStep
  (Default|CEStopNarrator (Variables|Default|GetWBP%20Naration))
  (Widget|RemovefromParent (Variables|Default|GetWBP%20Naration)))

(event EventOnStartStep
  (bind _returnvalue (UserInterface|CreateWidget "/Game/UI/WBP_Naration.WBP_Naration_C"))
  (bind _output_get (Variables|Default|SetWBP%20Naration _returnvalue))
  (UserInterface|Viewport|AddtoViewport _output_get 0)
  (Default|CEPlayNarrator (Variables|Default|GetWBP%20Naration) (Variables|Default|GetText) (Variables|Default|GetAudio) "VOC_Narrator_Face1" 2.0 2.0 5.0 2.0 2.0))

(fn ConstructionScript)
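; Tutorial-style step Blueprint for Face 1 that waits until the two fishing rods (grab objects 103 and 104) are socketed.
; On start it highlights both objects and the face's teleporters through SaveCubeSubsystem.
; Tick polls each object's state, clears its highlight once socketed, then calls StepManager.NextStep when both are done.
; Ending the step clears all highlights, while auto-step forces both objects into their sockets.
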(event EventOnStartStep
  (Variables|Default|SetIsReady true)
  (Class|SaveCubeSubsystem|SetObjectHighlight (Subsystems|GetSaveCubeSubsystem) 103 true)
  (Class|SaveCubeSubsystem|SetObjectHighlight (Subsystems|GetSaveCubeSubsystem) 104 true)
  (Class|SaveCubeSubsystem|SetTeleporterHighlightforFace (Subsystems|GetSaveCubeSubsystem) 1))

(event EventTick
  (params (DeltaSeconds :type Float%20%28single-precision%29))
  (if (Variables|Default|GetIsReady)
    (bind _returnvalue (Class|SaveCubeSubsystem|GetGrabObjectfromID (Subsystems|GetSaveCubeSubsystem) 103))
    (bind _returnvalue_2 (Class|SaveCubeSubsystem|GetGrabObjectfromID (Subsystems|GetSaveCubeSubsystem) 104))
    (Utilities|FlowControl|Sequence
      (:then_0
        (if (not (Variables|Default|Get104IsInSocket))
          (if (== (.objectstate _returnvalue_2) 0)
            (Variables|Default|Set104IsInSocket true)
            (Class|SaveCubeSubsystem|SetObjectHighlight (Subsystems|GetSaveCubeSubsystem) 104 false))))
      (:then_1
        (if (not (Variables|Default|Get103IsInSocket))
          (if (== (.objectstate _returnvalue) 0)
            (Variables|Default|Set103IsInSocket true)
            (Class|SaveCubeSubsystem|SetObjectHighlight (Subsystems|GetSaveCubeSubsystem) 103 false))))
      (:then_2
        (if (Variables|Default|Get104IsInSocket)
          (if (Variables|Default|Get103IsInSocket)
            (Variables|Default|SetIsReady false)
            (Class|StepManager|NextStep (Variables|Default|GetStepManager))))))))

(event EventOnEndStep
  (Class|SaveCubeSubsystem|SetObjectHighlight (Subsystems|GetSaveCubeSubsystem) 103 false)
  (Class|SaveCubeSubsystem|SetObjectHighlight (Subsystems|GetSaveCubeSubsystem) 104 false)
  (Class|SaveCubeSubsystem|ResetAllTeleporterHighlight (Subsystems|GetSaveCubeSubsystem)))

(event EventOnAutoStep
  (Variables|Default|SetIsReady false)
  (Class|SaveCubeSubsystem|SetObjectState (Subsystems|GetSaveCubeSubsystem) 103 "InSocket" 103)
  (Class|SaveCubeSubsystem|SetObjectState (Subsystems|GetSaveCubeSubsystem) 104 "InSocket" 104))

(fn ConstructionScript)
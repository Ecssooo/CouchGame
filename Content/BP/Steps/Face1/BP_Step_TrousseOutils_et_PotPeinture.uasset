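; Tutorial-style step Blueprint for the toolkit and paint pot (objects 101, 102) on cube face 1.
; On start it highlights both objects and the face's teleporters; ending clears them.
; Tick polls each object's state to drop its highlight and advances StepManager once both socket flags are true, though this graph only sets them false.
; Auto-step stops polling and forces both objects into their sockets.
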(event EventOnStartStep
  (Variables|Default|SetIsReady true)
  (Class|SaveCubeSubsystem|SetObjectHighlight (Subsystems|GetSaveCubeSubsystem) 101 true)
  (Class|SaveCubeSubsystem|SetObjectHighlight (Subsystems|GetSaveCubeSubsystem) 102 true)
  (Class|SaveCubeSubsystem|SetTeleporterHighlightforFace (Subsystems|GetSaveCubeSubsystem) 1))

(event EventTick
  (params (DeltaSeconds :type Float%20%28single-precision%29))
  (if (Variables|Default|GetIsReady)
    (bind _returnvalue (Class|SaveCubeSubsystem|GetGrabObjectfromID (Subsystems|GetSaveCubeSubsystem) 101))
    (bind _returnvalue_2 (Class|SaveCubeSubsystem|GetGrabObjectfromID (Subsystems|GetSaveCubeSubsystem) 102))
    (Utilities|FlowControl|Sequence
      (:then_0
        (if (not (Variables|Default|Get102IsInSocket))
          (if (== (.objectstate _returnvalue_2) 0)
            (Variables|Default|Set102IsInSocket false)
            (Class|SaveCubeSubsystem|SetObjectHighlight (Subsystems|GetSaveCubeSubsystem) 102 false))))
      (:then_1
        (if (not (Variables|Default|Get101IsInSocket))
          (if (== (.objectstate _returnvalue) 0)
            (Variables|Default|Set101IsInSocket false)
            (Class|SaveCubeSubsystem|SetObjectHighlight (Subsystems|GetSaveCubeSubsystem) 101 false))))
      (:then_2
        (if (Variables|Default|Get102IsInSocket)
          (if (Variables|Default|Get101IsInSocket)
            (Variables|Default|SetIsReady false)
            (Class|StepManager|NextStep (Variables|Default|GetStepManager))))))))

(event EventOnEndStep
  (Class|SaveCubeSubsystem|SetObjectHighlight (Subsystems|GetSaveCubeSubsystem) 101 false)
  (Class|SaveCubeSubsystem|SetObjectHighlight (Subsystems|GetSaveCubeSubsystem) 102 false)
  (Class|SaveCubeSubsystem|ResetAllTeleporterHighlight (Subsystems|GetSaveCubeSubsystem)))

(event EventOnAutoStep
  (Variables|Default|SetIsReady false)
  (Class|SaveCubeSubsystem|SetObjectState (Subsystems|GetSaveCubeSubsystem) 101 "InSocket" 101)
  (Class|SaveCubeSubsystem|SetObjectState (Subsystems|GetSaveCubeSubsystem) 102 "InSocket" 102))

(fn ConstructionScript)
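; Tutorial or progression step for Face1's swing that waits for interaction 101 to be completed before advancing the step manager.
; On start it highlights the interaction through the SaveCube subsystem, then polls its saved completion state every Tick and calls NextStep once done.
; Auto-step marks the interaction completed and clears the highlight.
; An unconnected branch that would enable sublevel teleporters never runs.
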(event EventOnAutoStep
  (Class|SaveCubeSubsystem|SaveInteractionData (Subsystems|GetSaveCubeSubsystem) 101 true)
  (Variables|Default|SetIsReady false)
  (Class|SaveCubeSubsystem|SetInteractionHighlight (Subsystems|GetSaveCubeSubsystem) 101 false))

(event EventOnStartStep
  (Class|SaveCubeSubsystem|SetInteractionHighlight (Subsystems|GetSaveCubeSubsystem) 101 true)
  (Variables|Default|SetIsReady true))

(event EventTick
  (params (DeltaSeconds :type Float%20%28single-precision%29))
  (if (Variables|Default|GetIsReady)
    (bind _returnvalue (Class|SaveCubeSubsystem|GetInteractionsDatasfromID (Subsystems|GetSaveCubeSubsystem) 101))
    (if (.iscompleted _returnvalue)
      (Variables|Default|SetIsReady false)
      (Class|StepManager|NextStep (Variables|Default|GetStepManager)))))

(event EventOnEndStep)

(fn ConstructionScript)
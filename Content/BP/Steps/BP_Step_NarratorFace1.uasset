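; Step Blueprint that plays the Face 1 narrator moment, showing narration text with a voice line, as one step in a managed sequence.
; On step start it creates a WBP_Naration widget, shows its background and text, then plays the narrator line through SoundManager.
; Fixed delays time the whole sequence through hiding and removing the widget, after which it tells StepManager to advance.
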(event EventOnStartStep
  (Development|PrintString "Start Face 1 Narrator" true true "(R=1.000000,G=0.164097,B=0.000000,A=1.000000)" 1e+01)
  (bind _returnvalue (UserInterface|CreateWidget "/Game/UI/WBP_Naration.WBP_Naration_C"))
  (bind _output_get (Variables|Default|SetWBP%20Naration _returnvalue))
  (UserInterface|Viewport|AddtoViewport _output_get 0)
  (Default|CEShowBG (Variables|Default|GetWBP%20Naration))
  (Utilities|FlowControl|Delay 1.0)
  (Default|CESetText (Variables|Default|GetWBP%20Naration) (Variables|Default|GetText))
  (Default|CEShowText (Variables|Default|GetWBP%20Naration))
  (Utilities|FlowControl|Delay 2.0)
  (Class|SoundManager|PlaySound (Subsystems|GetSoundManager) "VOC_Narrator_Face1" (Variables|Default|GetAudio))
  (Utilities|FlowControl|Delay 4.0)
  (Default|CEHideText (Variables|Default|GetWBP%20Naration))
  (Utilities|FlowControl|Delay 2.0)
  (Default|CEHideBG (Variables|Default|GetWBP%20Naration))
  (Utilities|FlowControl|Delay 2.0)
  (Widget|RemovefromParent (Variables|Default|GetWBP%20Naration))
  (Class|StepManager|NextStep (Variables|Default|GetStepManager)))

(fn ConstructionScript)
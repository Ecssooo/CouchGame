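; Step Blueprint for the bench interaction on cube face 5, run as part of a StepManager sequence.
; On start it highlights interaction 501 and face 5's teleporters through SaveCubeSubsystem, then refreshes teleporter states via BP_SaveSubLevelManager.
; Tick polls that interaction's saved completion and advances to the next step once done.
; Ending clears the highlights, and auto-step saves the interaction as completed.
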(event EventOnStartStep
  (Class|SaveCubeSubsystem|ResetAllTeleporterHighlight (Subsystems|GetSaveCubeSubsystem))
  (Class|SaveCubeSubsystem|SetInteractionHighlight (Subsystems|GetSaveCubeSubsystem) 501 true)
  (Variables|Default|SetIsReady true)
  (Class|SaveCubeSubsystem|SetTeleporterHighlightforFace (Subsystems|GetSaveCubeSubsystem) 5)
  (bind _returnvalue (Actor|GetActorOfClass "/Game/BP/Systems/BP_SaveSubLevelManager.BP_SaveSubLevelManager_C"))
  (Class|SaveSubLevelManager|UpdateAllTeleporterState _returnvalue))

(event EventOnAutoStep
  (Class|SaveCubeSubsystem|SaveInteractionData (Subsystems|GetSaveCubeSubsystem) 501 true)
  (Variables|Default|SetIsReady false))

(event EventTick
  (params (DeltaSeconds :type Float%20%28single-precision%29))
  (if (Variables|Default|GetIsReady)
    (bind _returnvalue (Class|SaveCubeSubsystem|GetInteractionsDatasfromID (Subsystems|GetSaveCubeSubsystem) 501))
    (if (.iscompleted _returnvalue)
      (Variables|Default|SetIsReady false)
      (Class|StepManager|NextStep (Variables|Default|GetStepManager)))))

(event EventOnEndStep
  (Class|SaveCubeSubsystem|SetInteractionHighlight (Subsystems|GetSaveCubeSubsystem) 501 false)
  (Class|SaveCubeSubsystem|ResetAllTeleporterHighlight (Subsystems|GetSaveCubeSubsystem)))

(fn ConstructionScript)
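; Step Blueprint for the snowball (BoulesNeige) objective on Face 5, completed once three grabbable objects are socketed.
; On start, it highlights the objects and the face's teleporters through SaveCubeSubsystem.
; Tick polls each object's state, clears its highlight once socketed, and calls StepManager.NextStep when all three are placed.
; Step end clears all highlights, while auto-step stops polling and forces the objects into the socketed state.
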(event EventOnStartStep
  (Variables|Default|SetIsReady true)
  (Class|SaveCubeSubsystem|SetObjectHighlight (Subsystems|GetSaveCubeSubsystem) 501 true)
  (Class|SaveCubeSubsystem|SetObjectHighlight (Subsystems|GetSaveCubeSubsystem) 502 true)
  (Class|SaveCubeSubsystem|SetObjectHighlight (Subsystems|GetSaveCubeSubsystem) 503 true)
  (Class|SaveCubeSubsystem|SetTeleporterHighlightforFace (Subsystems|GetSaveCubeSubsystem) 5))

(event EventTick
  (params (DeltaSeconds :type Float%20%28single-precision%29))
  (if (Variables|Default|GetIsReady)
    (bind _returnvalue (Class|SaveCubeSubsystem|GetGrabObjectfromID (Subsystems|GetSaveCubeSubsystem) 503))
    (bind _returnvalue_2 (Class|SaveCubeSubsystem|GetGrabObjectfromID (Subsystems|GetSaveCubeSubsystem) 501))
    (bind _returnvalue_3 (Class|SaveCubeSubsystem|GetGrabObjectfromID (Subsystems|GetSaveCubeSubsystem) 502))
    (Utilities|FlowControl|Sequence
      (:then_0
        (if (not (Variables|Default|Get502IsInSocket))
          (if (Utilities|Enum|Equal(Enum) (.objectstate _returnvalue_3) "InSocket")
            (Variables|Default|Set502IsInSocket true)
            (Class|SaveCubeSubsystem|SetObjectHighlight (Subsystems|GetSaveCubeSubsystem) 502 false))))
      (:then_1
        (if (not (Variables|Default|Get501IsInSocket))
          (if (Utilities|Enum|Equal(Enum) (.objectstate _returnvalue_2) "InSocket")
            (Variables|Default|Set501IsInSocket true)
            (Class|SaveCubeSubsystem|SetObjectHighlight (Subsystems|GetSaveCubeSubsystem) 501 false))))
      (:then_2
        (if (not (Variables|Default|Get503IsInSocket))
          (if (Utilities|Enum|Equal(Enum) (.objectstate _returnvalue) "InSocket")
            (Variables|Default|Set503IsInSocket true)
            (Class|SaveCubeSubsystem|SetObjectHighlight (Subsystems|GetSaveCubeSubsystem) 503 false))))
      (:then_4
        (if (Math|Boolean|ANDBoolean (Variables|Default|Get503IsInSocket) (Variables|Default|Get501IsInSocket) (Variables|Default|Get502IsInSocket))
          (Variables|Default|SetIsReady false)
          (Class|StepManager|NextStep (Variables|Default|GetStepManager)))))))

(event EventOnEndStep
  (Class|SaveCubeSubsystem|SetObjectHighlight (Subsystems|GetSaveCubeSubsystem) 501 false)
  (Class|SaveCubeSubsystem|SetObjectHighlight (Subsystems|GetSaveCubeSubsystem) 502 false)
  (Class|SaveCubeSubsystem|SetObjectHighlight (Subsystems|GetSaveCubeSubsystem) 503 false)
  (Class|SaveCubeSubsystem|ResetAllTeleporterHighlight (Subsystems|GetSaveCubeSubsystem)))

(event EventOnAutoStep
  (Variables|Default|SetIsReady false)
  (Class|SaveCubeSubsystem|SetObjectState (Subsystems|GetSaveCubeSubsystem) 501 "InSocket" 501)
  (Class|SaveCubeSubsystem|SetObjectState (Subsystems|GetSaveCubeSubsystem) 502 "InSocket" 502)
  (Class|SaveCubeSubsystem|SetObjectState (Subsystems|GetSaveCubeSubsystem) 503 "InSocket" 503))

(fn ConstructionScript)
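; BP_Step_Dialogue is a step Blueprint that shows a dialogue line during a step sequence.
; On start, it creates a WBP_Dialogue widget, adds it to the viewport and plays the dialogue with its crow flag, text and audio component.
; On auto step, it removes the widget from the screen.
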(event EventOnAutoStep
  (Widget|RemovefromParent (Variables|Default|GetWBP%20Dialogue)))

(event EventOnStartStep
  (bind _returnvalue (UserInterface|CreateWidget "/Game/UI/WBP_Dialogue.WBP_Dialogue_C"))
  (bind _output_get (Variables|Default|SetWBP%20Dialogue _returnvalue))
  (UserInterface|Viewport|AddtoViewport _output_get 0)
  (Default|CEPlayDialogue (Variables|Default|GetWBP%20Dialogue) (Variables|Default|GetIs%20Crow) (Variables|Default|GetText) (Variables|Default|GetAudio)))

(fn ConstructionScript)
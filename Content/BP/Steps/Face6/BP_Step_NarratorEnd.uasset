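; BP_Step_NarratorEnd is a step Blueprint, filed under Face6, that plays the ending narration and then opens the Credits level.
; On step start it creates a WBP_Naration widget, adds it to the viewport and plays the VOC_NarratorEnd voice with text and zero-length background show and hide times.
; Auto-step stops the narrator, and step end loads Credits by object reference.
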(event EventOnAutoStep
  (Default|CEStopNarrator (Variables|Default|GetWBP%20Naration)))

(event EventOnEndStep
  (Game|OpenLevel(byObjectReference) "/Game/Levels/Cube/Credits.Credits"))

(event EventOnStartStep
  (bind _returnvalue (UserInterface|CreateWidget "/Game/UI/WBP_Naration.WBP_Naration_C"))
  (bind _output_get (Variables|Default|SetWBP%20Naration _returnvalue))
  (UserInterface|Viewport|AddtoViewport _output_get 0)
  (Default|CEPlayNarrator (Variables|Default|GetWBP%20Naration) (Variables|Default|GetText) (Variables|Default|GetAudio) "VOC_NarratorEnd" 0.0 2.0 5.0 2.0 0.0))

(fn ConstructionScript)
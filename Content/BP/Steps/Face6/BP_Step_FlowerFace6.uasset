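; Step Blueprint for the Face 6 flower step, built around six grab objects tracked through the SaveCube subsystem.
; Step start highlights the objects, and Tick polls their states, clearing the highlights once all are in their sockets.
; Auto-step forces all six into InSocket, and step end resets teleporter highlights.
; The StepManager NextStep call is unconnected, so completion does not advance the step from here.
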(event EventOnEndStep
  (Class|SaveCubeSubsystem|ResetAllTeleporterHighlight (Subsystems|GetSaveCubeSubsystem)))

(event EventOnStartStep
  (bind _returnvalue (Subsystems|GetSaveCubeSubsystem))
  (Variables|Default|SetIs%20Ready true)
  (Class|SaveCubeSubsystem|SetObjectHighlight _returnvalue 601 true)
  (Class|SaveCubeSubsystem|SetObjectHighlight _returnvalue 602 true)
  (Class|SaveCubeSubsystem|SetObjectHighlight _returnvalue 603 true)
  (Class|SaveCubeSubsystem|SetObjectHighlight _returnvalue 604 true)
  (Class|SaveCubeSubsystem|SetObjectHighlight _returnvalue 605 true)
  (Class|SaveCubeSubsystem|SetObjectHighlight _returnvalue 606 true))

(event EventTick
  (params (DeltaSeconds :type Float%20%28single-precision%29))
  (bind _returnvalue (Subsystems|GetSaveCubeSubsystem))
  (if (Variables|Default|GetIs%20Ready)
    (bind _returnvalue_2 (CallFunction|GetGrabStateIsinSocket))
    (if _returnvalue_2
      (Class|SaveCubeSubsystem|SetObjectHighlight _returnvalue 601 false)
      (Class|SaveCubeSubsystem|SetObjectHighlight _returnvalue 602 false)
      (Class|SaveCubeSubsystem|SetObjectHighlight _returnvalue 603 false)
      (Class|SaveCubeSubsystem|SetObjectHighlight _returnvalue 604 false)
      (Class|SaveCubeSubsystem|SetObjectHighlight _returnvalue 605 false)
      (Class|SaveCubeSubsystem|SetObjectHighlight _returnvalue 606 false))))

(event EventOnAutoStep
  (bind _returnvalue (Subsystems|GetSaveCubeSubsystem))
  (Class|SaveCubeSubsystem|SetObjectState _returnvalue 601 "InSocket" 601)
  (Class|SaveCubeSubsystem|SetObjectState _returnvalue 602 "InSocket" 602)
  (Class|SaveCubeSubsystem|SetObjectState _returnvalue 603 "InSocket" 603)
  (Class|SaveCubeSubsystem|SetObjectState _returnvalue 604 "InSocket" 604)
  (Class|SaveCubeSubsystem|SetObjectState _returnvalue 605 "InSocket" 605)
  (Class|SaveCubeSubsystem|SetObjectState _returnvalue 606 "InSocket" 606)
  (Variables|Default|SetIs%20Ready false))

(fn ConstructionScript)

(fn GetGrabStateIsinSocket
  (bind _returnvalue (Subsystems|GetSaveCubeSubsystem))
  (Utilities|FlowControl|Sequence
    (:then_0
      (bind _returnvalue_2 (Class|SaveCubeSubsystem|GetGrabObjectfromID _returnvalue 601)))
    (:then_1
      (bind _returnvalue_3 (Class|SaveCubeSubsystem|GetGrabObjectfromID _returnvalue 602)))
    (:then_2
      (bind _returnvalue_4 (Class|SaveCubeSubsystem|GetGrabObjectfromID _returnvalue 603)))
    (:then_3
      (bind _returnvalue_5 (Class|SaveCubeSubsystem|GetGrabObjectfromID _returnvalue 604)))
    (:then_4
      (bind _returnvalue_6 (Class|SaveCubeSubsystem|GetGrabObjectfromID _returnvalue 605)))
    (:then_5
      (bind _returnvalue_7 (Class|SaveCubeSubsystem|GetGrabObjectfromID _returnvalue 606)))
    (:then_6
      (return (Math|Boolean|ANDBoolean (Utilities|Enum|Equal(Enum) (.objectstate _returnvalue_2) "InSocket") (Utilities|Enum|Equal(Enum) (.objectstate _returnvalue_3) "InSocket") (Utilities|Enum|Equal(Enum) (.objectstate _returnvalue_4) "InSocket") (Utilities|Enum|Equal(Enum) (.objectstate _returnvalue_5) "InSocket") (Utilities|Enum|Equal(Enum) (.objectstate _returnvalue_6) "InSocket") (Utilities|Enum|Equal(Enum) (.objectstate _returnvalue_7) "InSocket"))))))
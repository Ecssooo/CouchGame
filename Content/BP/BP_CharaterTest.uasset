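; BP_CharaterTest is a test character Blueprint that drives rotation of a cube actor from numpad input.
; On BeginPlay it finds and caches the BP_Cube and BP_TPManager actors in the level.
; Numpad 8, 2, 4 and 6 each call FUnloadLevel on the manager, then the cube's matching up, down, left or right rotate event.
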(event EventBeginPlay
  (Utilities|FlowControl|Sequence
    (:then_0
      (bind _returnvalue (Actor|GetActorOfClass "/Game/BP/BP_Cube.BP_Cube_C"))
      (Variables|Default|SetBP_Cube _returnvalue))
    (:then_1
      (bind _returnvalue_2 (Actor|GetActorOfClass "/Game/BP/BP_TPManager.BP_TPManager_C"))
      (Variables|Default|SetBP_TPManager _returnvalue_2))))

(event Collision|EventActorBeginOverlap
  (params (OtherActor :type Actor%20Object%20Reference)))

(event EventTick
  (params (DeltaSeconds :type Float%20%28single-precision%29)))

(event Input|KeyboardEvents|NumPadSix
  (params (Key :type Key%20Structure :default "None"))
  (:Pressed
    (Default|FUnloadLevel (Variables|Default|GetBP_TPManager))
    (Default|CERotateRight (Variables|Default|GetBP_Cube))))

(event Input|KeyboardEvents|NumPadEight
  (params (Key :type Key%20Structure :default "None"))
  (:Pressed
    (Default|FUnloadLevel (Variables|Default|GetBP_TPManager))
    (Default|CERotateUp (Variables|Default|GetBP_Cube))))

(event Input|KeyboardEvents|NumPadTwo
  (params (Key :type Key%20Structure :default "None"))
  (:Pressed
    (Default|FUnloadLevel (Variables|Default|GetBP_TPManager))
    (Default|CERotateDown (Variables|Default|GetBP_Cube))))

(event Input|KeyboardEvents|NumPadFour
  (params (Key :type Key%20Structure :default "None"))
  (:Pressed
    (Default|FUnloadLevel (Variables|Default|GetBP_TPManager))
    (Default|CERotateLeft (Variables|Default|GetBP_Cube))))

(fn ConstructionScript)
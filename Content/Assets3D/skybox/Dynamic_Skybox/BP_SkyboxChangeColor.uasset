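; Skybox color controller that fades a vector parameter in a Material Parameter Collection to one of six face colors, selected by level-load index.
; BeginPlay requests color 1, then assigns the timeline's Alpha curve from class defaults.
; CE_ChangeColor scales the timeline's play rate by ChangeDuration and lerps RGB toward GetColor's result.
; Each update lerps from the parameter's current value, so the blend compounds; finishing prints a debug string.
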(event Custom|CE_ChangeColor
  (params (LevelLoad :type Integer))
  (bind _materialcollection (Variables|Default|GetMaterialCollection))
  (Components|Timeline|SetPlayRate (Variables|Default|GetChangeColor) (Math|Float|SafeDivide 1.0 (Variables|Default|GetChangeDuration)))
  (bind _alpha (Timeline|ChangeColor PlayFromStart)
    (:Update
      (bind _color (CallFunction|GetColor LevelLoad))
      (bind _returnvalue (Rendering|Material|GetVectorParameterValue _materialcollection (Variables|Default|GetParameter%20Name) :!class /Script/Engine.KismetMaterialLibrary))
      (Rendering|Material|SetVectorParameterValue _materialcollection (Variables|Default|GetParameter%20Name) (Math|Color|MakeColor (Math|Float|Lerp (.R (Math|Color|BreakColor _returnvalue)) (.R (Math|Color|BreakColor _color)) _alpha) (Math|Float|Lerp (.G (Math|Color|BreakColor _returnvalue)) (.G (Math|Color|BreakColor _color)) _alpha) (Math|Float|Lerp (.B (Math|Color|BreakColor _returnvalue)) (.B (Math|Color|BreakColor _color)) _alpha)) :!class /Script/Engine.KismetMaterialLibrary))
    (:Finished
      (Development|PrintString "Hello"))))

(event EventBeginPlay
  (CallFunction|CEChangeColor 1)
  (Class|TimelineComponent|SetFloatCurve (Variables|Default|GetChangeColor) (Utilities|ResolveSoftReference (Utilities|GetClassDefaults "/Script/CouchGame.TimelineSettings")) "Alpha"))

(fn ConstructionScript)

(fn GetColor
  (params (LevelLoad :type Integer))
  (switch int LevelLoad
    (:1
      (return (Variables|Default|GetColor_Face1)))
    (:2
      (return (Variables|Default|GetColor_Face2)))
    (:3
      (return (Variables|Default|GetColor_Face3)))
    (:4
      (return (Variables|Default|GetColor_Face4)))
    (:5
      (return (Variables|Default|GetColor_Face5)))
    (:6
      (return (Variables|Default|GetColor_Face6)))))